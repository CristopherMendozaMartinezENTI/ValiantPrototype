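; BP_SlidingDoor is a two-panel stone door that slides apart and back together, toggled by Flow notifies.
; Each notify alternates through a FlipFlop between OpenDoor, which also opens an optional Lock, and CloseDoor.
; Both events use TweenVector to move the panels in opposite directions along local Y over a shared Duration.
; Sliding sounds attach to both panels, but only the second panel's sound receives the IsClosing parameter.
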(event `CloseDoor`
  (bind (_asynctaskproxy _value) (`FCTweenBPActionVector.TweenVector` (0.0 236.0 0.0) (0.0 0.0 0.0) (`self.Duration`))
    (:`then`
      (bind (_asynctaskproxy_2 _value_2) (`FCTweenBPActionVector.TweenVector` (0.0 -236.0 0.0) (0.0 0.0 0.0) (`self.Duration`))
        (:`ApplyEasing`
          (`SceneComponent.K2_SetRelativeLocation` (`self.Box2_StaticMeshComponent0`) _value_2 false false))))
    (:`ApplyEasing`
      (`SceneComponent.K2_SetRelativeLocation` (`self.Box_StaticMeshComponent0`) _value false false))))

(event `OpenDoor`
  (bind _duration (`self.Duration`))
  (bind _lock (`self.Lock`))
  (`/Engine/EditorBlueprintResources/StandardMacros.IsValid` _lock
    (:`Is Valid`
      (`/Game/Blueprints/BP_Lock.OpenLock` _lock))
    (:`Is Not Valid`
      _))
  (bind (_asynctaskproxy _value) (`FCTweenBPActionVector.TweenVector` (0.0 0.0 0.0) (0.0 236.0 0.0) _duration)
    (:`then`
      (bind (_asynctaskproxy_2 _value_2) (`FCTweenBPActionVector.TweenVector` (0.0 0.0 0.0) (0.0 -236.0 0.0) _duration)
        (:`ApplyEasing`
          (`SceneComponent.K2_SetRelativeLocation` (`self.Box2_StaticMeshComponent0`) _value_2 false false))))
    (:`ApplyEasing`
      (`SceneComponent.K2_SetRelativeLocation` (`self.Box_StaticMeshComponent0`) _value false false))))

(event `self.Flow.ReceiveNotify`
  (params (FlowComponent :type "FlowComponent Object Reference") (NotifyTag :type "GameplayTag Structure (by ref)"))
  (`/Engine/EditorBlueprintResources/StandardMacros.FlipFlop`
    (:`A`
      (`self.OpenDoor`)
      (`FMODBlueprintStatics.PlayEventAttached` "/Game/FMOD/Events/SFX/Props/SlidingStoneDoor.SlidingStoneDoor" (`self.Box_StaticMeshComponent0`) "None" (0.0 0.0 0.0) "KeepRelativeOffset")
      (bind _returnvalue (`FMODBlueprintStatics.PlayEventAttached` "/Game/FMOD/Events/SFX/Props/SlidingStoneDoor.SlidingStoneDoor" (`self.Box2_StaticMeshComponent0`) "None" (0.0 0.0 0.0) "KeepRelativeOffset"))
      (`FMODAudioComponent.SetParameter` _returnvalue "IsClosing" 0.0))
    (:`B`
      (`self.CloseDoor`)
      (`FMODBlueprintStatics.PlayEventAttached` "/Game/FMOD/Events/SFX/Props/SlidingStoneDoor.SlidingStoneDoor" (`self.Box_StaticMeshComponent0`) "None" (0.0 0.0 0.0) "KeepRelativeOffset")
      (bind _returnvalue_2 (`FMODBlueprintStatics.PlayEventAttached` "/Game/FMOD/Events/SFX/Props/SlidingStoneDoor.SlidingStoneDoor" (`self.Box2_StaticMeshComponent0`) "None" (0.0 0.0 0.0) "KeepRelativeOffset"))
      (`FMODAudioComponent.SetParameter` _returnvalue_2 "IsClosing" 1.0))))

(fn `UserConstructionScript`)
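; Actor component that lets the player interact with its owner, showing an interact prompt by proximity.
; Tick checks player distance unless interaction is external or disabled, using paired DoOnce gates to show or hide the prompt.
; The prompt, UW_Interact, is pushed onto the HUD's game layer and its event triggers Interact.
; Interact optionally restarts an external Flow graph on a freshly added FlowComponent, then broadcasts OnInteract.
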(event `self.ReceiveBeginPlay`)

(event `ShowInteractionHUD`
  ;[1 1 1] Start and Stop interactions
  (bind _asbp_valiant_hud (cast `/Game/UI/BP_ValiantHUD` (`PlayerController.GetHUD` (`GameplayStatics.GetPlayerController` 0))))
  (bind _returnvalue (`/PMDialogue/W_OverallUILayout.PushWidgetToLayerStack` (`/Game/UI/BP_ValiantHUD.OverallWidget` _asbp_valiant_hud) (struct :`TagName` "UI.Layer.Game") "/Game/Blueprints/PROTOTYPEQuest/UW_Interact.UW_Interact_C"))
  (bind _asuw_interact (cast `/Game/Blueprints/PROTOTYPEQuest/UW_Interact` _returnvalue))
  (bind _output_get (set `self.NewVar` _asuw_interact))
  (clear `/Game/Blueprints/PROTOTYPEQuest/UW_Interact.OnInteract` _output_get)
  (`WidgetBlueprintLibrary.SetInputMode_GameOnly` (`GameplayStatics.GetPlayerController` 0))
  (add `/Game/Blueprints/PROTOTYPEQuest/UW_Interact.OnInteract` _output_get (delegate `PrivateInteract`)))

(event `PrivateInteract`
  ;[1 1 1] Start and Stop interactions
  (`self.Interact`))

(event `Interact`
  (bind _flowcom (`self.FlowCom`))
  ;[1 1 1] Start and Stop interactions
  (if (`self.StartExternalFlow`)
    (`/Engine/EditorBlueprintResources/StandardMacros.IsValid` _flowcom
      (:`Is Valid`
        (`self.K2_DestroyComponent` _flowcom))
      (:`Is Not Valid`
        _))
    (bind _returnvalue (`|AddComponentByClass` (`self.GetOwner`) "/Script/Flow.FlowComponent"))
    (set `self.FlowCom` _returnvalue)
    (set `FlowComponent.RootFlow` (`self.ExternalFlow`) _returnvalue)
    (`FlowComponent.StartRootFlow` _returnvalue))
  (`self.OnInteract`))

(event `HideInteractionHUD`
  ;[1 1 1] Start and Stop interactions
  (bind _asbp_valiant_hud (cast `/Game/UI/BP_ValiantHUD` (`PlayerController.GetHUD` (`GameplayStatics.GetPlayerController` 0))))
  (`/PMDialogue/W_OverallUILayout.RemoveLayer` (`/Game/UI/BP_ValiantHUD.OverallWidget` _asbp_valiant_hud) (struct :`TagName` "UI.Layer.Game") (`self.NewVar`)))

(event `self.ReceiveTick`
  (params (DeltaSeconds :type "Float (single-precision)"))
  ;[1 1 1] Detect interaction
  (if (`self.ExternalInteraction`)
    _
    (elif (`self.InteractionEnabled`)
      (if (<= (`Actor.GetDistanceTo` (`self.GetOwner`) (`GameplayStatics.GetPlayerCharacter` 0)) (`self.DistanceToInteract`))
        (`|ExecutionSequence`
          (:`then_0`
            (`/Engine/EditorBlueprintResources/StandardMacros.DoOnce` false :!label _label
              (:`Completed`
                (`self.ShowInteractionHUD`)
                (goto _label_2 :!via `Reset`)))))
        (else
          (`/Engine/EditorBlueprintResources/StandardMacros.DoOnce` false :!label _label_2
            (:`Completed`
              (`self.HideInteractionHUD`)
              (goto _label :!via `Reset`))))))))
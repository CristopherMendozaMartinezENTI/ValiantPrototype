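; Experimental pawn that aims an Arrow component with mouse look, limited to the front half-circle of yaw.
; BeginPlay adds the default Enhanced Input mapping context.
; Each tick, MouseTick polls IA_Look and skips both yaw and pitch input when the predicted yaw falls in the rear half, printing that yaw for debugging.
; The Arrow then copies control rotation as relative rotation, with yaw clamped to ±90 degrees.
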(event `self.ReceiveBeginPlay`
  (bind _asplayer_controller (cast `PlayerController` (`self.GetController`)))
  (bind _returnvalue (pcsubsystem `EnhancedInputLocalPlayerSubsystem` _asplayer_controller))
  (`/Engine/EditorBlueprintResources/StandardMacros.IsValid` _returnvalue
    (:`Is Valid`
      (`EnhancedInputSubsystemInterface.AddMappingContext` _returnvalue "/Game/ThirdPerson/Input/IMC_Default.IMC_Default" 0 (struct)))))

(event `EnhancedInput|/Game/ThirdPerson/Input/Actions/IA_Look`
  (params (ActionValue :type "Vector2D Structure") (ElapsedSeconds :type "Float (double-precision)") (TriggeredSeconds :type "Float (double-precision)") (InputAction :type "InputAction Object Reference" :default "/Game/ThirdPerson/Input/Actions/IA_Look.IA_Look")))

(event `self.ReceiveTick`
  (params (DeltaSeconds :type "Float (single-precision)"))
  (bind (_returnvalue_roll _returnvalue_pitch _returnvalue_yaw) (`KismetMathLibrary.BreakRotator` (`self.GetControlRotation`)))
  (bind (_relativerotation_roll _relativerotation_pitch _relativerotation_yaw) (`KismetMathLibrary.BreakRotator` (`SceneComponent.RelativeRotation` (`self.Arrow`))))
  (`self.Mouse Tick`)
  (`SceneComponent.K2_SetRelativeRotation` (`self.Arrow`) (`KismetMathLibrary.MakeRotator` _returnvalue_roll _returnvalue_pitch _returnvalue_yaw) false false)
  (`SceneComponent.K2_SetRelativeRotation` (`self.Arrow`) (`KismetMathLibrary.MakeRotator` _relativerotation_roll _relativerotation_pitch (`KismetMathLibrary.ClampAngle` _relativerotation_yaw -90.0 90.0)) false false))

(event `Mouse Tick`
  (bind (_returnvalue_roll _returnvalue_pitch _returnvalue_yaw) (`KismetMathLibrary.BreakRotator` (`self.GetControlRotation`)))
  (bind (_returnvalue_x _returnvalue_y) (`KismetMathLibrary.BreakVector2D` (`|GetInputActionValue`)))
  (bind _baselookuprate (`self.BaseLookUpRate`))
  (bind _returnvalue (* _returnvalue_x (`self.BaseTurnRate`)))
  (bind _returnvalue_2 (+ _returnvalue_y 0.0))
  (bind _returnvalue_3 (+ _returnvalue _returnvalue_yaw))
  (`KismetSystemLibrary.PrintString` (`KismetStringLibrary.Conv_DoubleToString` _returnvalue_3) true true (struct :`G` 0.66 :`B` 1.0 :`A` 1.0) _returnvalue_3)
  (if (not (or (and (> _returnvalue_3 90.0) (< _returnvalue_3 180.0)) (and (> _returnvalue_3 180.0) (< _returnvalue_3 270.0))))
    (`self.AddControllerYawInput` _returnvalue)
    (if (`self.InvertMouse`)
      (`self.AddControllerPitchInput` (* _returnvalue_2 _baselookuprate))
      (else
        (`self.AddControllerPitchInput` (* (* _returnvalue_2 -1.0) _baselookuprate))))))

(fn `UserConstructionScript`)
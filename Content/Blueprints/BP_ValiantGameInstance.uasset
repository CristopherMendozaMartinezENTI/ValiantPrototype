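; BP_ValiantGameInstance is the game instance that exposes setters for the game's audio and graphics settings.
; Volume setters write to the Master, Music and SFX audio buses.
; Graphics setters build console commands for shadow, texture and foliage quality, screen percentage, anti-aliasing and motion blur.
; Anti-aliasing remaps option 3 to method 4, and motion blur is a simple on/off toggle.
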(fn `SetAntiAliasingMode`
  (params (Value :type Integer))
  (if (== Value 3)
    (`KismetSystemLibrary.ExecuteConsoleCommand` "r.AntiAliasingMethod 4" (`GameplayStatics.GetPlayerController` 0))
    (else
      (`KismetSystemLibrary.ExecuteConsoleCommand` (`KismetStringLibrary.Concat_StrStr` "r.AntiAliasingMethod " (`KismetStringLibrary.Conv_IntToString` Value)) (`GameplayStatics.GetPlayerController` 0)))))

(fn `SetFoliageQuality`
  (params (Value :type Integer))
  (`KismetSystemLibrary.ExecuteConsoleCommand` (`KismetStringLibrary.Concat_StrStr` "FoliageQuality " (`KismetStringLibrary.Conv_IntToString` Value)) (`GameplayStatics.GetPlayerController` 0)))

(fn `SetMasterVolume`
  (params (Value :type "Float (double-precision)"))
  (`FMODBlueprintStatics.BusSetVolume` "/Game/FMOD/Buses/Master.Master" Value))

(fn `SetMotionBlur`
  (params (Enabled :type Boolean))
  (if Enabled
    (`KismetSystemLibrary.ExecuteConsoleCommand` "r.MotionBlurQuality 3" null)
    (else
      (`KismetSystemLibrary.ExecuteConsoleCommand` "r.MotionBlurQuality 0" null))))

(fn `SetMusicVolume`
  (params (Value :type "Float (double-precision)"))
  (`FMODBlueprintStatics.BusSetVolume` "/Game/FMOD/Buses/Master/Music.Music" Value))

(fn `SetScreenPercentage`
  (params (Value :type "Float (double-precision)"))
  (`KismetSystemLibrary.ExecuteConsoleCommand` (`KismetStringLibrary.Concat_StrStr` "r.ScreenPercentage " (`KismetStringLibrary.Conv_DoubleToString` Value)) (`GameplayStatics.GetPlayerController` 0)))

(fn `SetSFXVolume`
  (params (Value :type "Float (double-precision)"))
  (`FMODBlueprintStatics.BusSetVolume` "/Game/FMOD/Buses/Master/SFX.SFX" Value))

(fn `SetShadowQuality`
  (params (Value :type Integer))
  (`KismetSystemLibrary.ExecuteConsoleCommand` (`KismetStringLibrary.Concat_StrStr` "sg.ShadowQuality " (`KismetStringLibrary.Conv_IntToString` Value)) (`GameplayStatics.GetPlayerController` 0)))

(fn `SetTextureQuality`
  (params (Value :type Integer))
  (`KismetSystemLibrary.ExecuteConsoleCommand` (`KismetStringLibrary.Concat_StrStr` "sg.TextureQuality " (`KismetStringLibrary.Conv_IntToString` Value)) (`GameplayStatics.GetPlayerController` 0)))
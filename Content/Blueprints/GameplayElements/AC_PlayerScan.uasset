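; AC_PlayerScan is an actor component that performs an expanding area scan around its owning player.
; ScanArea attaches the NS_Scan effect to the owner's Character mesh and tweens a sphere trace radius up to Radius with smoothstep easing.
; Each tween update multi-traces at the owner's location with one-frame debug drawing, calling ScanResponse on hit actors' AC_ScanObjetive components, so targets can respond repeatedly during one scan.
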(event `ScanArea`
  (bind _returnvalue (`Actor.K2_GetActorLocation` (`self.GetOwner`)))
  (`self.SpawnVFX`)
  (bind (_asynctaskproxy _value) (`FCTweenBPActionFloat.TweenFloat` 0.0 (`self.Radius`) 1.0 "Smoothstep")
    (:`ApplyEasing`
      (bind (_outhits _returnvalue_2) (`KismetSystemLibrary.SphereTraceMulti` :`Start` _returnvalue :`End` _returnvalue :`Radius` _value :`TraceChannel` "TraceTypeQuery5" :`DrawDebugType` "ForOneFrame"))
      (if _returnvalue_2
        (for _array_element _outhits
          (bind _returnvalue_3 (`Actor.GetComponentByClass` (`.HitActor` (`GameplayStatics.BreakHitResult` _array_element)) "/Game/Blueprints/GameplayElements/AC_ScanObjetive.AC_ScanObjetive_C"))
          (`/Engine/EditorBlueprintResources/StandardMacros.IsValid` _returnvalue_3
            (:`Is Valid`
              (`/Game/Blueprints/GameplayElements/AC_ScanObjetive.ScanResponse` _returnvalue_3))))))))

(fn `SpawnVFX`
  (bind _ascharacter (cast `Character` (`self.GetOwner`)))
  (`NiagaraFunctionLibrary.SpawnSystemAttached` "/Game/VFX/VFX/ScanVFx/VFX/NS_Scan.NS_Scan" (`Character.Mesh` _ascharacter) "None" (0.0 0.0 0.0) (struct) "KeepRelativeOffset"))
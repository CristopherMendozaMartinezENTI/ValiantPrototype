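; Component that shows a timed on-screen navigation icon for its owning actor when it gets scanned.
; If scanning is allowed, it creates a GUI_NavigationIcon widget targeting the owner's root component, or reactivates the cached one.
; A Delay then hides and deactivates the icon after Duration, with a DoOnce gating reactivation until that reset.
; Disabling scannability hides the icon immediately.
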(event `self.ReceiveBeginPlay`)

(event `self.ReceiveTick`
  (params (DeltaSeconds :type "Float (single-precision)")))

(event `AddIcon`
  (bind _iconref (`self.IconRef`))
  (bind _rootcomponent (`Actor.RootComponent` (`self.GetOwner`)))
  (if (`self.IsScaneable`)
    (`/Engine/EditorBlueprintResources/StandardMacros.IsValid` _rootcomponent
      (:`Is Valid`
        (`/Engine/EditorBlueprintResources/StandardMacros.IsValid` (`self.IconRef`)
          (:`Is Valid`
            (`/Engine/EditorBlueprintResources/StandardMacros.DoOnce` false :!label _label
              (:`Completed`
                (set `/Game/Blueprints/GameplayElements/Scan/NavigationIcons/Blueprints/GUI_NavigationIcon.Active` true _iconref)
                (`Widget.SetVisibility` _iconref "HitTestInvisible"))))
          (:`Is Not Valid`
            (bind _returnvalue (`|CreateWidget` "/Game/Blueprints/GameplayElements/Scan/NavigationIcons/Blueprints/GUI_NavigationIcon.GUI_NavigationIcon_C" null _rootcomponent (`self.Active`) (`self.ImageInfo`) (`self.TextInfo`) (`self.MovInfo`)))
            (bind _output_get (set `self.IconRef` _returnvalue))
            (`UserWidget.AddToViewport` _output_get 0)))
        (`KismetSystemLibrary.Delay` (`self.Duration`))
        (`self.RemoveIcon`)
        (goto _label :!via `Reset`)))))

(event `RemoveIcon`
  (bind _iconref (`self.IconRef`))
  (`/Engine/EditorBlueprintResources/StandardMacros.IsValid` _iconref
    (:`Is Valid`
      (set `/Game/Blueprints/GameplayElements/Scan/NavigationIcons/Blueprints/GUI_NavigationIcon.Active` false _iconref)
      (`Widget.SetVisibility` _iconref "Hidden"))))

(event `SetIsScaneable`
  (params (IsScaneable :type Boolean))
  (bind _output_get (set `self.IsScaneable` IsScaneable))
  (if (not _output_get)
    (`self.RemoveIcon`)))

(event `/Game/Blueprints/GameplayElements/Scan/NavigationIcons/Blueprints/I_Scanable.OnGetScaned`
  (`self.AddIcon`))
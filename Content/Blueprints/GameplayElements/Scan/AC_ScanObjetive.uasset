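; Actor component that marks its owner as a scan objective and plays Niagara feedback when a scan hits it.
; ScanResponse, gated by the IsScanable flag, attaches a beacon effect to the owner's root, plus a raised respond effect if IsEntity is set.
; A DoOnce reset after a delay throttles repeat responses, and SetIsScanable toggles whether the owner responds.
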(event `self.ReceiveBeginPlay`)

(event `ScanResponse`
  (if (`self.IsScanable`)
    (`/Engine/EditorBlueprintResources/StandardMacros.DoOnce` false :!label _label
      (:`Completed`
        (if (`self.IsEntity`)
          (`NiagaraFunctionLibrary.SpawnSystemAttached` "/Game/VFX/VFX/ScanVFx/VFX/NS_Scan_Respond.NS_Scan_Respond" (`Actor.RootComponent` (`self.GetOwner`)) "None" (0.0 0.0 20.0) (struct) "KeepRelativeOffset"))
        (`NiagaraFunctionLibrary.SpawnSystemAttached` "/Game/VFX/VFX/ScanVFx/VFX/NS_Beacons.NS_Beacons" (`Actor.RootComponent` (`self.GetOwner`)) "None" (0.0 0.0 0.0) (struct) "KeepRelativeOffset")
        (`KismetSystemLibrary.Delay` 5.0)
        (goto _label :!via `Reset`)))))

(event `SetIsScanable`
  (params (IsScanable :type Boolean))
  (set `self.IsScanable` IsScanable))
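; Scene component that marks a scannable point for the scan overlay, exposing its location, active state and visibility as indicator data.
; It registers with BP_ScanOverlay_Manager when the camera is within range and fades visibility smoothly by distance.
; Beyond the turn-off distance it unregisters and throttles its tick to a random longer interval to save cost.
; Scan responses activate it if scannable, while changing scannability sets its active state directly.
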(event `self.ReceiveBeginPlay`
  ;[1 1 1] Get HUD Overlay Actor
  (bind _returnvalue (`GameplayStatics.GetActorOfClass` "/Game/Blueprints/GameplayElements/Scan/ScanOverlay/Blueprints/BP_ScanOverlay_Manager.BP_ScanOverlay_Manager_C"))
  (set `self.ScanOverlayActor` _returnvalue))

(event `self.ReceiveTick`
  (params (DeltaSeconds :type "Float (single-precision)"))
  (bind _scanoverlayactor (`self.ScanOverlayActor`))
  (bind _returnvalue (`KismetMathLibrary.VSize` (- (`self.K2_GetComponentLocation`) (`self.CameraLocation`))))
  ;[1 1 1] Event Tick happens every frame only if Scan Overlay is close to Player. In other case it sleep and tick once in couple of seconds
  (`|ExecutionSequence`
    (:`then_0`
      ;;[1 1 1] Get Discance to active Camera Component (or Pawn) and deside if this component should tick every frame or turn off
      (bind _returnvalue_2 (`/Game/Blueprints/GameplayElements/Scan/ScanOverlay/Blueprints/BP_ScanOverlay_Manager.GetCameraLocation` (`self.ScanOverlayActor`)))
      (set `self.CameraLocation` _returnvalue_2)
      (if (< (`KismetMathLibrary.VSize` (- (`self.K2_GetComponentLocation`) (`self.CameraLocation`))) (`self.TurnOffDistance`))
        ;;[1 1 1] Go to Active Mode - Add component to active list (inside BP_ScanOverlay_Manager) and get Min, Max and TurnOff distances
        (if (`self.TurnOffMode`)
          (set `self.TurnOffMode` false)
          (bind (_visibledistancemax _visibledistancemin _sleepdistance) (`/Game/Blueprints/GameplayElements/Scan/ScanOverlay/Blueprints/BP_ScanOverlay_Manager.Add Edge Component` _scanoverlayactor self))
          (set `self.VisibleDistanceMax` _visibledistancemax)
          (set `self.VisibleDistanceMin` _visibledistancemin)
          (set `self.TurnOffDistance` _sleepdistance)
          (`self.SetComponentTickInterval` 0.0)
          (set `self.TargetVisibility` 0.0))
        (else
          ;;[1 1 1] Set to TurnOff Mode
          (if (not (`self.TurnOffMode`))
            (set `self.TurnOffMode` true)
            (`/Game/Blueprints/GameplayElements/Scan/ScanOverlay/Blueprints/BP_ScanOverlay_Manager.RemoveEdgeComponent` _scanoverlayactor self)
            (`self.SetComponentTickInterval` (`KismetMathLibrary.RandomFloatInRange` (`self.TurnOff Tick Interval Min`) (`self.TurnOff Tick Interval Max`)))))))
    (:`then_1`
      (if (not (`self.TurnOffMode`))
        ;;[1 1 1] If this Component is not in TurnOff Mode, update visibility (ie Opacity) if needed
        (set `self.Delta Seconds` DeltaSeconds)
        (if (> _returnvalue (`self.VisibleDistanceMax`))
          (set `self.TargetVisibility` 0.0)
          (else
            (set `self.TargetVisibility` (`KismetMathLibrary.MapRangeClamped` (`KismetMathLibrary.FClamp` _returnvalue (`self.VisibleDistanceMin`) (`self.VisibleDistanceMax`)) (`self.VisibleDistanceMin`) (`self.VisibleDistanceMax`) 1.0))))
        (if (!= (`self.CurrentVisibility`) (`self.TargetVisibility`))
          (set `self.CurrentVisibility` (`KismetMathLibrary.FInterpTo` (`self.CurrentVisibility`) (`self.TargetVisibility`) (`self.Delta Seconds`) 5.0)) ; Slowly change Visibility over time
        )))))

(event `self.ReceiveEndPlay`
  (params (EndPlayReason :type "EEndPlayReason Enum" :default "Destroyed"))
  ;[1 1 1] End of Play
  (`/Game/Blueprints/GameplayElements/Scan/ScanOverlay/Blueprints/BP_ScanOverlay_Manager.RemoveEdgeComponent` (`self.ScanOverlayActor`) self))

(event `ScanResponse`
  (if (`self.IsScanable`)
    (set `self.Active` true)))

(event `SetIsScanable`
  (params (IsScanable :type Boolean))
  (bind _output_get (set `self.IsScanable` IsScanable))
  (set `self.Active` _output_get))

(fn `GetIndicatorData`
  (returns (Location :type "Vector Structure") (Active :type Boolean) (CurrentVisibility :type "Float (double-precision)"))
  (return (`self.K2_GetComponentLocation`) (`self.Active`) (`self.CurrentVisibility`)))
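; Scan overlay manager that draws screen-edge indicators for off-screen scan targets into a render target.
; Components register through AddEdgeComponent, receive shared distance settings and supply location, active state and visibility.
; Each Tick clears the target, projects active components to screen, then draws a rotated texture clamped to the nearest edge, faded by visibility.
; Points that fail projection are mirrored across the camera plane and reprojected.
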(event `self.ReceiveBeginPlay`
  ;[1 1 1] Set Scan Overlay Component Instances on HUD
  ;;[1 0.005858 0] Get Camera Component (if Pawn have one) and Player Controller reference
  (`self.UpdateCameraReference`)
  (set `self.PlayerController` (`GameplayStatics.GetPlayerController` 0))
  ;;[1 0.3203 0] Get HUD Overlay Texture Size
  (bind _astexture_2d (cast `Texture2D` (`self.ScanOverlayTexture`)))
  (set `self.IndicatorTextureSize` (`KismetMathLibrary.Conv_IntToDouble` (`Texture2D.Blueprint_GetSizeX` _astexture_2d)))
  ;;[0.2102 1 0] Calculate offsets depending on HUD Overlay texture size
  (set `self.TextureShift_Left` (`KismetMathLibrary.MakeVector2D` 0.0 (* (`self.IndicatorTextureSize`) -1.0)))
  (set `self.TextureShift_Right` (`KismetMathLibrary.MakeVector2D` 0.0 (`self.IndicatorTextureSize`)))
  (set `self.TextureShift_Up` (`KismetMathLibrary.MakeVector2D` (`self.IndicatorTextureSize`)))
  (set `self.TextureShift_Down` (`KismetMathLibrary.MakeVector2D` (* (`self.IndicatorTextureSize`) -1.0))))

(event `self.ReceiveTick`
  (params (DeltaSeconds :type "Float (single-precision)"))
  (bind _returnvalue (`GameplayStatics.GetPlayerCameraManager` 0))
  (bind _cameracomponentref (`self.CameraComponentRef`))
  (bind _cameracomponentref_2 (`self.CameraComponentRef`))
  (bind _returnvalue_2 (- (/ (`self.Screen Position`) (`WidgetLayoutLibrary.GetViewportSize`)) (0.5 0.5)))
  (bind _returnvalue_3 (`KismetMathLibrary.GetAbsMax2D` _returnvalue_2))
  ;[1 1 1] Update Scan Overlay Component Instances on HUD
  (`|ExecutionSequence`
    (:`then_0`
      ;;[0 0.9626 1] Get camera Location and Forward vector
      (if (and (!= _cameracomponentref_2 null) (`KismetSystemLibrary.IsValid` _cameracomponentref_2))
        (set `self.CameraLocation` (`SceneComponent.K2_GetComponentLocation` _cameracomponentref))
        (set `self.CameraForwardVector` (`SceneComponent.GetForwardVector` _cameracomponentref))
        (else
          (set `self.CameraLocation` (`PlayerCameraManager.GetCameraLocation` _returnvalue))
          (set `self.CameraForwardVector` (`SceneComponent.GetForwardVector` (`PlayerCameraManager.TransformComponent` _returnvalue))))))
    (:`then_1`
      (`KismetRenderingLibrary.ClearRenderTarget2D` "/Game/Blueprints/GameplayElements/Scan/ScanOverlay/RenderTargets/RT_Scan_Overlay.RT_Scan_Overlay" (struct)) ; RT must be clean even if there is no Edge Indicators visible
      (set `self.CameraPlane` (`KismetMathLibrary.MakePlaneFromPointAndNormal` (`self.CameraLocation`) (`self.CameraForwardVector`)))
      (if (> (`KismetArrayLibrary.Array_Length` (`self.ScanOverlayComponents`)) 0)
        ;;[1 0.4871 0.0636] Draw to RenderTexture
        (bind (_canvas _size _context) (`KismetRenderingLibrary.BeginDrawCanvasToRenderTarget` "/Game/Blueprints/GameplayElements/Scan/ScanOverlay/RenderTargets/RT_Scan_Overlay.RT_Scan_Overlay"))
        (set `self.Canvas` _canvas)
        (set `self.Size` _size)
        (set `self.Context` _context)
        ;;[1 0.7014 0.528] Calculate screen position and discance, decide if we need to draw HUD Overlay to Render Texture
        (for _array_element (`self.ScanOverlayComponents`)
          (bind (_location _active _currentvisibility) (`/Game/Blueprints/GameplayElements/Scan/ScanOverlay/Blueprints/BP_ScanOverlay_Component.GetIndicatorData` _array_element)) ; We need to know Location, Visibility (0-1 value) and if this component is Active
          (if _active
            (set `self.CurrentVisibility` _currentvisibility)
            (bind (_screenposition _returnvalue_4) (`GameplayStatics.ProjectWorldToScreen` (`self.PlayerController`) _location))
            (if _returnvalue_4
              (set `self.Screen Position` _screenposition)
              (if (> _returnvalue_3 0.52)
                (bind _output_get (set `self.ScreenPosUV` (/ _returnvalue_2 (`KismetMathLibrary.MakeVector2D` _returnvalue_3 _returnvalue_3)) :!label _label))
                (bind (_x _y) (`KismetMathLibrary.BreakVector2D` _output_get))
                ;;[0.5202 1 0.5194] Select rotation and additional shift depending on screen indicator location
                (if (== _x -1.0)
                  (set `self.IndicatorRotation` 0.0)
                  (set `self.AdditionalShift` (`self.TextureShift_Left`))
                  (elif (== _x 1.0)
                    (set `self.IndicatorRotation` 180.0)
                    (set `self.AdditionalShift` (`self.TextureShift_Right`))
                    (elif (== _y -1.0)
                      (set `self.IndicatorRotation` 90.0)
                      (set `self.AdditionalShift` (`self.TextureShift_Up`))
                      (elif (== _y 1.0)
                        (set `self.IndicatorRotation` -90.0)
                        (set `self.AdditionalShift` (`self.TextureShift_Down`))))))
                ;;[0.4842 0.5991 1] Calculate screen position and draw to Render Target.
                (bind _output_get_2 (set `self.ScreenPositionCalculatedPX` (* (`self.Size`) (+ (* (`self.ScreenPosUV`) (0.5 0.5)) (0.5 0.5))))) ; Calculate screen position in pixels
                (`Canvas.K2_DrawTexture` (`self.Canvas`) (`self.ScanOverlayTexture`) (+ _output_get_2 (`self.AdditionalShift`)) (128.0 512.0) (0.0 0.0) (1.0 1.0) (make `LinearColor` 1.0 1.0 1.0 (`self.CurrentVisibility`)) "BLEND_Translucent" (`self.IndicatorRotation`) (0.0 0.0)) ; Draw to Render Target. Render Target only have R channel
              )
              (else
                (set `self.Screen Position` (`GameplayStatics.ProjectWorldToScreen` (`self.PlayerController`) (`KismetMathLibrary.Vector_MirrorByPlane` _location (`self.CameraPlane`)))) ; Project again using mirrored vector
                (goto _label)))))
        (`KismetRenderingLibrary.EndDrawCanvasToRenderTarget` (`self.Context`))))))

(fn `Add Edge Component`
  (params (EdgeComponent :type "/Game/Blueprints/GameplayElements/Scan/ScanOverlay/Blueprints/BP_ScanOverlay_Component Object Reference (by ref)"))
  (returns (VisibleDistanceMax :type "Float (double-precision)") (VisibleDistanceMin :type "Float (double-precision)") (SleepDistance :type "Float (double-precision)"))
  (`KismetArrayLibrary.Array_Add` (`self.ScanOverlayComponents`) EdgeComponent)
  (return (`self.Visible Distance Max`) (`self.Visible Distance Min`) (`self.TurnOff Distance`)))

(fn `GetCameraLocation`
  (returns (ReturnValue :type "Vector Structure"))
  (return (`self.CameraLocation`)))

(fn `RemoveEdgeComponent`
  (params (EdgeComponent :type "/Game/Blueprints/GameplayElements/Scan/ScanOverlay/Blueprints/BP_ScanOverlay_Component Object Reference (by ref)"))
  (`KismetArrayLibrary.Array_RemoveItem` (`self.ScanOverlayComponents`) EdgeComponent))

(fn `UpdateCameraReference`
  (set `self.CameraComponentRef` (`self.GetComponentByClass` (`Controller.K2_GetPawn` (`GameplayStatics.GetPlayerController` 0)) "/Script/Engine.CameraComponent")))

(fn `UserConstructionScript`)
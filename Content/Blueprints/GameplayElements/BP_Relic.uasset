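; Collectible relic that flies to the player and disappears once picked up.
; Overlapping its sphere with BP_PlayerCharacter attaches a Niagara effect to the player's mesh, plays a 2D pickup sound, removes the sphere and sets a Collected flag.
; Tick then eases the relic toward player 0 with VInterpTo and destroys it when close.
; No score or inventory update happens in this Blueprint.
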(event `self.ReceiveTick`
  (params (DeltaSeconds :type "Float (single-precision)"))
  (bind _returnvalue (`self.K2_GetActorLocation`))
  (bind _returnvalue_2 (`self.K2_GetActorLocation` (`GameplayStatics.GetPlayerCharacter` 0)))
  (if (`self.Collected`)
    (`self.K2_SetActorLocation` (`KismetMathLibrary.VInterpTo` _returnvalue _returnvalue_2 DeltaSeconds 2.0))
    (if (< (`KismetMathLibrary.VSize` (- _returnvalue_2 _returnvalue)) 120.0)
      (`self.K2_DestroyActor`))))

(event `self.Sphere.OnComponentBeginOverlap`
  (params (OverlappedComponent :type "PrimitiveComponent Object Reference") (OtherActor :type "Actor Object Reference") (OtherComp :type "PrimitiveComponent Object Reference") (OtherBodyIndex :type Integer) (bFromSweep :type Boolean) (SweepResult :type "HitResult Structure (by ref)"))
  (bind _asbp_player_character (cast `/Game/Blueprints/PlayerCharacter/BP_PlayerCharacter` OtherActor))
  (`NiagaraFunctionLibrary.SpawnSystemAttached` "/Game/VFX/VFX/ScanVFx/VFX/NS_GetCollectable.NS_GetCollectable" (`Character.Mesh` _asbp_player_character) "None" (0.0 0.0 0.0) (struct) "KeepRelativeOffset")
  (`FMODBlueprintStatics.PlayEvent2D` "/Game/FMOD/Events/SFX/Collectables/Collectable_PickUp.Collectable_PickUp")
  (`ActorComponent.K2_DestroyComponent` (`self.Sphere`))
  (set `self.Collected` true))

(fn `UserConstructionScript`)
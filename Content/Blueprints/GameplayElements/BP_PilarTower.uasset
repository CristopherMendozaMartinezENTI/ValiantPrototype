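; Pillar tower actor that moves vertically and glows when the player character bumps into it.
; A hit with a near-zero vertical impulse plays a Timeline that offsets the mesh downward, with a flag blocking retriggers until it finishes.
; The same hit tweens the emissive color up on a dynamic material instance created at BeginPlay.
; When the player ends overlap with a second mesh component, another tween fades the glow to black.
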(event `self.ReceiveBeginPlay`
  (bind _returnvalue (`PrimitiveComponent.CreateDynamicMaterialInstance` (`self.SM_PilatTower`) 0 null "None"))
  (set `self.DynMat` _returnvalue)
  (`MaterialInstanceDynamic.SetVectorParameterValue` (`self.DynMat`) "EmisiveColor" (`KismetMathLibrary.LinearColorLerp` (struct :`A` 1.0) (struct :`R` 20.0 :`G` 10.112405 :`B` 0.978813 :`A` 1.0))))

(event `self.SM_PilatTower.OnComponentHit`
  (params (HitComponent :type "PrimitiveComponent Object Reference") (OtherActor :type "Actor Object Reference") (OtherComp :type "PrimitiveComponent Object Reference") (NormalImpulse :type "Vector Structure") (Hit :type "HitResult Structure (by ref)"))
  (bind (_relativelocation_x _relativelocation_y _relativelocation_z) (`KismetMathLibrary.BreakVector` (`SceneComponent.RelativeLocation` (`self.SM_PilatTower`))))
  (cast `/Game/Blueprints/PlayerCharacter/BP_PlayerCharacter` OtherActor)
  (if (and (< (`KismetMathLibrary.Abs` (`KismetMathLibrary.Dot_VectorVector` NormalImpulse (0.0 0.0 1.0))) 0.2) (not (`self.Animating`)))
    (set `self.Animating` true)
    (set `self.Relative Location Z` _relativelocation_z)
    (`|ExecutionSequence`
      (:`then_0`
        (bind (_direction _alpha _newtrack_0) (`Timeline|Timeline` :!via `PlayFromStart`)
          (:`Update`
            (`SceneComponent.K2_SetRelativeLocation` (`self.SM_PilatTower`) (`KismetMathLibrary.MakeVector` 0.0 0.0 (`KismetMathLibrary.Lerp` 0.0 -25.0 _alpha)) false false))
          (:`Finished`
            (set `self.Animating` false))))
      (:`then_1`
        (bind (_asynctaskproxy _value) (`FCTweenBPActionFloat.TweenFloat` 0.0 5.0 0.25)
          (:`ApplyEasing`
            (`MaterialInstanceDynamic.SetVectorParameterValue` (`self.DynMat`) "EmisiveColor" (`KismetMathLibrary.LinearColorLerp` (struct :`A` 1.0) (struct :`R` 10.0 :`G` 5.056202 :`B` 0.489407 :`A` 1.0) _value))))))))

(event `self.SM_PilatTower1.OnComponentEndOverlap`
  (params (OverlappedComponent :type "PrimitiveComponent Object Reference") (OtherActor :type "Actor Object Reference") (OtherComp :type "PrimitiveComponent Object Reference") (OtherBodyIndex :type Integer))
  (cast `/Game/Blueprints/PlayerCharacter/BP_PlayerCharacter` OtherActor)
  (bind (_asynctaskproxy _value) (`FCTweenBPActionFloat.TweenFloat` 1.0 0.0 0.25)
    (:`ApplyEasing`
      (`MaterialInstanceDynamic.SetVectorParameterValue` (`self.DynMat`) "EmisiveColor" (`KismetMathLibrary.LinearColorLerp` (struct :`A` 1.0) (struct :`R` 20.0 :`G` 10.112405 :`B` 0.978813 :`A` 1.0) _value)))))

(fn `UserConstructionScript`)
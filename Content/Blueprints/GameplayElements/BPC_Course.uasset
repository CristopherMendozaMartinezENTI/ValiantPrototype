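; Course component that runs a countdown for a timed course of torus checkpoints, adding bonus time on pass-throughs.
; On BeginPlay it binds to every non-start Bp_CourseTorus, so passing through extends the time and the end-of-course event stops the timer.
; StartCountdown creates the UW_CourseCounter widget and a looping millisecond timer that decrements the Timespan and updates its text.
; Time bonuses punch the widget, and Reset restores the starting time.
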(event `self.ReceiveBeginPlay`
  (set `self.StartingTime` (`self.Timespan`))
  (bind _outactors (`GameplayStatics.GetAllActorsOfClass` "/Game/Blueprints/GameplayElements/Bp_CourseTorus.Bp_CourseTorus_C"))
  (for _array_element _outactors
    (if (not (`/Game/Blueprints/GameplayElements/Bp_CourseTorus.CourseStart` _array_element))
      (add `/Game/Blueprints/GameplayElements/Bp_StaminaTorus.OnPassthrough` _array_element (delegate `AddSum`))
      (add `/Game/Blueprints/GameplayElements/Bp_CourseTorus.OnEndCourse` _array_element (delegate `EndCourse`)))))

(event `EndCourse`
  (bind _timer (`self.Timer`))
  (`KismetSystemLibrary.K2_PauseTimerHandle` _timer)
  (`KismetSystemLibrary.K2_ClearAndInvalidateTimerHandle` _timer))

(event `self.ReceiveTick`
  (params (DeltaSeconds :type "Float (single-precision)")))

(event `AddSum`
  (params (Torus :type "/Game/Blueprints/GameplayElements/Bp_StaminaTorus Object Reference"))
  (`self.AddPlus` (`KismetMathLibrary.MakeTimespan` 0 0 0 20)))

(event `StartCountdown`
  (`self.Widget`
    (:`then`
      _)
    (:`else`
      (bind _returnvalue (`|CreateWidget` "/Game/Blueprints/GameplayElements/UW_CourseCounter.UW_CourseCounter_C"))
      (set `self.Widget` _returnvalue)
      (`UserWidget.AddToViewport` _returnvalue 0)))
  (bind _returnvalue_2 (`KismetSystemLibrary.K2_SetTimerDelegate` (delegate `AddCount`) 0.001 true))
  (set `self.Timer` _returnvalue_2))

(event `AddCount`
  (bind _output_get (set `self.Timespan` (- (`self.Timespan`) (`KismetMathLibrary.MakeTimespan` 0 0 0 0 1))))
  (`TextBlock.SetText` (`/Game/Blueprints/GameplayElements/UW_CourseCounter.TextBlock_0` (`self.Widget`)) (`KismetTextLibrary.Conv_StringToText` (`KismetStringLibrary.Concat_StrStr` (`KismetStringLibrary.Conv_IntToString` (`KismetMathLibrary.GetMinutes` _output_get)) ":" (`KismetStringLibrary.Conv_IntToString` (`KismetMathLibrary.GetSeconds` _output_get)) ":" (`KismetStringLibrary.Conv_IntToString` (`KismetMathLibrary.GetMilliseconds` _output_get))))))

(event `AddPlus`
  (params (`Time to add` :type "Timespan Structure"))
  (set `self.Timespan` (+ (`self.Timespan`) `Time to add`))
  (`/Game/Blueprints/GameplayElements/UW_CourseCounter.Punch` (`self.Widget`)))

(event `Reset`
  (set `self.Timespan` (`self.StartingTime`)))
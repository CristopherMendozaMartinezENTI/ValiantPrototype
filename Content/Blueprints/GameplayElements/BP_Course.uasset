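; Timed ring course that the player runs by passing through toruses placed along a spline.
; The construction script spawns Bp_CourseTorus child actors at spline points flagged in PointHasTorus.
; Each passthrough closes that ring, opens the next and tweens a Niagara fairy-orb lightball along the spline toward it.
; The first ring starts the BPC_Course countdown; on timeout, the player fades out, teleports to the start and the first ring reopens.
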(event `self.ReceiveBeginPlay`
  (bind _coursetorus (`self.CourseTorus`))
  (`|ExecutionSequence`
    (:`then_0`
      (if (`self.StartClosed`)
        (`/Game/Blueprints/GameplayElements/Bp_StaminaTorus.CloseRing` (`|GetArrayItem` (`self.CourseTorus`)))))
    (:`then_1`
      (set `/Game/Blueprints/GameplayElements/BPC_Course.Timespan` (`KismetMathLibrary.MakeTimespan` 0 0 (`self.Minutes`) (`self.Seconds`)) (`self.BPC_Course`))
      (for _array_element (`self.CourseTorus`)
        (add `/Game/Blueprints/GameplayElements/Bp_StaminaTorus.OnPassthrough` _array_element (delegate `StartLightball`))
        (add `/Game/Blueprints/GameplayElements/Bp_StaminaTorus.OnPassthrough` _array_element (delegate `StartCourse`)))
      (add `/Game/Blueprints/GameplayElements/Bp_CourseTorus.OnEndCourse` (`|GetArrayItem` _coursetorus (`KismetArrayLibrary.Array_LastIndex` _coursetorus)) (delegate `EndCourse`)))
    (:`then_2`
      (`NiagaraComponent.SetVariableFloat` (`self.NS_FairyOrb`) "Alpha" 0.0)
      (`SceneComponent.SetVisibility` (`self.Lightball`) true false))))

(event `EndCourse`
  (`/Game/Blueprints/GameplayElements/BPC_Course.EndCourse` (`self.BPC_Course`))
  (`KismetSystemLibrary.PrintString` "Hello"))

(event `StartCourse`
  (params (Torus :type "/Game/Blueprints/GameplayElements/Bp_StaminaTorus Object Reference"))
  (bind _asbp_course_torus (cast `/Game/Blueprints/GameplayElements/Bp_CourseTorus` Torus :!pure true))
  (bind _output (`|GetArrayItem` (`self.CourseTorus`) (`KismetMathLibrary.Clamp` (+ (`KismetArrayLibrary.Array_Find` (`self.CourseTorus`) _asbp_course_torus) 1) 0 (`KismetArrayLibrary.Array_Length` (`self.CourseTorus`)))))
  (if (== (`KismetArrayLibrary.Array_Find` (`self.CourseTorus`) _asbp_course_torus) 0)
    (`/Game/Blueprints/GameplayElements/BPC_Course.StartCountdown` (`self.BPC_Course`)))
  (if (`KismetSystemLibrary.IsValid` _output)
    (`/Game/Blueprints/GameplayElements/Bp_StaminaTorus.OpenRing` _output)
    (`/Game/Blueprints/GameplayElements/Bp_StaminaTorus.CloseRing` Torus)
    (else
      (`/Game/Blueprints/GameplayElements/BPC_Course.EndCourse` (`self.BPC_Course`))
      (`SceneComponent.SetVisibility` (`self.Lightball`) false true)
      (`self.OnEndCourse`))))

(event `StartLightball`
  (params (Torus :type "/Game/Blueprints/GameplayElements/Bp_StaminaTorus Object Reference"))
  (bind _asbp_course_torus (cast `/Game/Blueprints/GameplayElements/Bp_CourseTorus` Torus :!pure true))
  (bind _lightball (`self.Lightball`))
  (bind _value (`BlueprintMapLibrary.Map_Find` (`self.PointsToCouseTorus`) _asbp_course_torus))
  (bind _returnvalue (`SplineComponent.GetDistanceAlongSplineAtSplinePoint` (`self.Spline`) _value))
  (bind _returnvalue_2 (`SplineComponent.GetDistanceAlongSplineAtSplinePoint` (`self.Spline`) (`self.GetNextPossibleTorus` (+ _value 1))))
  (if (not (`/Game/Blueprints/GameplayElements/Bp_CourseTorus.CourseEnd` _asbp_course_torus))
    (`SceneComponent.SetVisibility` (`self.Lightball`) true false)
    (`NiagaraComponent.SetVariableFloat` (`self.NS_FairyOrb`) "Alpha" 1.0)
    (bind (_asynctaskproxy _value_2) (`FCTweenBPActionFloat.TweenFloat` _returnvalue _returnvalue_2 (/ (- _returnvalue_2 _returnvalue) (`self.LigthballSpeed`)))
      (:`ApplyEasing`
        (bind (_returnvalue_location _returnvalue_rotation) (`KismetMathLibrary.BreakTransform` (`SplineComponent.GetTransformAtDistanceAlongSpline` (`self.Spline`) _value_2 "Local" false)))
        (`SceneComponent.K2_SetRelativeTransform` _lightball (`KismetMathLibrary.MakeTransform` _returnvalue_location _returnvalue_rotation (`SceneComponent.RelativeScale3D` _lightball)) false false))
      (:`OnComplete`
        (`SceneComponent.SetVisibility` (`self.Lightball`) false false)
        (`NiagaraComponent.SetVariableFloat` (`self.NS_FairyOrb`) "Alpha" 0.0)))))

(event `ResetAll`
  (bind _returnvalue (`GameplayStatics.GetPlayerController` 0))
  (bind _returnvalue_2 (`GameplayStatics.GetPlayerCharacter` 0))
  (bind _startingplayerlocation (`self.StartingPlayerLocation`))
  (`/Engine/EditorBlueprintResources/StandardMacros.DoOnce` false :!label _label
    (:`Completed`
      (set `MovementComponent.Velocity` (0.0 0.0 0.0) (`Character.CharacterMovement` _returnvalue_2))
      (`self.DisableInput` _returnvalue_2 _returnvalue)
      (`PlayerCameraManager.StartCameraFade` :`self` (`PlayerController.PlayerCameraManager` _returnvalue) :`ToAlpha` 1.0 :`Duration` 0.5 :`bHoldWhenFinished` true)
      (`KismetSystemLibrary.Delay` 0.6)
      (`self.K2_TeleportTo` _returnvalue_2 (`SceneComponent.K2_GetComponentLocation` _startingplayerlocation) (`SceneComponent.K2_GetComponentRotation` _startingplayerlocation))
      (set `/Game/Blueprints/GameplayElements/BPC_Course.Timespan` (`KismetMathLibrary.MakeTimespan` 0 0 (`self.Minutes`) (`self.Seconds`)) (`self.BPC_Course`))
      (`KismetSystemLibrary.Delay` 0.2)
      (`PlayerCameraManager.StartCameraFade` :`self` (`PlayerController.PlayerCameraManager` _returnvalue) :`FromAlpha` 1.0 :`Duration` 0.5)
      (`self.EnableInput` (`GameplayStatics.GetPlayerCharacter` 0) (`GameplayStatics.GetPlayerController` 0))
      (`/Game/Blueprints/GameplayElements/Bp_StaminaTorus.OpenRing` (`|GetArrayItem` (`self.CourseTorus`)))
      (goto _label :!via `Reset`))))

(event `self.BPC_Course.CountdownEnded`
  (`self.ResetAll`))

(event `OpenCourse`
  (`/Game/Blueprints/GameplayElements/Bp_StaminaTorus.Activate` (`|GetArrayItem` (`self.CourseTorus`))))

(event `DestroyCourse`
  (`self.K2_DestroyActor`))

(fn `GetNextPossibleTorus`
  (params (Index :type Integer))
  (returns (indx1 :type Integer))
  (locals (indx :type Integer) (IsLastIndex :type "Array of Boolean"))
  (set `local.indx` Index)
  (while (or (not (`|GetArrayItem` (`self.PointHasTorus`) (`local.indx`))) (>= (`local.indx`) (`KismetArrayLibrary.Array_LastIndex` (`self.PointHasTorus`))))
    (`/Engine/EditorBlueprintResources/StandardMacros.IncrementInt` (`local.indx`)
      (:`  `
        (if (>= (`local.indx`) (`KismetArrayLibrary.Array_LastIndex` (`self.PointHasTorus`)))
          (return (`local.indx`))))))
  (return (`local.indx`)))

(fn `UserConstructionScript`
  (bind _spline (`self.Spline`))
  (bind _returnvalue (`SplineComponent.GetNumberOfSplinePoints` _spline))
  (`KismetArrayLibrary.Array_Clear` (`self.CourseTorus`))
  (`BlueprintMapLibrary.Map_Clear` (`self.PointsToCouseTorus`))
  (for _index (range (+ _returnvalue 1))
    (if (not (`KismetArrayLibrary.Array_IsValidIndex` (`self.PointHasTorus`) _index))
      (`KismetArrayLibrary.Array_Add` (`self.PointHasTorus`) true))
    (if (== _index 0)
      (bind (_returnvalue_inputkey _returnvalue_position _returnvalue_arrivetangent) (break `SplinePoint` (`SplineComponent.GetSplinePointAt` _spline _index "Local")))
      (bind (_returnvalue_inputkey_2 _returnvalue_position_2 _returnvalue_arrivetangent_2 _returnvalue_leavetangent _returnvalue_rotation) (break `SplinePoint` (`SplineComponent.GetSplinePointAt` (`self.Spline`) _index "Local")))
      (bind _returnvalue_2 (`KismetMathLibrary.MakeTransform` _returnvalue_position (`KismetMathLibrary.MakeRotator` (.roll _returnvalue_rotation) (+ (.pitch _returnvalue_rotation) 90.0) (.yaw _returnvalue_rotation))))
      (bind _returnvalue_3 (`AddComponent|NODE_AddChildActorComponent-0` :`RelativeTransform` _returnvalue_2))
      (bind _asbp_course_torus (cast `/Game/Blueprints/GameplayElements/Bp_CourseTorus` (`ChildActorComponent.ChildActor` _returnvalue_3) :!pure true))
      (`KismetArrayLibrary.Array_Add` (`self.CourseTorus`) _asbp_course_torus)
      (`BlueprintMapLibrary.Map_Add` (`self.PointsToCouseTorus`) _asbp_course_torus _index)
      (elif (== _index _returnvalue)
        _
        (elif (`|GetArrayItem` (`self.PointHasTorus`) _index)
          (bind _returnvalue_4 (`AddComponent|NODE_AddChildActorComponent-2` :`RelativeTransform` _returnvalue_2))
          (bind _asbp_course_torus_2 (cast `/Game/Blueprints/GameplayElements/Bp_CourseTorus` (`ChildActorComponent.ChildActor` _returnvalue_4) :!pure true))
          (`KismetArrayLibrary.Array_Add` (`self.CourseTorus`) _asbp_course_torus_2)
          (`BlueprintMapLibrary.Map_Add` (`self.PointsToCouseTorus`) _asbp_course_torus_2 _index)))))
  (set `/Game/Blueprints/GameplayElements/Bp_CourseTorus.CourseEnd` true (`|GetArrayItem` (`self.CourseTorus`) _returnvalue)))
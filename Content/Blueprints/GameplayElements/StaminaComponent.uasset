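; Stamina component that tracks a clamped stamina value, starting at its maximum on BeginPlay.
; Add and Remove functions adjust the value and fire increase or decrease event dispatchers, while getters expose the current amount and whether any remains.
; The run-out check in Remove subtracts the amount again from the updated value, so that dispatcher can fire before stamina reaches zero.
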(event `self.ReceiveBeginPlay`
  (set `self.Current Stamina` (`self.Max Stamina`)))

(fn `Add Stamina`
  (params (`Stamina to add` :type "Float (double-precision)"))
  (set `self.Current Stamina` (`KismetMathLibrary.FClamp` (+ (`self.Current Stamina`) `Stamina to add`) 0.0 (`self.Max Stamina`)))
  (`self.OnIncreaseStamina`))

(fn `Get Current Stamina`
  (returns (`Current Stamina` :type "Float (double-precision)"))
  (return (`self.Current Stamina`)))

(fn `HasAnyStaminaLeft`
  (returns (ReturnValue :type Boolean))
  (return (> (`self.Current Stamina`) 0.0)))

(fn `Remove Stamina`
  (params (`Stamina to remove` :type "Float (double-precision)"))
  (bind _returnvalue (`KismetMathLibrary.FClamp` (- (`self.Current Stamina`) `Stamina to remove`) 0.0 (`self.Max Stamina`)))
  (set `self.Current Stamina` _returnvalue)
  (`self.OnDecreaseStamina`)
  (if (<= _returnvalue 0.0)
    (`self.OnRunOutOfStamina`)))
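; Stamina ring that forms a link in a chain of pass-through rings making up a course.
; On player overlap it plays a sound, fires passthrough events, then tweens itself closed and opens NextRing, or broadcasts CourseFinished when none follows.
; SetOpen and SetClose drive the Niagara ring alpha, wind and leaf spawn rates, and toggle the box's overlap events.
; The construction script applies the initial state from IsOpen.
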(event `self.ReceiveBeginPlay`
  (bind _asbp_player_character (cast `/Game/Blueprints/PlayerCharacter/BP_PlayerCharacter` (`GameplayStatics.GetPlayerCharacter` 0)))
  (set `self.As BP Player Character` _asbp_player_character))

(event `self.ReceiveActorBeginOverlap`
  (params (OtherActor :type "Actor Object Reference"))
  (cast `/Game/Blueprints/PlayerCharacter/BP_PlayerCharacter` OtherActor)
  (`FMODBlueprintStatics.PlayEventAtLocation` "/Game/FMOD/Events/SFX/Props/StaminaRing.StaminaRing" (`self.GetTransform`))
  (`self.Passthrough`)
  (`self.OnPassthrough` self)
  (`KismetSystemLibrary.Delay` 0.2)
  (bind (_asynctaskproxy _value) (`FCTweenBPActionFloat.TweenFloat` 1.0 0.0)
    (:`then`
      (`/Engine/EditorBlueprintResources/StandardMacros.IsValid` (`self.NextRing`)
        (:`Is Valid`
          (bind (_asynctaskproxy_2 _value_2) (`FCTweenBPActionFloat.TweenFloat` 0.0)
            (:`ApplyEasing`
              (`self.SetOpen` (`self.NextRing`) _value_2))))
        (:`Is Not Valid`
          (`self.CourseFinished`))))
    (:`ApplyEasing`
      (`self.SetClose` _value))))

(event `/Game/Blueprints/Interfaces/BPI_FlowActivator.Activate`
  (`self.SetOpen` 1.0))

(event `/Game/Blueprints/Interfaces/BPI_FlowActivator.Deactivate`
  (`self.SetClose` 0.0))

(event `Passthrough`)

(event `OpenRing`
  (bind (_asynctaskproxy _value) (`FCTweenBPActionFloat.TweenFloat` 0.0)
    (:`ApplyEasing`
      (`self.SetOpen` _value))))

(event `CloseRing`
  (bind (_asynctaskproxy _value) (`FCTweenBPActionFloat.TweenFloat` 1.0 0.0)
    (:`ApplyEasing`
      (`self.SetClose` _value))))

(fn `SetClose`
  (params (Alpha :type "Float (double-precision)"))
  (`NiagaraComponent.SetVariableFloat` (`self.Ring`) "Alpha" Alpha)
  (`NiagaraComponent.SetVariableFloat` (`self.Wind`) "Wind_SpawnRate" 0.0)
  (`NiagaraComponent.SetVariableFloat` (`self.Leaves`) "Leaves_SpawnRate" 0.0)
  (set `PrimitiveComponent.bGenerateOverlapEvents` false (`self.Box`)))

(fn `SetOpen`
  (params (Alpha :type "Float (double-precision)"))
  (`NiagaraComponent.SetVariableFloat` (`self.Ring`) "Alpha" Alpha)
  (`NiagaraComponent.SetVariableFloat` (`self.Wind`) "Wind_SpawnRate" 2.0)
  (`NiagaraComponent.SetVariableFloat` (`self.Leaves`) "Leaves_SpawnRate" 25.0)
  (set `PrimitiveComponent.bGenerateOverlapEvents` true (`self.Box`)))

(fn `UserConstructionScript`
  (if (`self.IsOpen`)
    (`self.SetOpen` 1.0)
    (else
      (`self.SetClose` 0.0))))
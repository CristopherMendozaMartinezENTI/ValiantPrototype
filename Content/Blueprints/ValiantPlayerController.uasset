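; Player controller for Valiant that handles game startup, menus and debug keys.
; On BeginPlay it clamps camera pitch, spawns the day-time manager, signals loading finished, loads the FlowSave slot if present and adds the overall UI layout.
; Escape or gamepad Start pushes the pause menu onto that layout's layer stack, while an input action toggles map selection, both pausing the game.
; Debug keys save FlowSave and toggle HDR output.
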(event Input|EnhancedActionEvents|EnhancedInputActionIA_MapSelectionMenu
  (params (ActionValue :type Boolean) (ElapsedSeconds :type Float%20%28double-precision%29) (TriggeredSeconds :type Float%20%28double-precision%29) (InputAction :type Input%20Action%20Object%20Reference :default "/Game/Blueprints/Inputs/IA_MapSelectionMenu.IA_MapSelectionMenu"))
  (bind _returnvalue (Game|GetPlayerController 0))
  (Utilities|FlowControl|FlipFlop
    (:A
      (Utilities|IsValid (Variables|Default|GetMapSelectionWidget)
        (:Is%20Valid
          _)
        (:Is%20Not%20Valid
          (bind _returnvalue_2 (UserInterface|CreateWidget "/Game/UI/WBP_MapSelection.WBP_MapSelection_C" _returnvalue))
          (bind _output_get (Variables|Default|SetMapSelectionWidget _returnvalue_2))))
      (UserInterface|Viewport|AddtoViewport _output_get 0)
      (Input|SetInputModeGameandUI (Game|GetPlayerController 0) (Variables|Default|GetMapSelectionWidget) "LockOnCapture" true false)
      (Game|SetGamePaused true))
    (:B
      (Widget|RemovefromParent (Variables|Default|GetMapSelectionWidget))
      (Input|SetInputModeGameOnly _returnvalue false)
      (Game|SetGamePaused false))))

(event EventBeginPlay
  (bind _returnvalue (Game|GetPlayerCameraManager 0))
  (Utilities|FlowControl|Sequence
    (:then_0
      (Variables|/Script/Engine.PlayerCameraManager|SetViewPitchMax _returnvalue 6e+01)
      (Variables|/Script/Engine.PlayerCameraManager|SetViewPitchMin _returnvalue -6e+01)
      (CallFunction|InitDayTimeManager)
      (Default|CallOnFinishedLoadingGame)
      (bind _returnvalue_2 (SaveGame|DoesSaveGameExist "FlowSave"))
      (if _returnvalue_2
        (bind _returnvalue_3 (SaveGame|LoadGamefromSlot "FlowSave"))
        (Variables|Default|SetFlowSaveGame (.AsBP%20Flow%20Save%20Game (Utilities|Casting|CastToBP_FlowSaveGame _returnvalue_3)))))
    (:then_1
      (bind _returnvalue_4 (UserInterface|CreateWidget "/PMDialogue/W_OverallUILayout.W_OverallUILayout_C"))
      (bind _output_get (Variables|Default|SetOveralWidget _returnvalue_4))
      (UserInterface|Viewport|AddtoViewport _output_get 0))))

(event EventTick
  (params (DeltaSeconds :type Float%20%28single-precision%29)))

(event Input|KeyboardEvents|DebugKeyJ
  (params (Key :type Key%20Structure :default "None") (ActionValue :type Input%20Action%20Value%20Structure))
  (:Pressed
    (SaveGame|SaveGametoSlot (Variables|Default|GetFlowSaveGame) "FlowSave")))

(event Input|KeyboardEvents|DebugKeyH
  (params (Key :type Key%20Structure :default "None") (ActionValue :type Input%20Action%20Value%20Structure))
  (:Pressed
    (Utilities|FlowControl|FlipFlop
      (:A
        (bind _returnvalue (Settings|GetGameUserSettings))
        (Class|GameUserSettings|EnableHDRDisplayOutput _returnvalue (Class|GameUserSettings|SupportsHDRDisplayOutput _returnvalue) 1000)
        (Class|GameUserSettings|ApplySettings _returnvalue true))
      (:B
        (bind _returnvalue_2 (Settings|GetGameUserSettings))
        (Class|GameUserSettings|EnableHDRDisplayOutput _returnvalue_2 false 1000)
        (Class|GameUserSettings|ApplySettings _returnvalue_2 true)))))

(event Input|GamepadEvents|GamepadSpecialRight
  (params (Key :type Key%20Structure :default "None"))
  (:Pressed
    (Default|PushWidgettoLayerStack (Variables|Default|GetOveralWidget) "(TagName=\"UI.Layer.GameMenu\")" "/PMDialogue/Hud/W_PauseMenu.W_PauseMenu_C")
    (Game|SetGamePaused true)
    (Input|SetInputModeUIOnly self 0 "DoNotLock" false)))

(event Input|KeyboardEvents|Escape
  (params (Key :type Key%20Structure :default "None"))
  (:Pressed
    (Default|PushWidgettoLayerStack (Variables|Default|GetOveralWidget) "(TagName=\"UI.Layer.GameMenu\")" "/PMDialogue/Hud/W_PauseMenu.W_PauseMenu_C")
    (Game|SetGamePaused true)
    (Input|SetInputModeUIOnly self 0 "DoNotLock" false)))

(fn ConstructionScript)

(fn InitDayTimeManager
  (bind _returnvalue (Game|SpawnActorfromClass "/Game/Blueprints/TimeManager/BP_DayTimeManager.BP_DayTimeManager_C" (Math|Transform|MakeTransform "0, 0, 0") "Undefined" "MultiplyWithRoot" 0 0))
  (Variables|Default|SetDayTimeManager _returnvalue))

(fn InitGameplaySettings
  (Input|SetInputModeGameOnly self true)
  (Variables|Default|SetbShowMouseCursor false))
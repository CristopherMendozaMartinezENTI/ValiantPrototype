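; Scene component that finds a possible landing point where the player is looking and exposes it through GetPossibleLandPoint.
; Each tick it sphere-traces from the camera to a point along camera forward, offset from the owner, and stores the impact point without checking for a hit.
; Trace and impact are debug-drawn every frame.
; The looking-down pitch check has empty branches, and BeginPlay attaches a static mesh component with no visible further use.
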(event `self.ReceiveBeginPlay`
  (bind _returnvalue (`|AddComponentByClass` (`self.GetOwner`) "/Script/Engine.StaticMeshComponent" false (`self.GetRelativeTransform`)))
  (`self.K2_AttachToComponent` _returnvalue self "None" "SnapToTarget" "SnapToTarget" "SnapToTarget" true))

(event `self.ReceiveTick`
  (params (DeltaSeconds :type "Float (single-precision)"))
  (bind _playercameramanager (`PlayerController.PlayerCameraManager` (`GameplayStatics.GetPlayerController` 0)))
  (if (`self.IsLookingDown`)
    _
    (else
      _))
  (bind _outhit (`KismetSystemLibrary.SphereTraceSingle` :`Start` (`PlayerCameraManager.GetCameraLocation` _playercameramanager) :`End` (+ (`Actor.K2_GetActorLocation` (`self.GetOwner`)) (* (`self.GetForwardVector` (`PlayerCameraManager.TransformComponent` _playercameramanager)) 1000.0)) :`Radius` 100.0 :`TraceChannel` "TraceTypeQuery1" :`DrawDebugType` "ForOneFrame"))
  (bind (_bblockinghit _binitialoverlap _time _distance _location _impactpoint) (`GameplayStatics.BreakHitResult` _outhit))
  (`KismetSystemLibrary.DrawDebugBox` _impactpoint (10.0 10.0 10.0) (struct :`R` 1.0 :`B` 0.084288 :`A` 1.0) (struct) DeltaSeconds)
  (set `self.Impact Point` _impactpoint))

(fn `GetPossibleLandPoint`
  (returns (`Impact Point` :type "Vector Structure"))
  (return (`self.Impact Point`)))

(fn `IsLookingDown`
  (returns (Return :type Boolean))
  (return (< (.pitch (`PlayerCameraManager.GetCameraRotation` (`GameplayStatics.GetPlayerCameraManager` 0))) -10.0)))
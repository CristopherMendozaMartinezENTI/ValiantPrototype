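; Player FSM state for braking the bird character in flight, including the transition down to landing.
; On start it stops dive camera shakes and adjusts post-processing, then each tick applies force against velocity until nearly stopped.
; When slow, a downward trace pulls the bird to the ground and switches it to Walking.
; Brake completion, early release or a dash flap changes state, with completion and dash tweening the pointer widget's opacity.
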(event `/Game/Blueprints/PlayerCharacter/BPI_InputHandler.IA_Brake_Complete`
  (if (not (`self.CompletedBrake`))
    (set `/Game/Blueprints/PlayerCharacter/BP_PlayerCharacter.IsBraking` false (`/Game/Blueprints/PlayerCharacter/BP_PlayerFSM.PlayerCharacter` (`self.FSM`)))
    (set `/Game/Blueprints/PlayerCharacter/BP_PlayerCharacter.BirdFlyingState` "NewEnumerator2" (`/Game/Blueprints/PlayerCharacter/BP_PlayerFSM.PlayerCharacter` (`self.FSM`)))
    (`/Game/Blueprints/PlayerCharacter/BP_PlayerFSM.Change State` (`self.FSM`) "NewEnumerator2")
    (`KismetSystemLibrary.PrintString` "Hello")))

(event `self.Start`
  (`parent.Start`)
  (set `/Game/Blueprints/PlayerCharacter/BP_PlayerCharacter.IsBraking` true (`/Game/Blueprints/PlayerCharacter/BP_PlayerFSM.PlayerCharacter` (`self.FSM`)))
  (set `self.CompletedBrake` false)
  (`CameraShakeSourceComponent.StopAllCameraShakes` (`/Game/Blueprints/PlayerCharacter/BP_PlayerCharacter.Diving Camera Shake` (`/Game/Blueprints/PlayerCharacter/BP_PlayerFSM.PlayerCharacter` (`self.FSM`))) true)
  (setmembers `PostProcessSettings` :`StructRef` (`CameraComponent.PostProcessSettings` (`/Game/Blueprints/PlayerCharacter/BP_PlayerCharacter.PlayerCamera` (`self.Player Character`))) :`DepthOfFieldSensorWidth` 24.0 :`DepthOfFieldSqueezeFactor` 1.0 :`DepthOfFieldFocalDistance` 0.0 :`DepthOfFieldDepthBlurAmount` 0.0 :`DepthOfFieldDepthBlurRadius` 2.0))

(event `self.End`
  (set `/Game/Blueprints/PlayerCharacter/BP_PlayerCharacter.IsBraking` false (`/Game/Blueprints/PlayerCharacter/BP_PlayerFSM.PlayerCharacter` (`self.FSM`)))
  (set `/Game/Blueprints/PlayerCharacter/BP_PlayerCharacter.IsLanding` false (`self.Player Character`)))

(event `self.Tick`
  (bind _player_character (`self.Player Character`))
  (bind _playercharacter (`/Game/Blueprints/PlayerCharacter/BP_PlayerFSM.PlayerCharacter` (`self.FSM`)))
  (bind _velocity (`MovementComponent.Velocity` (`Character.CharacterMovement` (`/Game/Blueprints/PlayerCharacter/BP_PlayerFSM.PlayerCharacter` (`self.FSM`)))))
  (`self.Land`)
  (`/Game/Blueprints/PlayerCharacter/BP_PlayerCharacter.Update Bird Direction` (`/Game/Blueprints/PlayerCharacter/BP_PlayerFSM.PlayerCharacter` (`self.FSM`)))
  (if (`/Game/Blueprints/PlayerCharacter/BP_PlayerCharacter.CloseToGround` _playercharacter)
    _
    (elif (not (and (`self.CompletedBrake`) (not (`/Game/Blueprints/PlayerCharacter/BP_PlayerCharacter.IsLanding` _playercharacter))))
      (`/Game/Blueprints/PlayerCharacter/BP_PlayerCharacter.UpdateCameraFlyingMode` _player_character)
      (`CharacterMovementComponent.AddForce` (`Character.CharacterMovement` _player_character) (* _velocity -50.0))
      (if (<= (`KismetMathLibrary.VSize` _velocity) 50.0)
        (`self.CompleteBrake`)
        (elif (`|EnumEquality` (`/Game/Blueprints/PlayerCharacter/BP_PlayerCharacter.BirdFlyingState` (`/Game/Blueprints/PlayerCharacter/BP_PlayerFSM.PlayerCharacter` (`self.FSM`))) "NewEnumerator0")
          _)))))

(event `CompleteBrake`
  (`/Game/Blueprints/PlayerCharacter/BP_PlayerFSM.Change State` (`self.FSM`) "NewEnumerator2")
  (set `/Game/Blueprints/PlayerCharacter/BP_PlayerCharacter.BirdFlyingState` "NewEnumerator3" (`/Game/Blueprints/PlayerCharacter/BP_PlayerFSM.PlayerCharacter` (`self.FSM`)))
  (set `self.CompletedBrake` true)
  (`KismetSystemLibrary.PrintString` "BRAKED")
  (`self.DeactivatePointer`))

(event `/Game/Blueprints/PlayerCharacter/BPI_InputHandler.IA_Look`
  (params (X :type "Float (double-precision)") (Y :type "Float (double-precision)"))
  (if (`self.CompletedBrake`)
    _
    (else
      _))
  (`Pawn.AddControllerPitchInput` (`/Game/Blueprints/PlayerCharacter/BP_PlayerFSM.PlayerCharacter` (`self.FSM`)) (* Y -1.0))
  (`Pawn.AddControllerYawInput` (`/Game/Blueprints/PlayerCharacter/BP_PlayerFSM.PlayerCharacter` (`self.FSM`)) X))

(event `/Game/Blueprints/PlayerCharacter/BPI_InputHandler.IA_Dash_Trigger`
  (`/Game/Blueprints/PlayerCharacter/BP_PlayerCharacter.Flap` (`/Game/Blueprints/PlayerCharacter/BP_PlayerFSM.PlayerCharacter` (`self.FSM`)))
  (`self.ActivatePointer`)
  (`/Game/Blueprints/PlayerCharacter/BP_PlayerFSM.Change State` (`self.FSM`) "NewEnumerator2"))

(fn `Land`
  (bind _returnvalue (`Actor.K2_GetActorLocation` (`self.Player Character`)))
  (if (< (`KismetMathLibrary.VSize` (`MovementComponent.Velocity` (`Character.CharacterMovement` (`self.Player Character`)))) 1000.0)
    (bind (_outhit _returnvalue_2) (`KismetSystemLibrary.LineTraceSingle` :`Start` _returnvalue :`End` (+ _returnvalue (0.0 0.0 -350.0)) :`TraceChannel` "TraceTypeQuery1" :`DrawDebugType` "ForOneFrame" :`TraceColor` (struct :`R` 0.674571 :`B` 1.0 :`A` 1.0)))
    (if _returnvalue_2
      (set `/Game/Blueprints/PlayerCharacter/BP_PlayerCharacter.IsLanding` true (`self.Player Character`))
      (if (< (`.Distance` (`GameplayStatics.BreakHitResult` _outhit)) 25.0)
        (`CharacterMovementComponent.SetMovementMode` (`Character.CharacterMovement` (`self.Player Character`)) "MOVE_Walking" 0)
        (set `/Game/Blueprints/PlayerCharacter/BP_PlayerCharacter.IsLanding` false (`self.Player Character`))
        (`/Game/Blueprints/PlayerCharacter/BP_PlayerFSM.Change State` (`self.FSM`) "NewEnumerator0")
        (else
          (`CharacterMovementComponent.AddForce` (`Character.CharacterMovement` (`self.Player Character`)) (0.0 0.0 -100000.0)))))))
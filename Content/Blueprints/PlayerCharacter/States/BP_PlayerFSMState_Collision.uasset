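; Player character FSM state for collisions, allowing camera look while active.
; On start it deactivates the player helper component, then after a short delay switches movement to Flying and changes state.
; Dash input moves the capsule to the mesh, stops mesh physics, reattaches the mesh, sets Walking and changes to another state.
; Ragdoll launch, montage, impulse and capsule-follow logic is left unconnected, and Tick is empty.
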(event `self.Start`
  (`parent.Start`)
  (`self.SetActive` (`/Game/Blueprints/PlayerCharacter/BP_PlayerCharacter.BPC_PlayerHelperComponent` (`self.Player Character`)) false false)
  (`KismetSystemLibrary.Delay` 1.5)
  (`CharacterMovementComponent.SetMovementMode` (`Character.CharacterMovement` (`/Game/Blueprints/PlayerCharacter/BP_PlayerFSM.PlayerCharacter` (`self.FSM`))) "MOVE_Flying" 0)
  (`/Game/Blueprints/PlayerCharacter/BP_PlayerFSM.Change State` (`self.FSM`) "NewEnumerator4"))

(event `/Game/Blueprints/PlayerCharacter/BPI_InputHandler.IA_Look`
  (params (X :type "Float (double-precision)") (Y :type "Float (double-precision)"))
  (`Pawn.AddControllerPitchInput` (`/Game/Blueprints/PlayerCharacter/BP_PlayerFSM.PlayerCharacter` (`self.FSM`)) (* Y -1.0))
  (`Pawn.AddControllerYawInput` (`/Game/Blueprints/PlayerCharacter/BP_PlayerFSM.PlayerCharacter` (`self.FSM`)) X))

(event `self.Tick`)

(event `/Game/Blueprints/PlayerCharacter/BPI_InputHandler.IA_Dash_Trigger`
  (bind _player_character (`self.Player Character`))
  (bind _mesh (`Character.Mesh` (`self.Player Character`)))
  (bind _mesh_2 (`Character.Mesh` _player_character))
  (bind _mesh_3 (`Character.Mesh` (`self.Player Character`)))
  (bind _returnvalue_location (`KismetMathLibrary.BreakTransform` (`SkinnedMeshComponent.GetBoneTransform` _mesh_3 "Root" "RTS_World")))
  (`KismetSystemLibrary.PrintString` (`KismetStringLibrary.Conv_VectorToString` _returnvalue_location))
  (`SceneComponent.K2_SetWorldLocation` (`Character.CapsuleComponent` (`self.Player Character`)) (`SceneComponent.K2_GetComponentLocation` _mesh_3) false true)
  (`PrimitiveComponent.SetSimulatePhysics` _mesh false)
  (`SkeletalMeshComponent.ResetAllBodiesSimulatePhysics` _mesh)
  (`AnimInstance.ResetDynamics` (`SkeletalMeshComponent.GetAnimInstance` _mesh) "ResetPhysics")
  (`SceneComponent.K2_SetRelativeLocationAndRotation` :`self` _mesh_2 :`NewLocation` (0.0 0.0 -15.0) :`bTeleport` true)
  (`SceneComponent.K2_AttachToComponent` _mesh_2 (`Character.CapsuleComponent` _player_character) "None" "KeepRelative" "KeepRelative" "KeepRelative" true)
  (`CharacterMovementComponent.SetMovementMode` (`Character.CharacterMovement` (`self.Player Character`)) "MOVE_Walking" 0)
  (`/Game/Blueprints/PlayerCharacter/BP_PlayerFSM.Change State` (`self.FSM`) "NewEnumerator0"))
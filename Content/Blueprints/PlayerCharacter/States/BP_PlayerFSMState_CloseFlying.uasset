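; Player FSM state for the bird character's close flying mode, applying flight rotation and collision size on start.
; Input drives thrust along auto-aim, braking, stationary look, and a bullet dive with tweened camera pitch.
; Tick updates the flying camera and brakes near ground, where a short trace switches to walking.
; Dash flaps into another state, or fades and teleports for NPC interaction, though NPC detection is never called.
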(event `self.Start`
  (bind _playercharacter (`/Game/Blueprints/PlayerCharacter/BP_PlayerFSM.PlayerCharacter` (`self.FSM`)))
  (bind _capsulecomponent (`Character.CapsuleComponent` (`self.Player Character`)))
  (bind _playerdata (`/Game/Blueprints/PlayerCharacter/BP_PlayerFSM.PlayerData` (`self.FSM`)))
  (`parent.Start`)
  (set `self.IsInteracting` false)
  (set `self.NearbyNPC` null)
  (set `CharacterMovementComponent.RotationRate` (`/Game/Blueprints/PlayerCharacter/DA_PlayerStats.Flying_RotationRate` (`/Game/Blueprints/PlayerCharacter/BP_PlayerFSM.PlayerData` (`self.FSM`))) (`Character.CharacterMovement` (`self.Player Character`)))
  ;[1 1 1] Activate Helper component
  (`/Game/Blueprints/PlayerCharacter/BP_PlayerCharacter.SetHelperComponentActive` (`self.Player Character`) true)
  (`CapsuleComponent.SetCapsuleHalfHeight` _capsulecomponent (`/Game/Blueprints/PlayerCharacter/DA_PlayerStats.Flying_CollisionHeight` _playerdata) true)
  (`CapsuleComponent.SetCapsuleRadius` _capsulecomponent (`/Game/Blueprints/PlayerCharacter/DA_PlayerStats.Flying_CollisionRadius` _playerdata) true)
  (`/Game/Blueprints/PlayerCharacter/DA_PlayerStats.ApplyDefaultFrictionDeaccleration` (`/Game/Blueprints/PlayerCharacter/BP_PlayerCharacter.PlayerStats` _playercharacter) _playercharacter))

(event `/Game/Blueprints/PlayerCharacter/BPI_InputHandler.IA_Accelerate`
  (params (Value :type "Float (double-precision)"))
  (`/Game/Blueprints/PlayerCharacter/BP_PlayerCharacter.OnStartFlying` (`self.Player Character`))
  (`Pawn.AddMovementInput` (`self.Player Character`) (`SceneComponent.GetForwardVector` (`/Game/Blueprints/PlayerCharacter/BP_PlayerCharacter.AutoAimDirection` (`self.Player Character`))) Value false)
  (if (< (stale `self.IA_Move` Y) 0.0)
    (`CharacterMovementComponent.AddForce` (`Character.CharacterMovement` (`self.Player Character`)) (* (`SceneComponent.GetForwardVector` (`/Game/Blueprints/PlayerCharacter/BP_PlayerCharacter.AutoAimDirection` (`self.Player Character`))) 100.0))))

(event `self.IA_Move`
  (params (X :type "Float (double-precision)") (Y :type "Float (double-precision)")))

(event `self.IA_Dash_Trigger`
  (bind (_returnvalue_x _returnvalue_y) (`KismetMathLibrary.BreakVector2D` (`WidgetLayoutLibrary.GetViewportSize`)))
  (bind _nearbynpc (`self.NearbyNPC`))
  (bind _playercameramanager (`PlayerController.PlayerCameraManager` (`GameplayStatics.GetPlayerController` 0)))
  (`/Engine/EditorBlueprintResources/StandardMacros.IsValid` _nearbynpc
    (:`Is Valid`
      (`/Game/Blueprints/NPC/BP_NPC.ToggleInteractionVisibility` (`self.NearbyNPC`) false)
      (set `self.IsInteracting` true)
      (`PlayerCameraManager.StartCameraFade` :`self` _playercameramanager :`ToAlpha` 1.0 :`Duration` 0.5 :`bHoldWhenFinished` true)
      (`KismetSystemLibrary.Delay` 0.5)
      (`/Game/Blueprints/PROTOTYPEQuest/AC_ValiantInteractionComponent.Interact` (`/Game/Blueprints/NPC/BP_NPC.AC_ValiantInteractionComponent` _nearbynpc))
      (`KismetSystemLibrary.Delay` 0.3)
      (`PlayerCameraManager.StartCameraFade` :`self` _playercameramanager :`FromAlpha` 1.0 :`Duration` 0.5)
      (`self.TeleportPlayer`)
      (set `/Game/Blueprints/PROTOTYPEQuest/AC_ValiantInteractionComponent.ExternalInteraction` false (`/Game/Blueprints/NPC/BP_NPC.AC_ValiantInteractionComponent` (`self.NearbyNPC`)))
      (set `self.NearbyNPC` null))
    (:`Is Not Valid`
      (if (`/Game/Blueprints/PlayerCharacter/BP_PlayerCharacter.CanFly` (`self.Player Character`))
        (`/Game/Blueprints/PlayerCharacter/BP_PlayerCharacter.Flap` (`self.Player Character`))
        (`self.ActivatePointer`)
        (`PlayerController.SetMouseLocation` (`GameplayStatics.GetPlayerController` 0) (`KismetMathLibrary.FTrunc` (/ _returnvalue_x 2.0)) (`KismetMathLibrary.FTrunc` (/ _returnvalue_y 2.0)))
        (`/Game/Blueprints/PlayerCharacter/BP_PlayerFSM.Change State` (`self.FSM`) "NewEnumerator2")))))

(event `self.Tick`
  (set `self.Turn Direction Offset` (`/Game/Blueprints/PlayerCharacter/BP_PlayerCharacter.TurnDirectionOffset` (`self.Player Character`)))
  (`/Game/Blueprints/PlayerCharacter/BP_PlayerCharacter.UpdateCameraFlyingMode` (`self.Player Character`))
  (`self.DeaccelerateWhenCloseToGround`))

(event `TeleportPlayer`
  (bind (_returnvalue_location _returnvalue_rotation) (`KismetMathLibrary.BreakTransform` (`SceneComponent.K2_GetComponentToWorld` (`/Game/Blueprints/NPC/BP_NPC.PlayerPoint` (`self.NearbyNPC`)))))
  (`KismetSystemLibrary.PrintString` "TELEPORTING PLAYER \n")
  (`Actor.K2_TeleportTo` (`self.GetOwner`) _returnvalue_location _returnvalue_rotation)
  (`/Game/Blueprints/PlayerCharacter/BP_PlayerFSM.Change State` (`self.FSM`) "NewEnumerator0"))

(event `self.End`
  ;[1 1 1] Activate Helper component
  (`/Game/Blueprints/PlayerCharacter/BP_PlayerCharacter.SetHelperComponentActive` (`self.Player Character`) true)
  (`/Game/Blueprints/PlayerCharacter/BP_PlayerCharacter.OnStopFlying` (`self.Player Character`)))

(event `self.IA_Brake_Trigger`
  (params (Value :type "Float (double-precision)"))
  (bind _charactermovement (`Character.CharacterMovement` (`self.Player Character`)))
  (bind _velocity (`MovementComponent.Velocity` _charactermovement))
  (if (> (`KismetMathLibrary.VSize` _velocity) 50.0)
    (`CharacterMovementComponent.AddForce` _charactermovement (* _velocity -40.0))))

(event `self.IA_Brake_Complete`)

(event `self.IA_Bullet_Started`
  (bind _cameraboom (`/Game/Blueprints/PlayerCharacter/BP_PlayerCharacter.CameraBoom` (`self.Player Character`)))
  (bind (_returnvalue_roll _returnvalue_pitch _returnvalue_yaw) (`KismetMathLibrary.BreakRotator` (`Controller.GetControlRotation` (`Pawn.GetController` (`self.Player Character`)))))
  (set `SpringArmComponent.bUsePawnControlRotation` true (`/Game/Blueprints/PlayerCharacter/BP_PlayerCharacter.CameraBoom` (`self.Player Character`)))
  (set `SpringArmComponent.bDoCollisionTest` false _cameraboom)
  (set `SpringArmComponent.bInheritRoll` true _cameraboom)
  (set `SpringArmComponent.bInheritYaw` true _cameraboom)
  (set `SpringArmComponent.bInheritPitch` true _cameraboom)
  (bind (_asynctaskproxy _value) (`FCTweenBPActionRotator.TweenRotator` (`KismetMathLibrary.MakeRotator` 0.0 _returnvalue_pitch _returnvalue_yaw) (`KismetMathLibrary.MakeRotator` 0.0 -45.0 _returnvalue_yaw) 1.5)
    (:`then`
      (set `self.BulletModeCamTransition` _asynctaskproxy))
    (:`ApplyEasing`
      (`Controller.SetControlRotation` (`Pawn.GetController` (`self.Player Character`)) _value))))

(event `self.IA_Bullet_Trigger`
  (set `/Game/Blueprints/PlayerCharacter/BP_PlayerCharacter.BirdFlyingState` "NewEnumerator4" (`self.Player Character`))
  (`CharacterMovementComponent.AddForce` (`Character.CharacterMovement` (`self.Player Character`)) (`/Game/Blueprints/PlayerCharacter/BP_PlayerCharacter.BulletModeForce` (`self.Player Character`))))

(event `self.IA_Bullet_Completed`
  (bind _bulletmodecamtransition (`self.BulletModeCamTransition`))
  (bind (_returnvalue_roll _returnvalue_pitch _returnvalue_yaw) (`KismetMathLibrary.BreakRotator` (`Controller.GetControlRotation` (`Pawn.GetController` (`self.Player Character`)))))
  (set `/Game/Blueprints/PlayerCharacter/BP_PlayerCharacter.BirdFlyingState` "NewEnumerator2" (`self.Player Character`))
  (`/Engine/EditorBlueprintResources/StandardMacros.IsValid` _bulletmodecamtransition
    (:`Is Valid`
      (`FCTweenBPAction.Stop` _bulletmodecamtransition))
    (:`Is Not Valid`
      _))
  (set `SpringArmComponent.bUsePawnControlRotation` true (`/Game/Blueprints/PlayerCharacter/BP_PlayerCharacter.CameraBoom` (`self.Player Character`)))
  (set `SpringArmComponent.bDoCollisionTest` true (`/Game/Blueprints/PlayerCharacter/BP_PlayerCharacter.CameraBoom` (`self.Player Character`)))
  (bind (_asynctaskproxy _value) (`FCTweenBPActionRotator.TweenRotator` (`KismetMathLibrary.MakeRotator` 0.0 _returnvalue_pitch _returnvalue_yaw) (`KismetMathLibrary.MakeRotator` 0.0 0.0 _returnvalue_yaw) 0.75)
    (:`ApplyEasing`
      (`Controller.SetControlRotation` (`Pawn.GetController` (`self.Player Character`)) _value))))

(event `self.IA_Look`
  (params (X :type "Float (double-precision)") (Y :type "Float (double-precision)"))
  (if (not (> (`KismetMathLibrary.VSize` (`Actor.GetVelocity` (`self.Player Character`))) 0.0))
    (`Pawn.AddControllerPitchInput` (`/Game/Blueprints/PlayerCharacter/BP_PlayerFSM.PlayerCharacter` (`self.FSM`)) (* Y -1.0))
    (`Pawn.AddControllerYawInput` (`/Game/Blueprints/PlayerCharacter/BP_PlayerFSM.PlayerCharacter` (`self.FSM`)) X)))

(fn `DeaccelerateWhenCloseToGround`
  (bind _returnvalue (`Actor.K2_GetActorLocation` (`self.Player Character`)))
  (bind _charactermovement (`Character.CharacterMovement` (`self.Player Character`)))
  (if (`/Game/Blueprints/PlayerCharacter/BP_PlayerCharacter.CloseToGround` (`self.Player Character`))
    (`CharacterMovementComponent.AddForce` _charactermovement (* (`MovementComponent.Velocity` _charactermovement) -75.0))
    (if (< (`KismetMathLibrary.VSize` (`MovementComponent.Velocity` (`Character.CharacterMovement` (`self.Player Character`)))) 605.0)
      (bind (_outhit _returnvalue_2) (`KismetSystemLibrary.LineTraceSingle` :`Start` _returnvalue :`End` (+ _returnvalue (0.0 0.0 -25.0)) :`TraceChannel` "TraceTypeQuery1" :`DrawDebugType` "ForOneFrame" :`TraceColor` (struct :`R` 0.674571 :`B` 1.0 :`A` 1.0)))
      (if _returnvalue_2
        (`CharacterMovementComponent.SetMovementMode` (`Character.CharacterMovement` (`self.Player Character`)) "MOVE_Walking" 0)
        (`/Game/Blueprints/PlayerCharacter/BP_PlayerFSM.Change State` (`self.FSM`) "NewEnumerator0")))))

(fn `DetectNearbyNPCs`
  (returns (ReturnValue :type "/Game/Blueprints/NPC/BP_NPC Object Reference") (`Found any?` :type Boolean))
  (locals (ResultActor :type "/Game/Blueprints/NPC/BP_NPC Object Reference") (VisibleActors :type "Array of Actor Object Reference"))
  (bind (_distance _returnvalue) (`GameplayStatics.FindNearestActor` (`Actor.K2_GetActorLocation` (`self.GetOwner`)) (`local.VisibleActors`)))
  (bind (_asbp_npc _bsuccess) (cast `/Game/Blueprints/NPC/BP_NPC` _returnvalue :!pure true))
  (bind (_outactors _returnvalue_2) (`KismetSystemLibrary.SphereOverlapActors` (`Actor.K2_GetActorLocation` (`self.GetOwner`)) (`self.NearbyNPCsDetectionRange`) (`|MakeArray` "ObjectTypeQuery3" :!type "EObjectTypeQuery Enum") "/Game/Blueprints/NPC/BP_NPC.BP_NPC_C"))
  (if _returnvalue_2
    (for _array_element _outactors
      (if (`/Game/Blueprints/NPC/BP_NPC.GetInteractionState` (cast `/Game/Blueprints/NPC/BP_NPC` _array_element :!pure true))
        (`KismetArrayLibrary.Array_Add` (`local.VisibleActors`) _array_element)))
    (`/Engine/EditorBlueprintResources/StandardMacros.IsValid` _returnvalue
      (:`Is Valid`
        (return _asbp_npc _bsuccess)))
    (else
      (return null false))))

(fn `NPCInteract`
  (params (Delegate :type "Delegate (by ref)"))
  (bind _nearbynpc (`self.NearbyNPC`))
  (bind _nearbynpc_2 (`self.NearbyNPC`))
  (if (not (`self.IsInteracting`))
    (bind (_returnvalue _found_any_) (`self.DetectNearbyNPCs`))
    (if _found_any_
      (if (== _returnvalue (`self.NearbyNPC`))
        (`/Engine/EditorBlueprintResources/StandardMacros.DoOnce` false :!label _label
          (:`Completed`
            (`/Game/Blueprints/NPC/BP_NPC.ToggleInteractionVisibility` _nearbynpc_2 true)
            (set `/Game/Blueprints/PROTOTYPEQuest/AC_ValiantInteractionComponent.ExternalInteraction` true (`/Game/Blueprints/NPC/BP_NPC.AC_ValiantInteractionComponent` _nearbynpc_2))))
        (else
          (`/Engine/EditorBlueprintResources/StandardMacros.IsValid` _nearbynpc
            (:`Is Valid`
              (`/Game/Blueprints/NPC/BP_NPC.ToggleInteractionVisibility` _nearbynpc false)
              (set `/Game/Blueprints/PROTOTYPEQuest/AC_ValiantInteractionComponent.ExternalInteraction` false (`/Game/Blueprints/NPC/BP_NPC.AC_ValiantInteractionComponent` _nearbynpc)))
            (:`Is Not Valid`
              _))
          (set `self.NearbyNPC` _returnvalue)
          (goto _label :!via `Reset`))))))

(fn `RollToDirection`)
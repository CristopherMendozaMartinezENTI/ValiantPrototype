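; Landing state in the player character's state machine, which nudges the player toward a traced surface point.
; On start it runs a visibility line trace from the camera along only the vertical component of its forward vector.
; On a hit, it sets the character's max velocity and adds a single movement input toward the impact, scaled by distance with a clamped range mapping.
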(event `self.Start`
  (bind _player_character (`self.Player Character`))
  (bind _playercamera (`/Game/Blueprints/PlayerCharacter/BP_PlayerCharacter.PlayerCamera` (`self.Player Character`)))
  (bind _returnvalue (`SceneComponent.K2_GetComponentLocation` _playercamera))
  (`parent.Start`)
  (bind (_outhit _returnvalue_2) (`KismetSystemLibrary.LineTraceSingle` _returnvalue (+ _returnvalue (* (* (`SceneComponent.GetForwardVector` _playercamera) (0.0 0.0 100.0)) 1000.0)) "TraceTypeQuery1"))
  (if _returnvalue_2
    (set `/Game/Blueprints/PlayerCharacter/BP_PlayerCharacter.MaxVelocity` 20.0 (`self.Player Character`))
    (bind _returnvalue_3 (- (`.Location` (`GameplayStatics.BreakHitResult` _outhit)) (`Actor.K2_GetActorLocation` _player_character)))
    (`Pawn.AddMovementInput` _player_character (`KismetMathLibrary.Normal` _returnvalue_3) (`KismetMathLibrary.MapRangeClamped` (`KismetMathLibrary.VSize` _returnvalue_3) 0.0 100.0 0.0 1.0) false)))
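; Player state machine state for bird flight, handling acceleration, flapping, a bullet dive and exits on braking or slow ground contact.
; Tick drives momentum and forward movement, with a helper component's obstacle check cutting speed near walls.
; A downward trace near the ground raises the camera, adds forward force, adjusts pitch and triggers grass particles.
; Look input without movement opens a free peek camera; move or camera input tweens it back.
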(event `self.Start`
  (bind _playercharacter (`/Game/Blueprints/PlayerCharacter/BP_PlayerFSM.PlayerCharacter` (`self.FSM`)))
  (bind _capsulecomponent (`Character.CapsuleComponent` (`self.Player Character`)))
  (bind _playerdata (`/Game/Blueprints/PlayerCharacter/BP_PlayerFSM.PlayerData` (`self.FSM`)))
  (`parent.Start`)
  (`/Game/Blueprints/PlayerCharacter/BP_PlayerCharacter.OnStartFlying` _playercharacter)
  (`/Game/Blueprints/PlayerCharacter/DA_PlayerStats.ApplyDefaultFrictionDeaccleration` (`/Game/Blueprints/PlayerCharacter/BP_PlayerCharacter.PlayerStats` _playercharacter) _playercharacter)
  (set `self.canPeak` false)
  (set `CharacterMovementComponent.RotationRate` (`/Game/Blueprints/PlayerCharacter/DA_PlayerStats.Flying_RotationRate` (`/Game/Blueprints/PlayerCharacter/BP_PlayerFSM.PlayerData` (`self.FSM`))) (`Character.CharacterMovement` (`self.Player Character`)))
  ;[1 1 1] Activate Helper component
  (`/Game/Blueprints/PlayerCharacter/BP_PlayerCharacter.SetHelperComponentActive` (`self.Player Character`) true)
  (`CapsuleComponent.SetCapsuleHalfHeight` _capsulecomponent (`/Game/Blueprints/PlayerCharacter/DA_PlayerStats.Flying_CollisionHeight` _playerdata) true)
  (`CapsuleComponent.SetCapsuleRadius` _capsulecomponent (`/Game/Blueprints/PlayerCharacter/DA_PlayerStats.Flying_CollisionRadius` _playerdata) true)
  (`KismetSystemLibrary.Delay` 2.0)
  (set `self.canPeak` true))

(event `/Game/Blueprints/PlayerCharacter/BPI_InputHandler.IA_Dash_Trigger`
  (bind _player_character (`self.Player Character`))
  (if (`/Game/Blueprints/PlayerCharacter/BP_PlayerCharacter.CanDash` _player_character)
    (`/Game/Blueprints/PlayerCharacter/BP_PlayerCharacter.Flap` _player_character)))

(event `/Game/Blueprints/PlayerCharacter/BPI_InputHandler.IA_Brake_Trigger`
  (params (Value :type "Float (double-precision)"))
  (if (>= Value 1.0)
    (`/Game/Blueprints/PlayerCharacter/BP_PlayerFSM.Change State` (`self.FSM`) "NewEnumerator4")))

(event `/Game/Blueprints/PlayerCharacter/BPI_InputHandler.IA_Brake_Complete`)

(event `self.Tick`
  (bind _player_character (`self.Player Character`))
  (set `self.Turn Direction Offset` (`/Game/Blueprints/PlayerCharacter/BP_PlayerCharacter.TurnDirectionOffset` (`self.Player Character`)))
  (if (not (`self.IsPeakingCameraOn`))
    (`/Game/Blueprints/PlayerCharacter/BP_PlayerCharacter.UpdateCameraFlyingMode` (`self.Player Character`))
    (`self.DoAcceleration`)
    (`self.UpdateFlyingState`))
  (`/Game/Blueprints/PlayerCharacter/BP_PlayerCharacter.UpdateMomentum` _player_character (`GameplayStatics.GetWorldDeltaSeconds`))
  (`/Game/Blueprints/PlayerCharacter/BP_PlayerCharacter.RecoverMomentum` _player_character)
  (`self.DeaccelerateWhenCloseToGround`)
  (`self.UpdateCameraOffsets`)
  (bind (_isclosetoground _distance _impactpoint) (`self.ElevateCameraWhenCloseToGround`))
  (`self.AccelerateWhenCloseToGround` _isclosetoground _distance)
  (set `self.Impact Point` _impactpoint)
  (set `self.isCloseToground` _isclosetoground)
  (`|ExecutionSequence`
    (:`then_0`
      (if (and (`self.isCloseToground`) (< _distance 100.0))
        (`SceneComponent.K2_SetRelativeLocation` (`self.NS_GrassParticles`) (`KismetMathLibrary.MakeVector` 0.0 0.0 (* _distance -0.85)) false false)
        (`SceneComponent.K2_SetRelativeLocation` (`/Game/Blueprints/PlayerCharacter/BP_PlayerCharacter.AC_InteractWithFoliage` (`self.Player Character`)) (`KismetMathLibrary.MakeVector` 0.0 0.0 (* _distance -0.85)) false false)
        (`/Engine/EditorBlueprintResources/StandardMacros.DoOnce` false :!label _label
          (:`Completed`
            (`self.Activate` (`self.NS_GrassParticles`) false)
            (goto _label_2 :!via `Reset`)))
        (else
          (`/Engine/EditorBlueprintResources/StandardMacros.DoOnce` false :!label _label_2
            (:`Completed`
              (`self.Deactivate` (`self.NS_GrassParticles`))
              (goto _label :!via `Reset`))))))
    (:`then_1`
      (`self.NewMacro` false))))

(event `/Game/Blueprints/PlayerCharacter/BPI_InputHandler.IA_Accelerate_Complete`
  (params (Value :type "Float (double-precision)"))
  (set `self.Acceleration` 0.1))

(event `self.End`
  (bind _player_character (`self.Player Character`))
  ;[1 1 1] Activate Helper component
  (`/Game/Blueprints/PlayerCharacter/BP_PlayerCharacter.OnStopFlying` _player_character)
  (`/Game/Blueprints/PlayerCharacter/BP_PlayerCharacter.SetHelperComponentActive` _player_character true)
  (`self.Deactivate` (`self.NS_GrassParticles`)))

(event `self.ReceiveBeginPlay`
  (bind _returnvalue (`NiagaraFunctionLibrary.SpawnSystemAttached` "/Game/VFX/VFX/EnviromentalVFX/VFX/NS_Scattering_Grass.NS_Scattering_Grass" (`Character.CapsuleComponent` (`GameplayStatics.GetPlayerCharacter` 0)) "None" (0.0 0.0 0.0) (struct) "KeepRelativeOffset"))
  (set `self.NS_GrassParticles` _returnvalue)
  (`self.Deactivate` (`self.NS_GrassParticles`)))

(event `/Game/Blueprints/PlayerCharacter/BPI_InputHandler.IA_Accelerate`
  (params (Value :type "Float (double-precision)"))
  (bind _output_get (set `self.Acceleration` Value))
  (`KismetSystemLibrary.PrintString` (`KismetStringLibrary.Conv_DoubleToString` _output_get) true true (struct :`R` 1.0 :`G` 0.109634 :`B` 0.199325 :`A` 1.0) 2.0 "acc"))

(event `/Game/Blueprints/PlayerCharacter/BPI_InputHandler.IA_Bullet_Started`
  (bind _cameraboom (`/Game/Blueprints/PlayerCharacter/BP_PlayerCharacter.CameraBoom` (`self.Player Character`)))
  (bind (_returnvalue_roll _returnvalue_pitch _returnvalue_yaw) (`KismetMathLibrary.BreakRotator` (`Controller.GetControlRotation` (`Pawn.GetController` (`self.Player Character`)))))
  (set `SpringArmComponent.bUsePawnControlRotation` true (`/Game/Blueprints/PlayerCharacter/BP_PlayerCharacter.CameraBoom` (`self.Player Character`)))
  (set `SpringArmComponent.bDoCollisionTest` false _cameraboom)
  (set `SpringArmComponent.bInheritRoll` true _cameraboom)
  (set `SpringArmComponent.bInheritYaw` true _cameraboom)
  (set `SpringArmComponent.bInheritPitch` true _cameraboom)
  (bind (_asynctaskproxy _value) (`FCTweenBPActionRotator.TweenRotator` (`KismetMathLibrary.MakeRotator` 0.0 _returnvalue_pitch _returnvalue_yaw) (`KismetMathLibrary.MakeRotator` 0.0 -45.0 _returnvalue_yaw) 1.5)
    (:`then`
      (set `self.BulletModeCamTransition` _asynctaskproxy))
    (:`ApplyEasing`
      (`Controller.SetControlRotation` (`Pawn.GetController` (`self.Player Character`)) _value))))

(event `/Game/Blueprints/PlayerCharacter/BPI_InputHandler.IA_Bullet_Trigger`
  (set `/Game/Blueprints/PlayerCharacter/BP_PlayerCharacter.BirdFlyingState` "NewEnumerator4" (`self.Player Character`))
  (`CharacterMovementComponent.AddForce` (`Character.CharacterMovement` (`self.Player Character`)) (`/Game/Blueprints/PlayerCharacter/BP_PlayerCharacter.BulletModeForce` (`self.Player Character`))))

(event `/Game/Blueprints/PlayerCharacter/BPI_InputHandler.IA_Bullet_Completed`
  (bind _bulletmodecamtransition (`self.BulletModeCamTransition`))
  (bind (_returnvalue_roll _returnvalue_pitch _returnvalue_yaw) (`KismetMathLibrary.BreakRotator` (`Controller.GetControlRotation` (`Pawn.GetController` (`self.Player Character`)))))
  (set `/Game/Blueprints/PlayerCharacter/BP_PlayerCharacter.BirdFlyingState` "NewEnumerator2" (`self.Player Character`))
  (`/Engine/EditorBlueprintResources/StandardMacros.IsValid` _bulletmodecamtransition
    (:`Is Valid`
      (`FCTweenBPAction.Stop` _bulletmodecamtransition))
    (:`Is Not Valid`
      _))
  (set `SpringArmComponent.bUsePawnControlRotation` true (`/Game/Blueprints/PlayerCharacter/BP_PlayerCharacter.CameraBoom` (`self.Player Character`)))
  (set `SpringArmComponent.bDoCollisionTest` true (`/Game/Blueprints/PlayerCharacter/BP_PlayerCharacter.CameraBoom` (`self.Player Character`)))
  (bind (_asynctaskproxy _value) (`FCTweenBPActionRotator.TweenRotator` (`KismetMathLibrary.MakeRotator` 0.0 _returnvalue_pitch _returnvalue_yaw) (`KismetMathLibrary.MakeRotator` 0.0 0.0 _returnvalue_yaw) 0.75)
    (:`ApplyEasing`
      (`Controller.SetControlRotation` (`Pawn.GetController` (`self.Player Character`)) _value))))

(event `SpawnGrassWhenCloseToGround`
  (`NiagaraFunctionLibrary.SpawnSystemAtLocation` "/Game/VFX/VFX/EnviromentalVFX/VFX/NS_Scattering_Grass.NS_Scattering_Grass" (+ (`self.Impact Point`) (0.0 0.0 50.0)) (struct) (1.0 1.0 1.0) true true "AutoRelease"))

(event `/Game/Blueprints/PlayerCharacter/BPI_InputHandler.IA_Look`
  (params (X :type "Float (double-precision)") (Y :type "Float (double-precision)"))
  (bind _returnvalue (`KismetMathLibrary.MakeVector2D` X Y))
  (bind _player_character (`self.Player Character`))
  (if (`self.canPeak`)
    (set `self.CurrentIALooko` _returnvalue)
    (if (and (>= (`KismetMathLibrary.VSize2D` _returnvalue) 0.1) (<= (`KismetMathLibrary.VSize2D` (`KismetMathLibrary.MakeVector2D` (`/Game/Blueprints/PlayerCharacter/BP_PlayerCharacter.MoveX` _player_character) (`/Game/Blueprints/PlayerCharacter/BP_PlayerCharacter.MoveY` _player_character))) 0.1))
      (`|ExecutionSequence`
        (:`then_0`
          (`/Engine/EditorBlueprintResources/StandardMacros.DoOnce` false :!label _label_3
            (:`Completed`
              (set `/Game/Blueprints/PlayerCharacter/BP_PlayerCharacter.UpdateArmLength` false (`self.Player Character`))
              (`self.ActivatePeakingCamera`))))
        (:`then_1`
          (`self.UpdatePeakingCamera`))))))

(event `ActivatePeakingCamera`
  (bind _charactermovement (`Character.CharacterMovement` (`self.Player Character`)))
  (set `self.LatestControlRotation` (`Controller.GetControlRotation` (`Pawn.GetController` (`self.Player Character`))))
  (set `self.IsPeakingCameraOn` true)
  (set `/Game/Blueprints/PlayerCharacter/BPC_PlayerHelperComponent.FollowPlayerCamera` false (`/Game/Blueprints/PlayerCharacter/BP_PlayerCharacter.BPC_PlayerHelperComponent` (`self.Player Character`)))
  (set `CharacterMovementComponent.bUseControllerDesiredRotation` false _charactermovement)
  (set `CharacterMovementComponent.bOrientRotationToMovement` true _charactermovement)
  (set `SpringArmComponent.bEnableCameraLag` false (`/Game/Blueprints/PlayerCharacter/BP_PlayerCharacter.CameraBoom` (`self.Player Character`)))
  (bind _output_get (set `self.StartingCameraDistance` (`SpringArmComponent.TargetArmLength` (`/Game/Blueprints/PlayerCharacter/BP_PlayerCharacter.CameraBoom` (`self.Player Character`)))))
  (bind (_asynctaskproxy _value) (`FCTweenBPActionFloat.TweenFloat` _output_get 400.0)
    (:`ApplyEasing`
      (set `SpringArmComponent.TargetArmLength` _value (`/Game/Blueprints/PlayerCharacter/BP_PlayerCharacter.CameraBoom` (`self.Player Character`))))))

(event `UpdatePeakingCamera`
  (bind _player_character (`self.Player Character`))
  (bind (_currentialooko_x _currentialooko_y) (`KismetMathLibrary.BreakVector2D` (`self.CurrentIALooko`)))
  (`Pawn.AddControllerYawInput` _player_character (* _currentialooko_x 2.0))
  (`Pawn.AddControllerPitchInput` _player_character (* _currentialooko_y -2.0)))

(event `ReturnToNormalCamera`
  (bind _latestcontrolrotation (`self.LatestControlRotation`))
  (bind _charactermovement (`Character.CharacterMovement` (`self.Player Character`)))
  (set `self.IsPeakingCameraOn` false :!label _label_4)
  (bind _output_get (set `self.StartingRot` (`Controller.GetControlRotation` (`Pawn.GetController` (`self.Player Character`)))))
  (bind (_asynctaskproxy _value) (`FCTweenBPActionRotator.TweenRotator` _output_get _latestcontrolrotation (* 2.0 (`KismetMathLibrary.Abs` (`KismetMathLibrary.Dot_VectorVector` (`KismetMathLibrary.Normal` (`KismetMathLibrary.GetAxes` _output_get)) (`KismetMathLibrary.Normal` (`KismetMathLibrary.GetAxes` _latestcontrolrotation))))))
    (:`then`
      (bind (_asynctaskproxy_2 _value_2) (`FCTweenBPActionFloat.TweenFloat` 400.0 (`self.StartingCameraDistance`))
        (:`ApplyEasing`
          (set `SpringArmComponent.TargetArmLength` _value_2 (`/Game/Blueprints/PlayerCharacter/BP_PlayerCharacter.CameraBoom` (`self.Player Character`))))
        (:`OnComplete`
          (set `/Game/Blueprints/PlayerCharacter/BP_PlayerCharacter.UpdateArmLength` true (`self.Player Character`)))))
    (:`ApplyEasing`
      (`Controller.SetControlRotation` (`Pawn.GetController` (`self.Player Character`)) _value))
    (:`OnComplete`
      (set `/Game/Blueprints/PlayerCharacter/BPC_PlayerHelperComponent.FollowPlayerCamera` true (`/Game/Blueprints/PlayerCharacter/BP_PlayerCharacter.BPC_PlayerHelperComponent` (`self.Player Character`)))
      (set `CharacterMovementComponent.bUseControllerDesiredRotation` true _charactermovement)
      (set `CharacterMovementComponent.bOrientRotationToMovement` false _charactermovement)
      (set `self.HasManuallyReturnedToNormalCamera` false)
      (set `SpringArmComponent.bEnableCameraLag` true (`/Game/Blueprints/PlayerCharacter/BP_PlayerCharacter.CameraBoom` (`self.Player Character`)))
      (goto _label_3 :!via `Reset`))))

(event `/Game/Blueprints/PlayerCharacter/BPI_InputHandler.IA_Camera`
  (params (NewParam :type Boolean))
  (if (`self.IsPeakingCameraOn`)
    (set `self.HasManuallyReturnedToNormalCamera` true :!label _label_5)
    (goto _label_4)))

(event `/Game/Blueprints/PlayerCharacter/BPI_InputHandler.IA_Move`
  (params (X :type "Float (double-precision)") (Y :type "Float (double-precision)"))
  (if (`self.IsPeakingCameraOn`)
    (goto _label_5)))

(fn `AccelerateWhenCloseToGround`
  (params (CanAccelerate :type Boolean) (Distance :type "Float (double-precision)"))
  (bind _player_character (`self.Player Character`))
  (bind (_returnvalue_roll _returnvalue_pitch) (`KismetMathLibrary.BreakRotator` (`PlayerCameraManager.GetCameraRotation` (`PlayerController.PlayerCameraManager` (`GameplayStatics.GetPlayerController` 0)))))
  (bind _returnvalue (+ _returnvalue_pitch -1.0))
  (bind _returnvalue_2 (`KismetMathLibrary.FMax` (`KismetMathLibrary.MultiplyMultiply_FloatFloat` (* _returnvalue 0.06) 2.0) 0.003))
  (if CanAccelerate
    (`CharacterMovementComponent.AddForce` (`Character.CharacterMovement` _player_character) (* (`SceneComponent.GetForwardVector` (`/Game/Blueprints/PlayerCharacter/BP_PlayerCharacter.AutoAimDirection` _player_character)) (`KismetMathLibrary.MapRangeClamped` Distance 0.0 300.0 10000.0)))
    (if (and (> (`KismetMathLibrary.Abs` _returnvalue) (/ 2.0 2.0)) (< (`/Game/Blueprints/PlayerCharacter/BP_PlayerCharacter.MoveY` (`self.Player Character`)) 0.1) (> (`KismetMathLibrary.VSize` (`Actor.GetVelocity` (`self.Player Character`))) 1400.0))
      (if true
        (`Pawn.AddControllerPitchInput` (`GameplayStatics.GetPlayerCharacter` 0) (* _returnvalue_2 (`KismetMathLibrary.SignOfFloat` _returnvalue)))
        (`KismetSystemLibrary.PrintString` (`KismetStringLibrary.Conv_DoubleToString` _returnvalue_2) true true (struct :`R` 1.0 :`G` 0.82426 :`A` 1.0) 2.0 "Powa")
        (return)))))

(fn `DeaccelerateWhenCloseToGround`
  (bind _returnvalue (`Actor.K2_GetActorLocation` (`self.Player Character`)))
  (if (< (`KismetMathLibrary.VSize` (`MovementComponent.Velocity` (`Character.CharacterMovement` (`self.Player Character`)))) 800.0)
    (bind (_outhit _returnvalue_2) (`KismetSystemLibrary.LineTraceSingle` :`Start` _returnvalue :`End` (+ _returnvalue (0.0 0.0 -25.0)) :`TraceChannel` "TraceTypeQuery1" :`DrawDebugType` "ForOneFrame" :`TraceColor` (struct :`R` 0.674571 :`B` 1.0 :`A` 1.0)))
    (if _returnvalue_2
      (`CharacterMovementComponent.SetMovementMode` (`Character.CharacterMovement` (`self.Player Character`)) "MOVE_Walking" 0)
      (`/Game/Blueprints/PlayerCharacter/BP_PlayerFSM.Change State` (`self.FSM`) "NewEnumerator0"))))

(fn `DoAcceleration`
  (bind _player_character (`self.Player Character`))
  (if (< (`KismetMathLibrary.VSize` (`Actor.GetVelocity` (`self.Player Character`))) 1500.0)
    (bind _returnvalue (`/Game/Blueprints/PlayerCharacter/BPC_PlayerHelperComponent.GetIfForwardIsNearObstacle` (`/Game/Blueprints/PlayerCharacter/BP_PlayerCharacter.BPC_PlayerHelperComponent` (`self.Player Character`))))
    (bind _output_get (set `self.IsInFrontOfWall` _returnvalue))
    (bind _output_get_2 (set `/Game/Characters/FinalBird/AnimBlueprint_Bruno.IsCloseToWal` _output_get (cast `/Game/Characters/FinalBird/AnimBlueprint_Bruno` (`SkeletalMeshComponent.GetAnimInstance` (`Character.Mesh` _player_character)) :!pure true)))
    (bind _output_get_3 (set `/Game/Blueprints/PlayerCharacter/BP_PlayerCharacter.VerticalHit` _output_get_2 _player_character))
    (if (not _output_get_3)
      (`Pawn.AddMovementInput` (`self.Player Character`) (`SceneComponent.GetForwardVector` (`/Game/Blueprints/PlayerCharacter/BP_PlayerCharacter.AutoAimDirection` (`self.Player Character`))) (`self.Acceleration`) false :!label _label))
    (else
      (goto _label))))

(fn `ElevateCameraWhenCloseToGround`
  (returns (IsCloseToGround :type Boolean) (Distance :type "Float (single-precision)") (ImpactPoint :type "Vector Structure"))
  (bind _returnvalue (`Actor.K2_GetActorLocation` (`self.Player Character`)))
  (bind _cameraboom (`/Game/Blueprints/PlayerCharacter/BP_PlayerCharacter.CameraBoom` (`self.Player Character`)))
  (bind (_outhit _returnvalue_2) (`KismetSystemLibrary.LineTraceSingle` :`Start` _returnvalue :`End` (+ _returnvalue (0.0 0.0 -300.0)) :`TraceChannel` "TraceTypeQuery1" :`DrawDebugType` "ForOneFrame"))
  (bind (_bblockinghit _binitialoverlap _time _distance _location _impactpoint) (`GameplayStatics.BreakHitResult` _outhit))
  (set `SpringArmComponent.TargetOffset` (`KismetMathLibrary.VInterpTo` (`SpringArmComponent.TargetOffset` _cameraboom) (`KismetMathLibrary.MakeVector` 0.0 0.0 (`KismetMathLibrary.SelectFloat` (`KismetMathLibrary.MapRangeClamped` _distance 300.0 0.0 0.0 50.0) 0.0 _returnvalue_2)) (`GameplayStatics.GetWorldDeltaSeconds`) 3.0) _cameraboom)
  (return _returnvalue_2 _distance _impactpoint))

(fn `Get Max Velocity`
  (returns (NewParam :type "Float (double-precision)"))
  (bind _returnvalue (`KismetMathLibrary.VSize` (`Actor.GetVelocity` (`self.Player Character`))))
  (bind _output_get (set `self.CurrVel` (`KismetMathLibrary.FInterpTo` (`KismetMathLibrary.VSize` (`Actor.GetVelocity` (`self.Player Character`))) (`KismetMathLibrary.MapRangeClamped` (`self.Acceleration`) 0.0 1.0 0.0 (`parent.Get Max Velocity`)) (`GameplayStatics.GetWorldDeltaSeconds`) 0.3)))
  (if (`self.IsInFrontOfWall`)
    (bind _output_get_2 (set `self.CurrVel` (`KismetMathLibrary.FInterpTo` _returnvalue 0.0 (`GameplayStatics.GetWorldDeltaSeconds`) (`KismetMathLibrary.MapRangeClamped` _returnvalue 600.0 2100.0 6.0 60.0))))
    (return _output_get_2)
    (else
      (return (`KismetMathLibrary.SelectFloat` (`parent.Get Max Velocity`) _output_get (> (`/Game/Blueprints/PlayerCharacter/BP_PlayerCharacter.Pitch` (`self.Player Character`)) 10.0))))))

(fn `RollToDirection`)

(fn `UpdateCameraOffsets`
  (bind _returnvalue (`KismetMathLibrary.FInterpTo` (`self.InterpMoveX`) (`KismetMathLibrary.Abs` (`/Game/Blueprints/PlayerCharacter/BP_PlayerCharacter.MoveX` (`self.Player Character`))) (`GameplayStatics.GetWorldDeltaSeconds`) 1.0))
  (set `self.InterpMoveX` _returnvalue)
  (`SceneComponent.K2_SetRelativeLocation` (`/Game/Blueprints/PlayerCharacter/BP_PlayerCharacter.CameraBoom` (`self.Player Character`)) (`KismetMathLibrary.MakeVector` 0.0 0.0 (`KismetMathLibrary.Lerp` 80.0 0.0 _returnvalue)) false false))

(fn `UpdateFlyingState`
  (if (and (`|EnumEquality` (`/Game/Blueprints/PlayerCharacter/BP_PlayerCharacter.BirdFlyingState` (`self.Player Character`)) "NewEnumerator3") (> (`self.Acceleration`) 0.3))
    (set `/Game/Blueprints/PlayerCharacter/BP_PlayerCharacter.BirdFlyingState` "NewEnumerator1" (`self.Player Character`))))
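; Player FSM state for walking, which on start adds stamina, applies movement and capsule settings from PlayerData, sets the camera boom and fades out the pointer widget.
; Input drives control-yaw-relative movement and look; the dash trigger jumps with an effect, or when falling switches state if CanCloseFly is set.
; Tick keeps depth-of-field focus on the capsule and smoothly tilts it to the ground normal via a short downward trace with debug drawing.
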(event `self.Start`
  (bind _player_character (`self.Player Character`))
  (bind _player_character_2 (`self.Player Character`))
  (bind _charactermovement (`Character.CharacterMovement` (`self.Player Character_0`)))
  (bind _capsulecomponent (`Character.CapsuleComponent` _player_character))
  (bind _playerdata (`/Game/Blueprints/PlayerCharacter/BP_PlayerFSM.PlayerData` (`self.FSM`)))
  (bind _charactermovement_2 (`Character.CharacterMovement` _player_character_2))
  (bind _uw_pointer (`/Game/Blueprints/PlayerCharacter/BP_PlayerCharacter.UW_Pointer` (`/Game/Blueprints/PlayerCharacter/BP_PlayerFSM.PlayerCharacter` (`self.FSM`))))
  (`parent.Start`)
  (`/Game/Blueprints/GameplayElements/StaminaComponent.Add Stamina` (`/Game/Blueprints/PlayerCharacter/BP_PlayerCharacter.StaminaComponent` _player_character_2) 100.0)
  (`CharacterMovementComponent.SetMovementMode` _charactermovement_2 "MOVE_Walking" 0)
  (set `CharacterMovementComponent.bUseControllerDesiredRotation` false _charactermovement_2)
  (set `CharacterMovementComponent.bOrientRotationToMovement` true _charactermovement_2)
  (`self.SetCameraOffset`)
  (set `self.Player Character_0` (`/Game/Blueprints/PlayerCharacter/BP_PlayerFSM.PlayerCharacter` (`self.FSM`)))
  (`/Game/Blueprints/PlayerCharacter/BP_PlayerCharacter.SetHelperComponentActive` (`self.Player Character`) false)
  (set `CharacterMovementComponent.MaxWalkSpeed` (`/Game/Blueprints/PlayerCharacter/DA_PlayerStats.Walking_Max Speed` (`/Game/Blueprints/PlayerCharacter/BP_PlayerFSM.PlayerData` (`self.FSM`))) _charactermovement)
  (set `CharacterMovementComponent.RotationRate` (`/Game/Blueprints/PlayerCharacter/DA_PlayerStats.Walking_RotationRate` (`/Game/Blueprints/PlayerCharacter/BP_PlayerFSM.PlayerData` (`self.FSM`))) _charactermovement)
  (`CapsuleComponent.SetCapsuleHalfHeight` _capsulecomponent (`/Game/Blueprints/PlayerCharacter/DA_PlayerStats.Walking_CollisionHeight` _playerdata) true)
  (`CapsuleComponent.SetCapsuleRadius` _capsulecomponent (`/Game/Blueprints/PlayerCharacter/DA_PlayerStats.Walking_CollisionRadius` _playerdata) true)
  (set `CharacterMovementComponent.GravityScale` 2.6 (`Character.CharacterMovement` _player_character))
  (bind (_asynctaskproxy _value) (`FCTweenBPActionFloat.TweenFloat` 1.0 0.0)
    (:`then`
      (`KismetSystemLibrary.DelayUntilNextTick`)
      (`Widget.SetVisibility` _uw_pointer "HitTestInvisible"))
    (:`ApplyEasing`
      (`Widget.SetRenderOpacity` _uw_pointer _value))))

(event `self.End`)

(event `/Game/Blueprints/PlayerCharacter/BPI_InputHandler.IA_Move`
  (params (X :type "Float (double-precision)") (Y :type "Float (double-precision)"))
  (bind (_returnvalue_roll _returnvalue_pitch _returnvalue_yaw) (`KismetMathLibrary.BreakRotator` (`Pawn.GetControlRotation` (`self.Player Character_0`))))
  (bind _returnvalue (`KismetMathLibrary.MakeRotator` 0.0 0.0 _returnvalue_yaw))
  (`Pawn.AddMovementInput` (`self.Player Character_0`) (`KismetMathLibrary.GetForwardVector` _returnvalue) Y false)
  (`Pawn.AddMovementInput` (`self.Player Character_0`) (`KismetMathLibrary.GetRightVector` _returnvalue) X false))

(event `self.Tick`
  (bind _player_character (`self.Player Character`))
  (bind _playercamera (`/Game/Blueprints/PlayerCharacter/BP_PlayerCharacter.PlayerCamera` _player_character))
  (setmembers `PostProcessSettings` :`StructRef` (`CameraComponent.PostProcessSettings` _playercamera) :`DepthOfFieldSensorWidth` 70.0 :`DepthOfFieldSqueezeFactor` 1.0 :`DepthOfFieldFocalDistance` (`KismetMathLibrary.Vector_Distance` (`SceneComponent.K2_GetComponentLocation` _playercamera) (`SceneComponent.K2_GetComponentLocation` (`Character.CapsuleComponent` _player_character))) :`DepthOfFieldDepthBlurAmount` 1.0 :`DepthOfFieldDepthBlurRadius` 2.0)
  (`self.AlignToSurfaceNormal`))

(event `/Game/Blueprints/PlayerCharacter/BPI_InputHandler.IA_Look`
  (params (X :type "Float (double-precision)") (Y :type "Float (double-precision)"))
  (`Pawn.AddControllerYawInput` (`self.Player Character_0`) X)
  (`Pawn.AddControllerPitchInput` (`self.Player Character_0`) (* Y -1.0)))

(event `/Game/Blueprints/PlayerCharacter/BPI_InputHandler.IA_Dash_Trigger`
  (if (`NavMovementComponent.IsFalling` (`Character.CharacterMovement` (`self.Player Character`)))
    (if (`/Game/Blueprints/PlayerCharacter/BP_PlayerCharacter.CanCloseFly` (`self.Player Character`))
      (`/Game/Blueprints/PlayerCharacter/BP_PlayerFSM.Change State` (`self.FSM`) "NewEnumerator1"))
    (else
      (`Character.Jump` (`self.Player Character`))
      (`/Game/Blueprints/PlayerCharacter/BP_PlayerCharacter.OnJump` (`self.Player Character_0`))
      (`NiagaraFunctionLibrary.SpawnSystemAtLocation` "/Game/VFX/VFX/DashVFX/VFX/NS_Jump.NS_Jump" (`Actor.K2_GetActorLocation` (`self.Player Character`))))))

(fn `AlignToSurfaceNormal`
  (bind _returnvalue (`Actor.K2_GetActorLocation` (`self.Player Character`)))
  (bind _capsulecomponent (`Character.CapsuleComponent` (`self.Player Character`)))
  (bind (_returnvalue_roll _returnvalue_pitch _returnvalue_yaw) (`KismetMathLibrary.BreakRotator` (`SceneComponent.K2_GetComponentRotation` _capsulecomponent)))
  (bind (_outhit _returnvalue_2) (`KismetSystemLibrary.LineTraceSingle` :`Start` _returnvalue :`End` (+ _returnvalue (0.0 0.0 -20.0)) :`TraceChannel` "TraceTypeQuery1" :`DrawDebugType` "ForOneFrame"))
  (if _returnvalue_2
    (bind (_bblockinghit _binitialoverlap _time _distance _location _impactpoint _normal _impactnormal) (`GameplayStatics.BreakHitResult` _outhit))
    (`KismetSystemLibrary.DrawDebugLine` _impactpoint (+ _impactpoint (* _impactnormal 60.0)) (struct :`R` 1.0 :`B` 0.418797 :`A` 1.0) (`GameplayStatics.GetWorldDeltaSeconds`) 1.0)
    (`SceneComponent.K2_SetWorldRotation` (`Character.CapsuleComponent` (`self.Player Character`)) (`KismetMathLibrary.RInterpTo` (`SceneComponent.K2_GetComponentRotation` (`Character.CapsuleComponent` (`self.Player Character`))) (`KismetMathLibrary.MakeRotator` (.roll (`KismetMathLibrary.MakeRotFromXZ` (`SceneComponent.GetForwardVector` _capsulecomponent) _impactnormal)) (.pitch (`KismetMathLibrary.MakeRotFromYZ` (`SceneComponent.GetRightVector` _capsulecomponent) _impactnormal)) _returnvalue_yaw) (`GameplayStatics.GetWorldDeltaSeconds`) 20.0) false false)))

(fn `SetCameraOffset`
  (bind _cameraboom (`/Game/Blueprints/PlayerCharacter/BP_PlayerCharacter.CameraBoom` (`self.Player Character`)))
  (set `SpringArmComponent.TargetOffset` (0.0 0.0 50.0) _cameraboom)
  (set `SpringArmComponent.TargetArmLength` 250.0 _cameraboom))

(fn `Walking`
  (bind (_returnvalue_x _returnvalue_y) (`KismetMathLibrary.BreakVector2D` (`|GetInputActionValue`)))
  (bind (_returnvalue_roll _returnvalue_pitch _returnvalue_yaw) (`KismetMathLibrary.BreakRotator` (`Pawn.GetControlRotation` (`self.Player Character_0`))))
  (bind _returnvalue (`KismetMathLibrary.MakeRotator` 0.0 0.0 _returnvalue_yaw))
  (`Pawn.AddMovementInput` (`self.Player Character_0`) (`KismetMathLibrary.GetForwardVector` _returnvalue) _returnvalue_y false)
  (`Pawn.AddMovementInput` (`self.Player Character_0`) (`KismetMathLibrary.GetRightVector` _returnvalue) _returnvalue_x false))
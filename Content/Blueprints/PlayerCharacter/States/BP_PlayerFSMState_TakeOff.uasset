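; Player FSM state for the bird's take-off: switches movement to Flying, resets the camera and starts a short vertical launch.
; A brief tween pushes the character upward, leaning slightly along camera forward, while an overhead line trace finds no obstruction.
; Once launched, dash (with a flap), forward move or accelerate input changes the FSM state.
; An older sphere-trace direction search and its angled take-off remain but are disconnected.
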(event `self.Start`
  (bind _player_character (`self.Player Character`))
  (bind _charactermovement (`Character.CharacterMovement` _player_character))
  (`parent.Start`)
  (`/Game/Blueprints/PlayerCharacter/BP_PlayerCharacter.OnTakeoff` (`self.Player Character`))
  (`/Game/Blueprints/PlayerCharacter/BP_PlayerCharacter.ResetCameraPosition` _player_character)
  (`CharacterMovementComponent.SetMovementMode` _charactermovement "MOVE_Flying" 0)
  (set `CharacterMovementComponent.bUseControllerDesiredRotation` true _charactermovement)
  (set `CharacterMovementComponent.bOrientRotationToMovement` false _charactermovement)
  (set `self.AutoAimDirection` (`/Game/Blueprints/PlayerCharacter/BP_PlayerCharacter.AutoAimDirection` (`self.Player Character`)))
  (set `self.SuitableYaw` 0.0)
  (`self.FindSuitableTakeOffDirection`)
  (setmembers `PostProcessSettings` :`StructRef` (`CameraComponent.PostProcessSettings` (`/Game/Blueprints/PlayerCharacter/BP_PlayerCharacter.PlayerCamera` (`self.Player Character`))) :`DepthOfFieldSensorWidth` 24.0 :`DepthOfFieldSqueezeFactor` 1.0 :`DepthOfFieldFocalDistance` 0.0 :`DepthOfFieldDepthBlurAmount` 0.0 :`DepthOfFieldDepthBlurRadius` 2.0))

(event `FindSuitableTakeOffDirection`
  (`self.VerticalTakeOff`))

(event `InitTakeOff`
  (bind (_returnvalue_x _returnvalue_y) (`KismetMathLibrary.BreakVector2D` (`WidgetLayoutLibrary.GetViewportSize`)))
  (bind _player_character (`self.Player Character`))
  (set `self.InitialControlRotation` (`Controller.GetControlRotation` (`Pawn.GetController` (`self.Player Character`))))
  (`/Game/Blueprints/PlayerCharacter/BP_PlayerCharacter.ResetCameraDIrection` (`self.Player Character`))
  (bind (_asynctaskproxy _value) (`FCTweenBPActionFloat.TweenFloat` 0.0)
    (:`then`
      (`/Game/Blueprints/PlayerCharacter/BP_PlayerCharacter.Flap` (`self.Player Character`))
      (bind (_asynctaskproxy_2 _value_2) (`FCTweenBPActionRotator.TweenRotator` (`SceneComponent.RelativeRotation` (`/Game/Blueprints/PlayerCharacter/BP_PlayerCharacter.TakeOffDirection` (`self.Player Character`))) (struct) 3.0)))
    (:`ApplyEasing`
      (`Pawn.AddMovementInput` _player_character (`SceneComponent.GetForwardVector` (`/Game/Blueprints/PlayerCharacter/BP_PlayerCharacter.TakeOffDirection` _player_character)) 1.0 false))
    (:`OnComplete`
      (`PlayerController.SetMouseLocation` (`GameplayStatics.GetPlayerController` 0) (`KismetMathLibrary.FTrunc` (/ _returnvalue_x 2.0)) (`KismetMathLibrary.FTrunc` (/ _returnvalue_y 2.0)))
      (`self.ActivatePointer`)
      (`/Game/Blueprints/PlayerCharacter/BP_PlayerFSM.Change State` (`self.FSM`) "NewEnumerator2"))))

(event `VerticalTakeOff`
  (bind _player_character (`self.Player Character`))
  (bind _player_character_2 (`self.Player Character`))
  (bind (_returnvalue_x _returnvalue_y) (`KismetMathLibrary.BreakVector` (`SceneComponent.GetForwardVector` (`/Game/Blueprints/PlayerCharacter/BP_PlayerCharacter.PlayerCamera` (`self.Player Character`)))))
  (`/Game/Blueprints/PlayerCharacter/BP_PlayerCharacter.ResetCameraDIrection` (`self.Player Character`))
  (set `/Game/Blueprints/PlayerCharacter/BP_PlayerCharacter.BirdFlyingState` "NewEnumerator3" _player_character)
  (set `/Game/Blueprints/PlayerCharacter/BP_PlayerCharacter.CurrentPlayerState` "NewEnumerator4" _player_character)
  (`FCTweenBPActionFloat.TweenFloat` 0.0 1.0 0.1
    (:`ApplyEasing`
      (bind (_outhit _returnvalue) (`KismetSystemLibrary.LineTraceSingle` :`Start` (`Actor.K2_GetActorLocation` _player_character_2) :`End` (+ (`Actor.K2_GetActorLocation` _player_character_2) (0.0 0.0 500.0)) :`TraceChannel` "TraceTypeQuery1" :`DrawDebugType` "ForOneFrame"))
      (if (not _returnvalue)
        (`Pawn.AddMovementInput` (`self.Player Character`) (`KismetMathLibrary.MakeVector` (* _returnvalue_x 0.1) (* _returnvalue_y 0.1) 1.0) 1.0 false)))
    (:`OnComplete`
      (set `self.VerticalLaunch` true))))

(event `self.Tick`
  (if (`self.VerticalLaunch`)
    _))

(event `/Game/Blueprints/PlayerCharacter/BPI_InputHandler.IA_Look`
  (params (X :type "Float (double-precision)") (Y :type "Float (double-precision)"))
  (`Pawn.AddControllerPitchInput` (`/Game/Blueprints/PlayerCharacter/BP_PlayerFSM.PlayerCharacter` (`self.FSM`)) (* Y -1.0))
  (`Pawn.AddControllerYawInput` (`/Game/Blueprints/PlayerCharacter/BP_PlayerFSM.PlayerCharacter` (`self.FSM`)) X))

(event `/Game/Blueprints/PlayerCharacter/BPI_InputHandler.IA_Dash_Trigger`
  (bind (_returnvalue_x _returnvalue_y) (`KismetMathLibrary.BreakVector2D` (`WidgetLayoutLibrary.GetViewportSize`)))
  (if (`self.VerticalLaunch`)
    (`/Game/Blueprints/PlayerCharacter/BP_PlayerCharacter.Flap` (`/Game/Blueprints/PlayerCharacter/BP_PlayerFSM.PlayerCharacter` (`self.FSM`)))
    (`self.ActivatePointer`)
    (`PlayerController.SetMouseLocation` (`GameplayStatics.GetPlayerController` 0) (`KismetMathLibrary.FTrunc` (/ _returnvalue_x 2.0)) (`KismetMathLibrary.FTrunc` (/ _returnvalue_y 2.0)))
    (`/Game/Blueprints/PlayerCharacter/BP_PlayerFSM.Change State` (`self.FSM`) "NewEnumerator2")))

(event `/Game/Blueprints/PlayerCharacter/BPI_InputHandler.IA_Move`
  (params (X :type "Float (double-precision)") (Y :type "Float (double-precision)"))
  (if (and (> Y 0.0) (`self.VerticalLaunch`))
    (`/Game/Blueprints/PlayerCharacter/BP_PlayerFSM.Change State` (`self.FSM`) "NewEnumerator2" :!label _label)))

(event `/Game/Blueprints/PlayerCharacter/BPI_InputHandler.IA_Accelerate`
  (params (Value :type "Float (double-precision)"))
  (if (and (> Value 0.0) (`self.VerticalLaunch`))
    (goto _label)))
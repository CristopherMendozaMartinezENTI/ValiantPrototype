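; Player helper component that steers the character's auto-aim direction and assists movement near ground and walls.
; Once SetVariables supplies references, Tick aims along the camera or turns by input, then at high max speed levels pitch to the traced ground slope.
; In one movement state, side traces ease ExtraPitch by wall distance.
; A forward obstacle query is exposed; older sphere and radial trace steering is disconnected.
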(event `self.ReceiveBeginPlay`
  (bind _asbp_player_character (cast `/Game/Blueprints/PlayerCharacter/BP_PlayerCharacter` (`self.GetOwner`)))
  (bind _output_get (set `self.As Pawn` _asbp_player_character))
  (`Actor.EnableInput` _output_get (`GameplayStatics.GetPlayerController` 0)))

(event `self.ReceiveTick`
  (params (DeltaSeconds :type "Float (single-precision)"))
  (if (and (`self.IsActive`) (`self.IsValidated`))
    (`self.SetStandardDirection`)
    (`self.HorizontalWallAnimationTraces`)
    (`self.DoGroundAutoControl`)))

(fn `DoGroundAutoControl`
  (bind (_returnvalue_roll _returnvalue_pitch _returnvalue_yaw) (`KismetMathLibrary.BreakRotator` (`self.GetStandardDirection`)))
  (bind _returnvalue (`Actor.K2_GetActorLocation` (`self.As Pawn`)))
  (if (and (`self.GroundAutoControl`) (< (`/Game/Blueprints/PlayerCharacter/BP_PlayerCharacter.MoveY` (`self.As Pawn`)) 0.5) (> (`/Game/Blueprints/PlayerCharacter/BP_PlayerFSMState.Get Max Velocity` (`/Game/Blueprints/PlayerCharacter/BP_PlayerFSM.GetCurrentState` (`/Game/Blueprints/PlayerCharacter/BP_PlayerCharacter.Player State Machine` (`self.As Pawn`)))) 1400.0))
    (bind (_outhit _returnvalue_2) (`KismetSystemLibrary.LineTraceSingle` :`Start` _returnvalue :`End` (+ _returnvalue (+ (* (`Actor.GetActorForwardVector` (`self.As Pawn`)) 600.0) (0.0 0.0 -150.0))) :`TraceChannel` "TraceTypeQuery3" :`DrawDebugType` "ForOneFrame" :`TraceColor` (struct :`R` 1.0 :`B` 0.947897 :`A` 1.0)))
    (if _returnvalue_2
      (bind (_returnvalue_roll_2 _returnvalue_pitch_2) (`KismetMathLibrary.BreakRotator` (`KismetMathLibrary.Conv_VectorToRotator` (`KismetMathLibrary.Cross_VectorVector` (`Actor.GetActorRightVector` (`self.As Pawn`)) (`.ImpactNormal` (`GameplayStatics.BreakHitResult` _outhit))))))
      (`SceneComponent.K2_SetWorldRotation` (`self.AutoaimDirection`) (`KismetMathLibrary.RInterpTo` (`SceneComponent.K2_GetComponentRotation` (`self.AutoaimDirection`)) (`KismetMathLibrary.MakeRotator` _returnvalue_roll (`KismetMathLibrary.Lerp` _returnvalue_pitch_2 _returnvalue_pitch (`KismetMathLibrary.FClamp` (`/Game/Blueprints/PlayerCharacter/BP_PlayerCharacter.MoveY` (`self.As Pawn`)))) _returnvalue_yaw) (`GameplayStatics.GetWorldDeltaSeconds`) 60.0) false false))))

(fn `GetIfForwardIsNearObstacle`
  (returns (ReturnValue :type Boolean))
  (locals (LinetraceLength :type "Float (single-precision)" :default 500.0))
  (bind _as_pawn (`self.As Pawn`))
  (bind _returnvalue (`Actor.K2_GetActorLocation` _as_pawn))
  (if (not (> (`/Game/Blueprints/PlayerCharacter/BP_PlayerCharacter.Pitch` _as_pawn) 10.0))
    (bind (_outhit _returnvalue_2) (`KismetSystemLibrary.LineTraceSingle` :`Start` _returnvalue :`End` (+ _returnvalue (* (`SceneComponent.GetForwardVector` (`/Game/Blueprints/PlayerCharacter/BP_PlayerCharacter.PlayerCamera` _as_pawn)) (`local.LinetraceLength`))) :`TraceChannel` "TraceTypeQuery1" :`DrawDebugType` "ForDuration"))
    (return (and _returnvalue_2 (< (`KismetMathLibrary.Abs` (`KismetMathLibrary.Dot_VectorVector` (`.Normal` (`GameplayStatics.BreakHitResult` _outhit)) (0.0 0.0 1.0))) 0.5)))
    (else
      (return false))))

(fn `GetStandardDirection`
  (returns (ReturnValue :type "Rotator Structure"))
  (return (`SceneComponent.K2_GetComponentRotation` (`self.Player Camera`))))

(fn `HorizontalLinetraces`
  (bind _returnvalue (`self.GetOwner`))
  (bind _autoaimdirection (`self.AutoaimDirection`))
  (bind _as_pawn (`self.As Pawn`))
  (bind _returnvalue_2 (`Actor.K2_GetActorLocation` _returnvalue))
  (for _index (range 19)
    (bind (_outhit _returnvalue_3) (`KismetSystemLibrary.LineTraceSingle` _returnvalue_2 (+ _returnvalue_2 (* (`KismetMathLibrary.RotateAngleAxis` (`Actor.GetActorForwardVector` _returnvalue) (* _index 20.0) (0.0 0.0 1.0)) (`self.LinetraceLength`))) "TraceTypeQuery1"))
    (if _returnvalue_3
      (bind (_bblockinghit _binitialoverlap _time _distance _location _impactpoint _normal) (`GameplayStatics.BreakHitResult` _outhit))
      (bind _returnvalue_4 (`KismetMathLibrary.Conv_VectorToRotator` _normal))
      (`SceneComponent.K2_SetWorldRotation` _autoaimdirection (`KismetMathLibrary.RInterpTo` (`SceneComponent.K2_GetComponentRotation` _autoaimdirection) _returnvalue_4 (`GameplayStatics.GetWorldDeltaSeconds`) 0.1) false false)
      (`Pawn.AddMovementInput` (`PawnMovementComponent.GetPawnOwner` (`self.Character Movement`)) _normal 1.0 false)
      (`Controller.SetControlRotation` (`Pawn.GetController` _as_pawn) (`KismetMathLibrary.RInterpTo` (`Pawn.GetControlRotation` _as_pawn) _returnvalue_4 (`GameplayStatics.GetWorldDeltaSeconds`) 0.1)))))

(fn `HorizontalWallAnimationTraces`
  (bind _returnvalue (`GameplayStatics.GetWorldDeltaSeconds`))
  (bind _returnvalue_2 (`GameplayStatics.GetWorldDeltaSeconds`))
  (bind _as_pawn (`self.As Pawn`))
  (bind _as_pawn_2 (`self.As Pawn`))
  (bind _returnvalue_3 (`Actor.K2_GetActorLocation` _as_pawn_2))
  (bind _returnvalue_4 (`Actor.K2_GetActorLocation` _as_pawn))
  (if (and (`|EnumEquality` (`.CurrentStateEnum` (`/Game/Blueprints/PlayerCharacter/BP_PlayerFSM.GetCurrentState` (`/Game/Blueprints/PlayerCharacter/BP_PlayerCharacter.Player State Machine` (`self.As Pawn`)))) "NewEnumerator2") true)
    (`|ExecutionSequence`
      (:`then_0`
        (bind (_outhit _returnvalue_5) (`KismetSystemLibrary.LineTraceSingle` _returnvalue_3 (+ _returnvalue_3 (* (`Actor.GetActorRightVector` _as_pawn_2) 250.0)) "TraceTypeQuery1"))
        (if _returnvalue_5
          (set `self.ExtraPitch` (`KismetMathLibrary.FInterpTo` (`self.ExtraPitch`) (`KismetMathLibrary.MapRangeClamped` (`.Distance` (`GameplayStatics.BreakHitResult` _outhit)) 50.0 250.0 -180.0) _returnvalue_2 1.0))
          (else
            (set `self.ExtraPitch` (`KismetMathLibrary.FInterpTo` (`self.ExtraPitch`) 0.0 _returnvalue_2 1.0)))))
      (:`then_1`
        (bind (_outhit_2 _returnvalue_6) (`KismetSystemLibrary.LineTraceSingle` _returnvalue_4 (+ _returnvalue_4 (* (`Actor.GetActorRightVector` _as_pawn) -250.0)) "TraceTypeQuery1"))
        (if _returnvalue_6
          (set `self.ExtraPitch` (`KismetMathLibrary.FInterpTo` (`self.ExtraPitch`) (`KismetMathLibrary.MapRangeClamped` (`.Distance` (`GameplayStatics.BreakHitResult` _outhit_2)) 50.0 250.0 180.0) _returnvalue 1.0))
          (else
            (set `self.ExtraPitch` (`KismetMathLibrary.FInterpTo` (`self.ExtraPitch`) 0.0 _returnvalue 1.0))))))
    (`KismetSystemLibrary.PrintString` (`KismetStringLibrary.Concat_StrStr` "EXTRA PITCH: " (`KismetStringLibrary.Conv_DoubleToString` (`self.ExtraPitch`))) true true (struct :`G` 0.66 :`B` 1.0 :`A` 1.0) 2.0 "eXTRAPITCH")
    (else
      (set `self.ExtraPitch` (`KismetMathLibrary.FInterpTo` (`self.ExtraPitch`) 0.0 (`GameplayStatics.GetWorldDeltaSeconds`) 1.0)))))

(fn `SetStandardDirection`
  (returns (ReturnValue :type "Rotator Structure"))
  (locals (Speed :type "Float (double-precision)" :default 1000.0))
  (bind _autoaimdirection (`self.AutoAimDirection`))
  (bind _returnvalue (`SceneComponent.K2_GetComponentRotation` (`self.Player Camera`)))
  (if (`self.FollowPlayerCamera`)
    (`SceneComponent.K2_SetWorldRotation` _autoaimdirection _returnvalue false false)
    (else
      (`SceneComponent.K2_SetWorldRotation` _autoaimdirection (`KismetMathLibrary.Conv_VectorToRotator` (`KismetMathLibrary.RotateAngleAxis` (`SceneComponent.GetForwardVector` (`self.AutoAimDirection`)) (* (`GameplayStatics.GetWorldDeltaSeconds`) (`/Game/Blueprints/PlayerCharacter/BP_PlayerCharacter.MoveX` (`self.As Pawn`)) (`local.Speed`)) (0.0 0.0 1.0))) false false)))
  (return _returnvalue))

(fn `SetVariables`
  (params (AutoaimDirection :type "ArrowComponent Object Reference") (`Character Movement` :type "CharacterMovementComponent Object Reference") (Mesh :type "SkeletalMeshComponent Object Reference") (`Capsule Component` :type "CapsuleComponent Object Reference") (`Player Camera` :type "CameraComponent Object Reference"))
  (set `self.AutoaimDirection` AutoaimDirection)
  (set `self.Character Movement` `Character Movement`)
  (set `self.Mesh` Mesh)
  (set `self.Capsule Component` `Capsule Component`)
  (set `self.Player Camera` `Player Camera`)
  (set `self.IsValidated` true))

(fn `TempTraces`
  (bind (_returnvalue_roll _returnvalue_pitch _returnvalue_yaw) (`KismetMathLibrary.BreakRotator` (`KismetMathLibrary.Conv_VectorToRotator` (`SceneComponent.GetForwardVector` (`self.Player Camera`)))))
  (bind _returnvalue (+ (`SceneComponent.K2_GetComponentLocation` (`self.Mesh`)) (0.0 0.0 0.0)))
  (bind (_outhit _returnvalue_2) (`KismetSystemLibrary.SphereTraceSingle` _returnvalue _returnvalue 100.0 "TraceTypeQuery1"))
  (if _returnvalue_2
    (bind _returnvalue_3 (`KismetMathLibrary.Cross_VectorVector` (`SceneComponent.GetRightVector` (`self.Capsule Component`)) (`.Normal` (`GameplayStatics.BreakHitResult` _outhit))))
    (`CharacterMovementComponent.AddForce` (`self.Character Movement`) (* _returnvalue_3 1000.0))
    (bind (_returnvalue_roll_2 _returnvalue_pitch_2) (`KismetMathLibrary.BreakRotator` (`KismetMathLibrary.Conv_VectorToRotator` _returnvalue_3)))
    (`SceneComponent.K2_SetWorldRotation` (`self.AutoAimDirection`) (`KismetMathLibrary.MakeRotator` _returnvalue_roll (`KismetMathLibrary.SelectFloat` _returnvalue_pitch _returnvalue_pitch_2 (> _returnvalue_pitch 10.0)) _returnvalue_yaw) false false)))
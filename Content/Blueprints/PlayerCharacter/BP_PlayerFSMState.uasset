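; Player state for the character's finite state machine, apparently a base for specific states given its empty Tick and End.
; Start caches the player character from the FSM and applies its PlayerStats.
; InterpolatePitchAndRoll smoothly banks the mesh by clamped turn offset and tilts it along the velocity direction, storing pitch on the character.
; Pitch and roll axes are swapped to suit the mesh's -90 yaw.
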(event `Start`
  (bind _playercharacter (`/Game/Blueprints/PlayerCharacter/BP_PlayerFSM.PlayerCharacter` (`self.FSM`)))
  (set `self.Player Character` _playercharacter)
  (`/Game/Blueprints/PlayerCharacter/DA_PlayerStats.ApplyStats` (`/Game/Blueprints/PlayerCharacter/BP_PlayerCharacter.PlayerStats` _playercharacter) _playercharacter))

(event `Tick`)

(event `End`)

(fn `InterpolatePitchAndRoll`
  (bind (_returnvalue_roll _returnvalue_pitch) (`KismetMathLibrary.BreakRotator` (`KismetMathLibrary.Conv_VectorToRotator` (`Actor.GetVelocity` (`self.Player Character`)))))
  (bind _relativerotation_roll (`KismetMathLibrary.BreakRotator` (`SceneComponent.RelativeRotation` (`Character.Mesh` (`self.Player Character`)))))
  (set `self.Roll` (`KismetMathLibrary.FInterpTo` (`self.Roll`) (`KismetMathLibrary.FClamp` (`self.Turn Direction Offset`) -60.0 60.0) (`GameplayStatics.GetWorldDeltaSeconds`) 10.0))
  (`SceneComponent.K2_SetRelativeRotation` (`Character.Mesh` (`self.Player Character`)) (`KismetMathLibrary.MakeRotator` (`self.Pitch`) (`self.Roll`) -90.0) false false)
  (bind _output_get (set `self.Pitch` (`KismetMathLibrary.FInterpTo` _relativerotation_roll (* _returnvalue_pitch -1.0) (`GameplayStatics.GetWorldDeltaSeconds`) 50.0)))
  (set `/Game/Blueprints/PlayerCharacter/BP_PlayerCharacter.Pitch` _output_get (`self.Player Character`)))
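; Finite state machine on the player character that switches it between ground and flight states such as walking, take-off, flying, landing and collision.
; On BeginPlay it adds each state object to the owning character, maps it by enum and enters the first, Walking.
; ChangeState ends the old state, starts the new one and routes character input to it.
; Tick forwards to the current state, with debug prints.
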(event `self.ReceiveBeginPlay`
  (bind _asbp_player_character (cast `/Game/Blueprints/PlayerCharacter/BP_PlayerCharacter` (`self.GetOwner`)))
  (set `self.PlayerCharacter` _asbp_player_character)
  (`self.InitializeStates`)
  (`/Game/Blueprints/PlayerCharacter/BP_PlayerCharacter.SetCurrentInputHandler` (`self.PlayerCharacter`) (`self.CurrentState`))
  (`self.Change State` "NewEnumerator0")
  (`self.OnFSMFinishedInitializing`)
  (set `self.IsRunning` true))

(event `Change State`
  (params (Key :type "/Game/Blueprints/PlayerCharacter/EPlayerStates Enum" :default "NewEnumerator0"))
  (`KismetSystemLibrary.PrintString` (`self.PlayerCharacter`) "Changing state")
  (bind _currentstate (`self.CurrentState`)
    (:`then`
      ;[1 1 1] End the old state
      (`/Game/Blueprints/PlayerCharacter/BP_PlayerFSMState.End` _currentstate))
    (:`else`
      _))
  (set `self.CurrentState` (`BlueprintMapLibrary.Map_Find` (`self.States`) Key))
  (set `self.CurrentStateEnum` Key)
  ;[1 1 1] Start the new state
  (`/Game/Blueprints/PlayerCharacter/BP_PlayerFSMState.Start` (`self.CurrentState`))
  ;[1 1 1] Redirect input to new state
  (`/Game/Blueprints/PlayerCharacter/BP_PlayerCharacter.SetCurrentInputHandler` (`self.PlayerCharacter`) (`self.CurrentState`))
  (set `/Game/Blueprints/PlayerCharacter/BP_PlayerCharacter.CurrentPlayerState` Key (`self.PlayerCharacter`)))

(event `self.ReceiveTick`
  (params (DeltaSeconds :type "Float (single-precision)"))
  (`self.OnFinishFSMTick`)
  (`KismetSystemLibrary.PrintString` (`|GetEnumeratorNameAsString` (`self.CurrentStateEnum`)) true true (struct :`R` 1.0 :`G` 0.891546 :`A` 1.0) 2.0 "CurentState")
  (`/Game/Blueprints/PlayerCharacter/BP_PlayerFSMState.Tick` (`self.CurrentState`)))

(fn `GetCurrentState`
  (returns (CurrentState :type "/Game/Blueprints/PlayerCharacter/BP_PlayerFSMState Object Reference") (CurrentStateEnum :type "/Game/Blueprints/PlayerCharacter/EPlayerStates Enum"))
  (return (`self.CurrentState`) (`self.CurrentStateEnum`)))

(fn `InitializeStates`
  (`|ExecutionSequence`
    (:`then_0`
      (bind _returnvalue (`|AddComponentByClass` (`self.PlayerCharacter`) "/Game/Blueprints/PlayerCharacter/States/BP_PlayerFSMState_Walking.BP_PlayerFSMState_Walking_C" self))
      (`BlueprintMapLibrary.Map_Add` (`self.States`) "NewEnumerator0" _returnvalue))
    (:`then_1`
      (bind _returnvalue_2 (`|AddComponentByClass` (`self.PlayerCharacter`) "/Game/Blueprints/PlayerCharacter/States/BP_PlayerFSMState_TakeOff.BP_PlayerFSMState_TakeOff_C" self))
      (`BlueprintMapLibrary.Map_Add` (`self.States`) "NewEnumerator1" _returnvalue_2))
    (:`then_2`
      (bind _returnvalue_3 (`|AddComponentByClass` (`self.PlayerCharacter`) "/Game/Blueprints/PlayerCharacter/States/BP_PlayerFSMState_Flying.BP_PlayerFSMState_Flying_C" self))
      (`BlueprintMapLibrary.Map_Add` (`self.States`) "NewEnumerator2" _returnvalue_3))
    (:`then_3`
      (bind _returnvalue_4 (`|AddComponentByClass` (`self.PlayerCharacter`) "/Game/Blueprints/PlayerCharacter/States/BP_PlayerFSMState_Landing.BP_PlayerFSMState_Landing_C" self))
      (`BlueprintMapLibrary.Map_Add` (`self.States`) "NewEnumerator3" _returnvalue_4))
    (:`then_4`
      (bind _returnvalue_5 (`|AddComponentByClass` (`self.PlayerCharacter`) "/Game/Blueprints/PlayerCharacter/States/BP_PlayerFSMState_Braking.BP_PlayerFSMState_Braking_C" self))
      (`BlueprintMapLibrary.Map_Add` (`self.States`) "NewEnumerator4" _returnvalue_5))
    (:`then_5`
      (bind _returnvalue_6 (`|AddComponentByClass` (`self.PlayerCharacter`) "/Game/Blueprints/PlayerCharacter/States/BP_PlayerFSMState_Collision.BP_PlayerFSMState_Collision_C" self))
      (`BlueprintMapLibrary.Map_Add` (`self.States`) "NewEnumerator5" _returnvalue_6))
    (:`then_6`
      (bind _returnvalue_7 (`|AddComponentByClass` (`self.PlayerCharacter`) "/Game/Blueprints/PlayerCharacter/States/BP_PlayerFSMState_CloseFlying.BP_PlayerFSMState_CloseFlying_C" self))
      (`BlueprintMapLibrary.Map_Add` (`self.States`) "NewEnumerator6" _returnvalue_7))))
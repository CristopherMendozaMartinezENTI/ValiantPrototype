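; Player camera manager for the Valiant player character that caches its camera component and snaps to that camera's transform on BeginPlay.
; UpdateCamFlying adds a height offset in two player states, eased out as smoothed sideways MoveX input grows.
; BlueprintUpdateCamera returns false and its UpdateCamFlying call is disconnected, so the custom view is inactive.
; ShouldUpdateRotation, a control-rotation angle check, is also unused.
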(event EventBeginPlay
  (bind _returnvalue (Game|GetPlayerCharacter 0))
  (bind _asbp_player_character (Utilities|Casting|CastToBP_PlayerCharacter _returnvalue))
  (Variables|Default|SetAs%20BP%20Player%20Character _asbp_player_character)
  (Variables|Default|SetPlayer%20Camera (Variables|/Game/Blueprints/PlayerCharacter/BP_PlayerCharacter.BP_PlayerCharacter_C|GetPlayerCamera _asbp_player_character))
  (Transformation|SetWorldTransform (Variables|Default|GetTransformComponent) (Transformation|GetWorldTransform (Variables|Default|GetPlayer%20Camera)) false true))

(event Collision|EventActorBeginOverlap
  (params (OtherActor :type Actor%20Object%20Reference)))

(event EventTick
  (params (DeltaSeconds :type Float%20%28single-precision%29)))

(fn ConstructionScript)

(fn BlueprintUpdateCamera
  (params (CameraTarget :type Actor%20Object%20Reference))
  (return (stale _camloc) (stale _camrot) (stale _fov) false))

(fn UpdateCamFlying
  (params (CamLocIn :type Vector) (CamRotIn :type Rotator) (FovIn :type Float%20%28double-precision%29))
  (bind _as_bp_player_character (Variables|Default|GetAs%20BP%20Player%20Character))
  (bind _player_state_machine (Variables|/Game/Blueprints/PlayerCharacter/BP_PlayerCharacter.BP_PlayerCharacter_C|GetPlayer%20State%20Machine _as_bp_player_character))
  (bind _currentstateenum (Default|GetCurrentState _player_state_machine))
  (if (or (Utilities|Enum|Equal(Enum) _currentstateenum "NewEnumerator2") (Utilities|Enum|Equal(Enum) _currentstateenum "NewEnumerator6"))
    (Variables|Default|SetInterpMoveX (Math|Interpolation|FInterpTo (Variables|Default|GetInterpMoveX) (Math|Float|Absolute(Float) (Variables|/Game/Blueprints/PlayerCharacter/BP_PlayerCharacter.BP_PlayerCharacter_C|GetMoveX (Variables|Default|GetAs%20BP%20Player%20Character))) (Utilities|Time|GetWorldDeltaSeconds) 1.0))
    (return (Math|Vector|Lerp(Vector) (+ CamLocIn "0.000000,0.000000,80.000000") CamLocIn (Math|Interpolation|FInterpTo (Variables|Default|GetInterpMoveX) (Math|Float|Absolute(Float) (Variables|/Game/Blueprints/PlayerCharacter/BP_PlayerCharacter.BP_PlayerCharacter_C|GetMoveX (Variables|Default|GetAs%20BP%20Player%20Character))) (Utilities|Time|GetWorldDeltaSeconds) 1.0)) CamRotIn FovIn)
    (else
      (return CamLocIn CamRotIn FovIn))))

(fn ShouldUpdateRotation
  (if (> (Math|Float|Absolute(Float) (Variables|/Game/Blueprints/PlayerCharacter/BP_PlayerCharacter.BP_PlayerCharacter_C|GetMoveX (Variables|Default|GetAs%20BP%20Player%20Character))) 0.1)
    (if (> (Class|KismetMathLibrary|DegAcos (Math|Vector|DotProduct (Math|Vector|GetForwardVector (Variables|Default|GetLatestControlRot)) (Math|Vector|GetForwardVector (Variables|Default|GetTransformComponent)))) 1e+01)
      (return false (Transformation|GetWorldRotation (Variables|Default|GetPlayer%20Camera)))
      (else
        (return false (Transformation|GetWorldRotation (Variables|Default|GetTransformComponent)))))
    (else
      (Variables|Default|SetLatestControlRot (Transformation|GetWorldRotation (Variables|Default|GetPlayer%20Camera))))))
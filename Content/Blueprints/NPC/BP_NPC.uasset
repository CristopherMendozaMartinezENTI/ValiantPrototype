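; BP_NPC is an NPC Blueprint that supports dialogue and player interaction.
; On BeginPlay it caches its BP_NPC_Controller and hides its Widget, whose visibility is then set through ToggleInteractionVisibility.
; BPC_DialogueComponent events stop the controller's AI when dialogue starts and restart it when dialogue ends.
; GetInteractionState reports whether ACValiantInteractionComponent has interaction enabled.
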(event `self.ReceiveBeginPlay`
  (set `self.As BP NPC Controller` (cast `/Game/Blueprints/NPC/BP_NPC_Controller` (`AIBlueprintHelperLibrary.GetAIController` self) :!pure true))
  (`SceneComponent.SetVisibility` (`self.Widget`) false false))

(event `self.BPC_DialogueComponent.OnStartDialogue`
  (`/Game/Blueprints/NPC/BP_NPC_Controller.StopAI` (`self.As BP NPC Controller`)))

(event `self.BPC_DialogueComponent.OnEndDialogue`
  (`/Game/Blueprints/NPC/BP_NPC_Controller.StartAI` (`self.As BP NPC Controller`)))

(event `ToggleInteractionVisibility`
  (params (bNewVisibility :type Boolean))
  (`SceneComponent.SetVisibility` (`self.Widget`) bNewVisibility false))

(event `self.ReceiveTick`
  (params (DeltaSeconds :type "Float (single-precision)")))

(fn `GetInteractionState`
  (returns (InteractionEnabled :type Boolean))
  (return (`/Game/Blueprints/PROTOTYPEQuest/AC_ValiantInteractionComponent.InteractionEnabled` (`self.AC_ValiantInteractionComponent`))))

(fn `UserConstructionScript`)
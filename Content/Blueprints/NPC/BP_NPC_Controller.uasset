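; BP_NPC_Controller drives an NPC pawn to wander around the navmesh, starting on BeginPlay.
; Wander picks a random navigable point near the pawn, moves there with AIMoveTo, then waits a random few seconds before looping while AIRunning is set.
; The loop continues only from a successful move.
; StopAI halts active movement and clears AIRunning; StartAI restarts Wander and sets it again.
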(event `Wander`
  (bind _randomlocation (`NavigationSystemV1.K2_GetRandomLocationInNavigableRadius` (`self.K2_GetActorLocation` (`self.K2_GetPawn`)) 1000.0 null null :!label _label))
  (`|AIMoveTo` (`self.K2_GetPawn`) _randomlocation null
    (:`OnSuccess`
      (`KismetSystemLibrary.Delay` (`KismetMathLibrary.RandomFloatInRange` 2.0 6.0))
      (if (`self.AIRunning`)
        (goto _label)))))

(event `self.ReceiveBeginPlay`
  (`self.Wander`))

(event `StopAI`
  (`NavMovementComponent.StopActiveMovement` (`Pawn.GetMovementComponent` (`self.K2_GetPawn`)))
  (set `self.AIRunning` false))

(event `StartAI`
  (`self.Wander`)
  (set `self.AIRunning` true))

(fn `UserConstructionScript`)
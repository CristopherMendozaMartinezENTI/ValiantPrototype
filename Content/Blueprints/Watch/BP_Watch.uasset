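; Pocket watch actor that displays the game's time of day on hour and minute hands and adds the UI_HUD widget on BeginPlay.
; Each Tick maps the DayTimeManager hour to hand yaw: the hour hand turns once per 24 hours, the minute hand follows the fractional hour.
; The construction script restricts its SceneCaptureComponent2D to the watch's own components, isolating it from the scene.
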(event `self.ReceiveBeginPlay`
  (bind _returnvalue (`|CreateWidget` "/Game/UI/UI_HUD.UI_HUD_C"))
  (`UserWidget.AddToViewport` _returnvalue 0))

(event `self.ReceiveTick`
  (params (DeltaSeconds :type "Float (single-precision)"))
  (bind _hour (`/Game/Blueprints/TimeManager/BP_DayTimeManager.Get Hour` (`/Game/Blueprints/TimeManager/BPC_TimeComponent.Day Time Manager` (`self.BPC_TimeComponent`))))
  (`SceneComponent.K2_SetRelativeRotation` (`self.Pocket_Watch_Hours`) (`KismetMathLibrary.MakeRotator` 0.0 0.0 (+ (`KismetMathLibrary.MapRangeClamped` _hour 0.0 24.0 -90.0 270.0) 180.0)) false false)
  (`SceneComponent.K2_SetRelativeRotation` (`self.Pocket_Watch_Minutes`) (`KismetMathLibrary.MakeRotator` 0.0 0.0 (`KismetMathLibrary.MapRangeClamped` (mod _hour 1.0) 0.0 1.0 -90.0 270.0)) false false))

(fn `UserConstructionScript`
  (`SceneCaptureComponent.ShowOnlyActorComponents` (`self.SceneCaptureComponent2D`) self false))
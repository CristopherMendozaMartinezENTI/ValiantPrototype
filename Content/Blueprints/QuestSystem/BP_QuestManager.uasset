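; Quest manager that drives the active-quest HUD, pushing UI_ActiveQuests onto the Valiant HUD's quest layer a tick after BeginPlay.
; SetQuestData and SetQuestProgress retry every 0.2s until the widget is valid, then update text and play a punch, with a sound for new objectives.
; HideQuestHUD removes the layer and broadcasts the finished quest's name.
; StartQuest is empty, FinishQuest only prints, and IncreaseProgress increments the required item count, not progress.
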(event `self.ReceiveBeginPlay`
  (`KismetSystemLibrary.DelayUntilNextTick`)
  (bind _returnvalue (`/PMDialogue/W_OverallUILayout.PushWidgetToLayerStack` (`/Game/UI/BP_ValiantHUD.OverallWidget` (cast `/Game/UI/BP_ValiantHUD` (`PlayerController.GetHUD` (`GameplayStatics.GetPlayerController` 0)) :!pure true)) (struct :`TagName` "UI.Layer.Quests") "/Game/Blueprints/QuestSystem/UI_ActiveQuests.UI_ActiveQuests_C" :!label _label))
  (bind _asui_active_quests (cast `/Game/Blueprints/QuestSystem/UI_ActiveQuests` _returnvalue))
  (set `self.ActiveQuestHUD` _asui_active_quests)
  (set `self.WBP Quest` (`/Game/Blueprints/QuestSystem/UI_ActiveQuests.WBP_Quest` _asui_active_quests)))

(event `ShowQuestHUD`
  (goto _label))

(event `StartQuest`
  (params (`New Quest` :type "/Game/Blueprints/QuestSystem/S_Quest Structure")))

(event `SetQuestData`
  (params (S_Quest :type "/Game/Blueprints/QuestSystem/S_Quest Structure (by ref)"))
  (bind (_questflowasset _questname _questdescription) (break `/Game/Blueprints/QuestSystem/S_Quest` S_Quest))
  (bind _wbp_quest (`self.WBP Quest`))
  (bind _returnvalue (`KismetStringLibrary.Conv_NameToString` _questname))
  (`/Engine/EditorBlueprintResources/StandardMacros.IsValid` (`self.WBP Quest`) :!label _label_2
    (:`Is Valid`
      (set `self.QuestName` _returnvalue)
      (`/Game/UI/WBP_Quest.SetQuestTitleText` _wbp_quest _returnvalue)
      (`/Game/UI/WBP_Quest.SetObjectiveText` _wbp_quest (`KismetTextLibrary.Conv_TextToString` _questdescription))
      (`/Game/Blueprints/QuestSystem/UI_ActiveQuests.DoQuestPunch` (`self.ActiveQuestHUD`))
      (if (`KismetStringLibrary.EqualEqual_StrStr` (`/Game/UI/WBP_Quest.QuestTitleText` (`self.WBP Quest`)) (`KismetStringLibrary.Conv_NameToString` _questname))
        (`FMODBlueprintStatics.PlayEvent2D` "/Game/FMOD/Events/SFX/UI/NewObjective.NewObjective")))
    (:`Is Not Valid`
      (`KismetSystemLibrary.Delay` 0.2)
      (goto _label_2))))

(event `FinishQuest`
  (`KismetSystemLibrary.PrintString` "Quest finishes"))

(event `Set Objective Count`
  (`/Game/UI/WBP_Quest.SetProgressText` (`self.WBP Quest`) ""))

(event `HideQuestHUD`
  (`/PMDialogue/W_OverallUILayout.RemoveLayer` (`/Game/UI/BP_ValiantHUD.OverallWidget` (cast `/Game/UI/BP_ValiantHUD` (`PlayerController.GetHUD` (`GameplayStatics.GetPlayerController` 0)) :!pure true)) (struct :`TagName` "UI.Layer.Quests") (`self.ActiveQuestHUD`))
  (`self.OnFinishQuest` (`self.QuestName`)))

(event `SetQuestProgress`
  (params (S_Quest :type "/Game/Blueprints/QuestSystem/S_Quest Structure (by ref)"))
  (bind _wbp_quest (`self.WBP Quest`))
  (`/Engine/EditorBlueprintResources/StandardMacros.IsValid` _wbp_quest :!label _label_3
    (:`Is Valid`
      (`/Game/UI/WBP_Quest.SetProgressText` _wbp_quest (`.QuestProgression_12_18C9A8DB41486C50479F79BCC735E534` (break `/Game/Blueprints/QuestSystem/S_Quest` S_Quest)))
      (`/Game/Blueprints/QuestSystem/UI_ActiveQuests.DoQuestPunch` (`self.ActiveQuestHUD`)))
    (:`Is Not Valid`
      (`KismetSystemLibrary.Delay` 0.2)
      (goto _label_3))))

(fn `IncreaseProgress`
  (`/Engine/EditorBlueprintResources/StandardMacros.IncrementInt` (`self.NecessaryQuestItems`)
    (:`  `
      (`/Game/UI/WBP_Quest.SetProgressText` (`self.WBP Quest`) (`KismetStringLibrary.Concat_StrStr` (`KismetStringLibrary.Conv_IntToString` (`self.QuestProgress`)) "/" (`KismetStringLibrary.Conv_IntToString` (`self.NecessaryQuestItems`)))))))

(fn `RemoveQuestProgress`)

(fn `SetupQuestProgress`
  (params (NecessaryQuestItems :type Integer))
  (set `self.QuestProgress` 0)
  (set `self.NecessaryQuestItems` NecessaryQuestItems)
  (`/Game/UI/WBP_Quest.SetProgressText` (`self.WBP Quest`) (`KismetStringLibrary.Concat_StrStr` (`KismetStringLibrary.Conv_IntToString` (`self.QuestProgress`)) "/" (`KismetStringLibrary.Conv_IntToString` (`self.NecessaryQuestItems`)))))

(fn `UserConstructionScript`)
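; BP_Collectable is a pickup actor that flies into the player once touched, then disappears.
; When BP_PlayerCharacter overlaps its Sphere, it attaches the NS_GetCollectable effect to the character's mesh, plays a 2D pickup sound event, removes the Sphere and sets Collected.
; Tick then homes the actor toward player 0 with VInterpTo and destroys it once close.
; The Blueprint itself awards no score or item.
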(event `self.ReceiveTick`
  (params (DeltaSeconds :type "Float (single-precision)"))
  (bind _returnvalue (`self.K2_GetActorLocation`))
  (bind _returnvalue_2 (`self.K2_GetActorLocation` (`GameplayStatics.GetPlayerCharacter` 0)))
  (if (`self.Collected`)
    (`self.K2_SetActorLocation` (`KismetMathLibrary.VInterpTo` _returnvalue _returnvalue_2 DeltaSeconds 10.0))
    (if (< (`KismetMathLibrary.VSize` (- _returnvalue_2 _returnvalue)) 120.0)
      (`self.K2_DestroyActor`))))

(event `self.Sphere.OnComponentBeginOverlap`
  (params (OverlappedComponent :type "PrimitiveComponent Object Reference") (OtherActor :type "Actor Object Reference") (OtherComp :type "PrimitiveComponent Object Reference") (OtherBodyIndex :type Integer) (bFromSweep :type Boolean) (SweepResult :type "HitResult Structure (by ref)"))
  (bind _asbp_player_character (cast `/Game/Blueprints/PlayerCharacter/BP_PlayerCharacter` OtherActor))
  (`NiagaraFunctionLibrary.SpawnSystemAttached` "/Game/VFX/VFX/ScanVFx/VFX/NS_GetCollectable.NS_GetCollectable" (`Character.Mesh` _asbp_player_character) "None" (0.0 0.0 0.0) (struct) "KeepRelativeOffset")
  (`FMODBlueprintStatics.PlayEvent2D` "/Game/FMOD/Events/SFX/Collectables/Collectable_PickUp.Collectable_PickUp")
  (`ActorComponent.K2_DestroyComponent` (`self.Sphere`))
  (set `self.Collected` true))

(fn `UserConstructionScript`)
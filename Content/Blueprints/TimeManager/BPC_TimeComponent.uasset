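; Actor component that lets its owner react to specific in-game hours through a list of day-time events.
; On BeginPlay it binds to the ValiantPlayerController's finished-loading dispatcher, then takes the DayTimeManager from that controller.
; If timed events are enabled, it listens for each passing hour and broadcasts ExecuteDayTimeEvent for entries matching the current hour.
; AddDayTimeEvent appends entries to that list.
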(event `self.ReceiveBeginPlay`
  (`|ExecutionSequence`
    (:`then_0`
      ;[1 1 1] Get Reference
      (bind _asvaliant_player_controller (cast `/Game/Blueprints/ValiantPlayerController` (`GameplayStatics.GetPlayerController` 0)))
      (set `self.As Valiant Player Controller` _asvaliant_player_controller)
      (add `/Game/Blueprints/ValiantPlayerController.OnFinishedLoadingGame` _asvaliant_player_controller (`|CreateDelegate` :!event `OnFinishLoadingGame`)))))

(event `CheckDayTimeEvents`
  (for _array_element (`self.DayTimeEvents`)
    (if (== (`.Hour_2_125DBFD347F898BFE26F439975BA141A` (break `/Game/Blueprints/TimeManager/SDayTime` _array_element)) (`/Game/Blueprints/TimeManager/BP_DayTimeManager.Get Hour` (`self.Day Time Manager`)))
      (`self.ExecuteDayTimeEvent` _array_element))))

(event `OnFinishLoadingGame`
  (set `self.Day Time Manager` (`/Game/Blueprints/ValiantPlayerController.DayTimeManager` (`self.As Valiant Player Controller`)))
  (if (`self.Execute Timed Event`)
    (add `/Game/Blueprints/TimeManager/BP_DayTimeManager.OnPassHour` (`self.Day Time Manager`) (`|CreateDelegate` :!event `CheckDayTimeEvents`))))

(fn `AddDayTimeEvent`
  (params (`DayTime ` :type "/Game/Blueprints/TimeManager/SDayTime Structure"))
  (`KismetArrayLibrary.Array_Add` (`self.DayTimeEvents`) `DayTime `))
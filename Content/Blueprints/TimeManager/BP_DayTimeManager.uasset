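; BP_DayTimeManager runs the game's day clock, advancing a 24-hour time value held in the CurrentTime struct.
; Tick calls UpdateTime, which adds one game hour per 15 seconds of delta time, wraps at 24 and writes it through SetTime.
; It calls OnPassHour only when the float hour lands exactly on a whole number, so frame steps can skip it.
; Getters expose the hour and the full struct.
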(event `self.ReceiveTick`
  (params (DeltaSeconds :type "Float (single-precision)"))
  (`self.UpdateTime` DeltaSeconds))

(fn `Get Current Time`
  (returns (CurrentTime :type "/Game/Blueprints/TimeManager/SDayTime Structure"))
  (return (`self.CurrentTime`)))

(fn `Get Hour`
  (returns (Hour :type "Float (double-precision)"))
  (return (`.Hour_2_125DBFD347F898BFE26F439975BA141A` (break `/Game/Blueprints/TimeManager/SDayTime` (`self.CurrentTime`)))))

(fn `SetTime`
  (params (Hour :type "Float (double-precision)"))
  (setmembers `/Game/Blueprints/TimeManager/SDayTime` :`StructRef` (`self.CurrentTime`) :`Hour` Hour))

(fn `UpdateTime`
  (params (`Delta Seconds` :type "Float (double-precision)"))
  (`self.SetTime` (mod (+ (/ `Delta Seconds` 15.0) (`.Hour_2_125DBFD347F898BFE26F439975BA141A` (break `/Game/Blueprints/TimeManager/SDayTime` (`self.CurrentTime`)))) 24.0))
  (if (== (mod (`.Hour_2_125DBFD347F898BFE26F439975BA141A` (break `/Game/Blueprints/TimeManager/SDayTime` (`self.CurrentTime`))) 1.0) 0.0)
    (`self.OnPassHour`)))

(fn `UserConstructionScript`)
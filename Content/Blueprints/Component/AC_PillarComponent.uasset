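; AC_PillarComponent is an actor component that detects when the player enters or leaves a pillar.
; On BeginPlay it binds to the begin and end overlap events of the owner's root primitive component.
; When the overlapping actor is the player character, it calls the OnEnterPillar or OnLeavePillar dispatcher with its PillarID and prints a debug message.
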(event `self.ReceiveBeginPlay`
  (bind _asprimitive_component (cast `PrimitiveComponent` (`Actor.RootComponent` (`self.GetOwner`))))
  (add `PrimitiveComponent.OnComponentBeginOverlap` _asprimitive_component (delegate `OnBeginoverlap`))
  (add `PrimitiveComponent.OnComponentEndOverlap` _asprimitive_component (delegate `OnEndOverlap`)))

(event `OnBeginoverlap`
  (params (OverlappedComponent :type "PrimitiveComponent Object Reference") (OtherActor :type "Actor Object Reference") (OtherComp :type "PrimitiveComponent Object Reference") (OtherBodyIndex :type Integer) (bFromSweep :type Boolean) (SweepResult :type "HitResult Structure (by ref)"))
  (if (== OtherActor (`GameplayStatics.GetPlayerCharacter` 0))
    (`self.OnEnterPillar` (`self.PillarID`))
    (`KismetSystemLibrary.PrintString` "Begin overlap")))

(event `OnEndOverlap`
  (params (OverlappedComponent :type "PrimitiveComponent Object Reference") (OtherActor :type "Actor Object Reference") (OtherComp :type "PrimitiveComponent Object Reference") (OtherBodyIndex :type Integer))
  (if (== OtherActor (`GameplayStatics.GetPlayerCharacter` 0))
    (`self.OnLeavePillar` (`self.PillarID`))
    (`KismetSystemLibrary.PrintString` "End overlap")))
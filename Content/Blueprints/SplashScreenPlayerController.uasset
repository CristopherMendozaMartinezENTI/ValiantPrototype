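; Player controller for the splash screen that prepares player settings before the main menu.
; On begin play it loads or creates the settings save, runs a one-time hardware benchmark to seed quality values, then applies saved audio, graphics and control options through the game instance.
; It pushes the splash widget, then a controller-recommended widget three seconds later.
; Only a gamepad key press triggers a fade-out and opens the main menu level.
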(event `self.ReceiveBeginPlay`
  (bind _settingssavegame (`self.SettingsSaveGame`))
  (bind _asbp_valiant_game_instance (cast `/Game/Blueprints/BP_ValiantGameInstance` (`GameplayStatics.GetGameInstance`)))
  (set `self.ValiantGameInstance` _asbp_valiant_game_instance)
  (`|ExecutionSequence`
    (:`then_0`
      (bind _returnvalue (`GameplayStatics.DoesSaveGameExist` "settings"))
      (if (not _returnvalue)
        (bind _returnvalue_2 (`GameplayStatics.CreateSaveGameObject` "/Game/Blueprints/SaveData/BP_SettingsSave.BP_SettingsSave_C"))
        (bind _output_get (set `self.SettingsSaveGame` _returnvalue_2))
        (`GameplayStatics.SaveGameToSlot` _output_get "settings"))
      (bind _returnvalue_3 (`GameplayStatics.LoadGameFromSlot` "settings"))
      (bind _asbp_settings_save (cast `/Game/Blueprints/SaveData/BP_SettingsSave` _returnvalue_3))
      (set `self.SettingsSaveGame` _asbp_settings_save)
      (if (not (`/Game/Blueprints/SaveData/BP_SettingsSave.BenchmarkDone` (`self.SettingsSaveGame`)))
        (bind _returnvalue_4 (`GameUserSettings.GetGameUserSettings`))
        (`GameUserSettings.RunHardwareBenchmark` _returnvalue_4 10 1.0 1.0)
        (`GameUserSettings.ApplyHardwareBenchmarkResults` _returnvalue_4)
        (set `/Game/Blueprints/SaveData/BP_SettingsSave.BenchmarkDone` true _settingssavegame)
        (set `/Game/Blueprints/SaveData/BP_SettingsSave.ShadowQualityValue` (`GameUserSettings.GetShadowQuality` _returnvalue_4) _settingssavegame)
        (set `/Game/Blueprints/SaveData/BP_SettingsSave.TextureQualityValue` (`GameUserSettings.GetTextureQuality` _returnvalue_4) _settingssavegame)
        (set `/Game/Blueprints/SaveData/BP_SettingsSave.FoliageQualityValue` (`GameUserSettings.GetFoliageQuality` _returnvalue_4) _settingssavegame)
        (`GameplayStatics.SaveGameToSlot` (`self.SettingsSaveGame`) "settings")))
    (:`then_1`
      (`self.ApplyLoadedSettings`)
      (bind _returnvalue_5 (`GameUserSettings.GetGameUserSettings`))
      (`GameUserSettings.LoadSettings` _returnvalue_5 false)
      (`GameUserSettings.ApplySettings` _returnvalue_5 true))
    (:`then_2`
      (`KismetSystemLibrary.DelayUntilNextTick`)
      (bind _asbp_valiant_hud (cast `/Game/UI/BP_ValiantHUD` (`self.GetHUD` (`GameplayStatics.GetPlayerController` 0))))
      (`/PMDialogue/W_OverallUILayout.PushWidgetToLayerStack` (`/Game/UI/BP_ValiantHUD.OverallWidget` _asbp_valiant_hud) (struct :`TagName` "UI.Layer.GameMenu") "/Game/UI/WBP_SplashScreen.WBP_SplashScreen_C")
      (`KismetSystemLibrary.Delay` 3.0)
      (bind _asbp_valiant_hud_2 (cast `/Game/UI/BP_ValiantHUD` (`self.GetHUD` (`GameplayStatics.GetPlayerController` 0))))
      (`/PMDialogue/W_OverallUILayout.PushWidgetToLayerStack` (`/Game/UI/BP_ValiantHUD.OverallWidget` _asbp_valiant_hud_2) (struct :`TagName` "UI.Layer.GameMenu") "/Game/UI/WBP_ControllerRecommended.WBP_ControllerRecommended_C")
      (`WidgetBlueprintLibrary.SetInputMode_GameOnly` self))))

(event `Key|AnyKey`
  (params (Key :type "Key Structure"))
  (:`Pressed`
    (if (`KismetInputLibrary.Key_IsGamepadKey` Key)
      (`PlayerCameraManager.StartCameraFade` :`self` (`GameplayStatics.GetPlayerCameraManager` 0) :`FromAlpha` 0.0 :`ToAlpha` 1.0 :`Duration` 1.0 :`bHoldWhenFinished` true)
      (`GameplayStatics.OpenLevelBySoftObjectPtr` "/Game/Maps/MainMenu.MainMenu"))))

(fn `ApplyLoadedSettings`
  (bind _settingssavegame (`self.SettingsSaveGame`))
  (bind _valiantgameinstance (`self.ValiantGameInstance`))
  (`/Game/Blueprints/BP_ValiantGameInstance.SetMasterVolume` _valiantgameinstance (`/Game/Blueprints/SaveData/BP_SettingsSave.MasterVolumeValue` _settingssavegame))
  (`/Game/Blueprints/BP_ValiantGameInstance.SetMusicVolume` _valiantgameinstance (`/Game/Blueprints/SaveData/BP_SettingsSave.MusicVolumeValue` _settingssavegame))
  (`/Game/Blueprints/BP_ValiantGameInstance.SetSFXVolume` _valiantgameinstance (`/Game/Blueprints/SaveData/BP_SettingsSave.SFXVolumeValue` _settingssavegame))
  (`/Game/Blueprints/BP_ValiantGameInstance.SetShadowQuality` _valiantgameinstance (`/Game/Blueprints/SaveData/BP_SettingsSave.ShadowQualityValue` _settingssavegame))
  (`/Game/Blueprints/BP_ValiantGameInstance.SetTextureQuality` _valiantgameinstance (`/Game/Blueprints/SaveData/BP_SettingsSave.TextureQualityValue` _settingssavegame))
  (`/Game/Blueprints/BP_ValiantGameInstance.SetFoliageQuality` _valiantgameinstance (`/Game/Blueprints/SaveData/BP_SettingsSave.FoliageQualityValue` _settingssavegame))
  (set `/Game/Blueprints/BP_ValiantGameInstance.InvertedControls` (`/Game/Blueprints/SaveData/BP_SettingsSave.InvertedControls` _settingssavegame) _valiantgameinstance)
  (set `/Game/Blueprints/BP_ValiantGameInstance.SensivilityValue` (`/Game/Blueprints/SaveData/BP_SettingsSave.SensitivityValue` _settingssavegame) _valiantgameinstance)
  (`/Game/Blueprints/BP_ValiantGameInstance.SetAntiAliasingMode` _valiantgameinstance (`/Game/Blueprints/SaveData/BP_SettingsSave.AntiAliasingModeValue` _settingssavegame))
  (`/Game/Blueprints/BP_ValiantGameInstance.SetMotionBlur` _valiantgameinstance (`/Game/Blueprints/SaveData/BP_SettingsSave.MotionBlurEnabled` _settingssavegame))
  (set `/Game/Blueprints/BP_ValiantGameInstance.CameraShakeEnabled` (`/Game/Blueprints/SaveData/BP_SettingsSave.CameraShakeEnabled` _settingssavegame) _valiantgameinstance))

(fn `UserConstructionScript`)
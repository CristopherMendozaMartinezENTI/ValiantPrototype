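; Spline-driven tree-house bridge that builds itself from spline mesh segments on BeginPlay, and in the construction script when AutoBuild is set.
; ConstructSplineMeshes divides spline length by Length, placing repeated middle meshes between start and end caps that share one mesh.
; Tangents are clamped to segment length, and the end cap also draws a debug sphere.
; StraightenSpline zeroes all point tangents but is not called here.
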(event `self.ReceiveBeginPlay`
  (`self.ConstructSplineMeshes`))

(fn `ConstructEndingMesh`
  (params (CurrentPoint :type Integer) (MaxPoints :type Integer))
  (bind _spline (`self.Spline`))
  (bind _spline_2 (`self.Spline`))
  (bind _returnvalue (* (+ CurrentPoint 1) (`self.StartingEndingMeshLength`)))
  (bind _returnvalue_2 (* CurrentPoint (`self.Length`)))
  (`|ExecutionSequence`
    (:`then_0`
      (bind _returnvalue_3 (`AddComponent|NODE_AddSplineMeshComponent-2`))
      (`StaticMeshComponent.SetStaticMesh` _returnvalue_3 "/Game/Models/WoodTown/SM_BridgeTreeHouse_SM_PuenteParte1.SM_BridgeTreeHouse_SM_PuenteParte1")
      (`SplineMeshComponent.SetForwardAxis` _returnvalue_3 "X" true)
      (`SplineMeshComponent.SetStartAndEnd` _returnvalue_3 (`SplineComponent.GetLocationAtDistanceAlongSpline` _spline _returnvalue "Local") (`KismetMathLibrary.ClampVectorSize` (`SplineComponent.GetTangentAtDistanceAlongSpline` _spline _returnvalue "Local") 0.0 (`self.StartingEndingMeshLength`)) (`SplineComponent.GetLocationAtDistanceAlongSpline` _spline_2 _returnvalue_2 "Local") (`KismetMathLibrary.ClampVectorSize` (`SplineComponent.GetTangentAtDistanceAlongSpline` _spline_2 _returnvalue_2 "Local") 0.0 (`self.StartingEndingMeshLength`)) true))
    (:`then_1`
      (`KismetSystemLibrary.DrawDebugSphere` (`SplineComponent.GetLocationAtDistanceAlongSpline` _spline_2 _returnvalue_2 "World") 40.0 12 (struct :`R` 1.0 :`G` 1.0 :`B` 1.0 :`A` 1.0) 5.0 2.0))))

(fn `ConstructMiddleMesh`
  (params (CurrentPoint :type Integer) (MaxPoints :type Integer))
  (bind _spline (`self.Spline`))
  (bind _spline_2 (`self.Spline`))
  (bind _returnvalue (* (+ CurrentPoint 1) (`self.Length`)))
  (bind _returnvalue_2 (- (`self.StartingEndingMeshLength`) (`self.Length`)))
  (bind _returnvalue_3 (+ (* CurrentPoint (`self.Length`)) (`KismetMathLibrary.SelectFloat` _returnvalue_2 (`KismetMathLibrary.SelectFloat` _returnvalue_2 0.0 (== CurrentPoint MaxPoints)) (== CurrentPoint 1))))
  (bind _returnvalue_4 (`AddComponent|NODE_AddSplineMeshComponent-0`))
  (`StaticMeshComponent.SetStaticMesh` _returnvalue_4 "/Game/Models/WoodTown/SM_BridgeTreeHouse_SM_PuenteParte2.SM_BridgeTreeHouse_SM_PuenteParte2")
  (`SplineMeshComponent.SetForwardAxis` _returnvalue_4 "X" true)
  (`SplineMeshComponent.SetStartAndEnd` _returnvalue_4 (`SplineComponent.GetLocationAtDistanceAlongSpline` _spline_2 _returnvalue_3 "Local") (`KismetMathLibrary.ClampVectorSize` (`SplineComponent.GetTangentAtDistanceAlongSpline` _spline_2 _returnvalue_3 "Local") 0.0 (`self.Length`)) (`SplineComponent.GetLocationAtDistanceAlongSpline` _spline _returnvalue "Local") (`KismetMathLibrary.ClampVectorSize` (`SplineComponent.GetTangentAtDistanceAlongSpline` _spline _returnvalue "Local") 0.0 (`self.Length`)) true))

(fn `ConstructSplineMeshes`
  (bind _returnvalue (`KismetMathLibrary.FTrunc` (/ (`SplineComponent.GetSplineLength` (`self.Spline`)) (`self.Length`))))
  (bind _returnvalue_2 (- _returnvalue 1))
  (`self.ConstructStartingMesh` 0 1)
  (for _index (range 1 (+ _returnvalue_2 1))
    (`self.ConstructMiddleMesh` _index _returnvalue))
  (`self.ConstructEndingMesh` (+ _returnvalue_2 1)))

(fn `ConstructStartingMesh`
  (params (CurrentPoint :type Integer) (MaxPoints :type Integer))
  (bind _spline (`self.Spline`))
  (bind _spline_2 (`self.Spline`))
  (bind _returnvalue (* (+ CurrentPoint 1) (`self.StartingEndingMeshLength`)))
  (bind _returnvalue_2 (* CurrentPoint (`self.StartingEndingMeshLength`)))
  (bind _returnvalue_3 (`AddComponent|NODE_AddSplineMeshComponent-1`))
  (`StaticMeshComponent.SetStaticMesh` _returnvalue_3 "/Game/Models/WoodTown/SM_BridgeTreeHouse_SM_PuenteParte1.SM_BridgeTreeHouse_SM_PuenteParte1")
  (`SplineMeshComponent.SetForwardAxis` _returnvalue_3 "X" true)
  (`SplineMeshComponent.SetStartAndEnd` _returnvalue_3 (`SplineComponent.GetLocationAtDistanceAlongSpline` _spline_2 _returnvalue_2 "Local") (`KismetMathLibrary.ClampVectorSize` (`SplineComponent.GetTangentAtDistanceAlongSpline` _spline_2 _returnvalue_2 "Local") 0.0 (`self.StartingEndingMeshLength`)) (`SplineComponent.GetLocationAtDistanceAlongSpline` _spline _returnvalue "Local") (`KismetMathLibrary.ClampVectorSize` (`SplineComponent.GetTangentAtDistanceAlongSpline` _spline _returnvalue "Local") 0.0 (`self.StartingEndingMeshLength`)) true))

(fn `StraightenSpline`
  (bind _returnvalue (`KismetMathLibrary.MakeVector` 0.0))
  (for _index (range (`SplineComponent.GetNumberOfSplinePoints` (`self.Spline`)))
    (`SplineComponent.SetTangentsAtSplinePoint` (`self.Spline`) _index _returnvalue _returnvalue "Local" true)))

(fn `UserConstructionScript`
  (if (`self.AutoBuild`)
    (`self.ConstructSplineMeshes`)))
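; Player component that runs the songbird singing mechanic, mapping input keys to learned notes and showing them on a D-pad HUD widget.
; PlayNote pushes the button in the UI, then, behind a short cooldown gate, plays the note's sound, spawns a colored Niagara effect and broadcasts OnSing.
; A sphere overlap passes each sung note to nearby SongbirdListener components.
; AddNote stores a new note and reveals its colored D-pad slot.
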(event `self.ReceiveBeginPlay`
  (set `self.Overall Widget` (`/Game/UI/BP_ValiantHUD.OverallWidget` (cast `/Game/UI/BP_ValiantHUD` (`PlayerController.GetHUD` (`GameplayStatics.GetPlayerController` 0)) :!pure true)))
  (`/Engine/EditorBlueprintResources/StandardMacros.IsValid` (`self.As WBP DPad`)
    (:`Is Valid`
      (if (not (`/PMDialogue/W_OverallUILayout.IsOnStack` (`self.Overall Widget`) (struct :`TagName` "UI.Layer.NotesHUD") (`self.As WBP DPad`)))
        (bind _returnvalue (`/PMDialogue/W_OverallUILayout.PushWidgetToLayerStack` (`self.Overall Widget`) (struct :`TagName` "UI.Layer.NotesHUD") "/Game/UI/WBP_DPad.WBP_DPad_C" :!label _label))
        (bind _aswbp_dpad (cast `/Game/UI/WBP_DPad` _returnvalue))
        (set `self.As WBP DPad` _aswbp_dpad)))
    (:`Is Not Valid`
      (goto _label))))

(event `PlayNote`
  (params (Key :type "/Game/Blueprints/SongbirdSystem/E_Notes Enum" :default "NewEnumerator0"))
  (bind _returnvalue (`self.GetOwner`))
  (bind (_value _returnvalue_2) (`BlueprintMapLibrary.Map_Find` (`self.Notes`) Key))
  (`self.ShowUI` Key)
  (if _returnvalue_2
    (`/Engine/EditorBlueprintResources/StandardMacros.Gate` false :!label _label_2
      (:`Exit`
        (`self.StreamSound` _value)
        (bind _returnvalue_3 (`NiagaraFunctionLibrary.SpawnSystemAtLocation` "/Game/VFX/VFX/SpawnVFX/VFX/MusicNotes/NS_Spawn_MusicNote.NS_Spawn_MusicNote" (+ (`Actor.K2_GetActorLocation` (`self.GetOwner`)) (0.0 0.0 50.0))))
        (`NiagaraComponent.SetVariableLinearColor` _returnvalue_3 "Color" (`KismetMathLibrary.Conv_ColorToLinearColor` (`/Game/Blueprints/SongbirdSystem/BP_SongbirdNote.Color` _value)))
        (`self.OnSing` _value (`Actor.K2_GetActorLocation` _returnvalue) (`Actor.K2_GetActorRotation` _returnvalue) (`.CurrentStateEnum` (`/Game/Blueprints/PlayerCharacter/BP_PlayerFSM.GetCurrentState` (`/Game/Blueprints/PlayerCharacter/BP_PlayerCharacter.Player State Machine` (cast `/Game/Blueprints/PlayerCharacter/BP_PlayerCharacter` _returnvalue :!pure true)))))
        (`|ExecutionSequence`
          (:`then_0`
            (`KismetSystemLibrary.Delay` 0.7)
            (goto _label_2 :!via `Open`))
          (:`then_1`
            (goto _label_2 :!via `Close`)))))))

(event `ShowUI`
  (params (Selection :type "/Game/Blueprints/SongbirdSystem/E_Notes Enum" :default "NewEnumerator0"))
  (`/Engine/EditorBlueprintResources/StandardMacros.IsValid` (`self.As WBP DPad`)
    (:`Is Valid`
      (if (not (`/PMDialogue/W_OverallUILayout.IsOnStack` (`self.Overall Widget`) (struct :`TagName` "UI.Layer.NotesHUD") (`self.As WBP DPad`)))
        (bind _returnvalue (`/PMDialogue/W_OverallUILayout.PushWidgetToLayerStack` (`self.Overall Widget`) (struct :`TagName` "UI.Layer.NotesHUD") "/Game/UI/WBP_DPad.WBP_DPad_C" :!label _label_3))
        (bind _aswbp_dpad (cast `/Game/UI/WBP_DPad` _returnvalue))
        (set `self.As WBP DPad` _aswbp_dpad)))
    (:`Is Not Valid`
      (goto _label_3)))
  (`/Game/UI/WBP_DPad.PushButton` (`self.As WBP DPad`) Selection))

(fn `AddNote`
  (params (Key :type "/Game/Blueprints/SongbirdSystem/E_Notes Enum (by ref)") (Value :type "/Game/Blueprints/SongbirdSystem/BP_SongbirdNote Object Reference (by ref)"))
  (`BlueprintMapLibrary.Map_Add` (`self.Notes`) Key Value)
  (`/Game/UI/WBP_DPad.SetNoteVisibility` (`self.As WBP DPad`) "Visible" Key)
  (`/Game/UI/WBP_DPad.SetNoteColour` (`self.As WBP DPad`) Key (`KismetMathLibrary.Conv_ColorToLinearColor` (`/Game/Blueprints/SongbirdSystem/BP_SongbirdNote.Color` Value))))

(fn `StreamSound`
  (params (Note :type "/Game/Blueprints/SongbirdSystem/BP_SongbirdNote Object Reference (by ref)"))
  (`FMODBlueprintStatics.PlayEventAtLocation` (`/Game/Blueprints/SongbirdSystem/BP_SongbirdNote.Sound` Note) (`Actor.GetTransform` (`self.GetOwner`)))
  (bind (_outcomponents _returnvalue) (`KismetSystemLibrary.SphereOverlapComponents` (`Actor.K2_GetActorLocation` (`self.GetOwner`)) (`self.ListenerRadius`) (`|MakeArray` "ObjectTypeQuery1" "ObjectTypeQuery2" "ObjectTypeQuery3" "ObjectTypeQuery4" :!type "EObjectTypeQuery Enum") "/Game/Blueprints/SongbirdSystem/BP_SongbirdListener.BP_SongbirdListener_C"))
  (if _returnvalue
    (for _array_element _outcomponents
      (bind _asbp_songbird_listener (cast `/Game/Blueprints/SongbirdSystem/BP_SongbirdListener` _array_element :!pure true))
      (`/Game/Blueprints/SongbirdSystem/BP_SongbirdListener.HearSound` _asbp_songbird_listener Note)
      (`KismetSystemLibrary.PrintString` (`KismetSystemLibrary.GetDisplayName` _asbp_songbird_listener)))))
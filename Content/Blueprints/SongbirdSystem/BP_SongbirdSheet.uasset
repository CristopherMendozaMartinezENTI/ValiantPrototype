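; Songbird music sheet that shows a listener's composition as note meshes on a decal and tracks whether it is sung back correctly.
; Construction script and BeginPlay build the notes, placed by staff position and order, each with a dynamic material.
; Heard notes are checked in sequence, coloring matches; a mistake flashes all bad and restarts.
; Completing the sequence recolors every note, then signals success; the decal-tracing helper is unwired.
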(event `ConstructSheet`
  (bind (_offset_x _offset_y) (`KismetMathLibrary.BreakVector2D` (`self.Offset`)))
  (bind (_size_x _size_y) (`KismetMathLibrary.BreakVector2D` (`self.Size`)))
  (bind (_size_x_2 _size_y_2) (`KismetMathLibrary.BreakVector2D` (`self.Size`)))
  (bind (_relativescale3d_x _relativescale3d_y _relativescale3d_z) (`KismetMathLibrary.BreakVector` (`SceneComponent.RelativeScale3D` (`self.Decal`))))
  (bind (_relativescale3d_x_2 _relativescale3d_y_2) (`KismetMathLibrary.BreakVector` (`SceneComponent.RelativeScale3D` (`self.Decal`))))
  (bind _composition (`/Game/Blueprints/SongbirdSystem/BP_SongbirdComposition.Composition` (`/Game/Blueprints/SongbirdSystem/BP_SongbirdListener.Composition` (`self.BP_SongbirdListener`))))
  (bind _returnvalue (* _size_y (/ 1.0 _relativescale3d_z)))
  (bind _returnvalue_2 (* (/ 1.0 (/ _size_x_2 100.0)) 2.0))
  (`/Engine/EditorBlueprintResources/StandardMacros.IsValid` (`/Game/Blueprints/SongbirdSystem/BP_SongbirdListener.Composition` (`self.BP_SongbirdListener`)) :!label _label
    (:`Is Valid`
      (for (_array_element _array_index) _composition
        (`KismetSystemLibrary.PrintString` "Hello")
        (bind _returnvalue_3 (`AddComponent|NODE_AddStaticMeshComponent-1` :`RelativeTransform` (`KismetMathLibrary.MakeTransform` (`KismetMathLibrary.MakeVector` 0.0 (+ (* _size_x (/ 1.0 _relativescale3d_y_2)) (* (`KismetMathLibrary.Conv_IntToDouble` (`/Game/Blueprints/SongbirdSystem/BP_SongbirdNote.StaffPosition` _array_element)) -20.0) _offset_y) (+ _returnvalue (* _array_index (/ _returnvalue (`KismetArrayLibrary.Array_Length` _composition)) -1.0) (* _offset_x -1.0))) (struct) (10.0 10.0 10.0))))
        (`KismetArrayLibrary.Array_Add` (`self.NotesMesh`) _returnvalue_3)
        (bind _returnvalue_4 (`PrimitiveComponent.CreateDynamicMaterialInstance` _returnvalue_3 0 null "None"))
        (`KismetArrayLibrary.Array_Add` (`self.NotesDynMats`) _returnvalue_4)
        (`SceneComponent.K2_AttachToComponent` _returnvalue_3 (`self.Decal`) "None" "KeepRelative" "KeepRelative" "KeepRelative" true)
        (`SceneComponent.SetRelativeScale3D` _returnvalue_3 (`KismetMathLibrary.MakeVector` _returnvalue_2 _returnvalue_2 (* (/ 1.0 (/ _size_y_2 100.0)) 2.0))))
      (`self.SetColors`)
      (set `self.IgnoreNotes` false))))

(event `self.ReceiveBeginPlay`
  (goto _label))

(event `self.ReceiveTick`
  (params (DeltaSeconds :type "Float (single-precision)")))

(event `self.BP_SongbirdListener.OnValidate`
  (params (IsValid :type Boolean)))

(event `self.BP_SongbirdListener.OnHearNote`
  (params (Note :type "/Game/Blueprints/SongbirdSystem/BP_SongbirdNote Object Reference"))
  (bind _returnvalue (`KismetArrayLibrary.Array_Length` (`self.NotesDynMats`)))
  (if (and (== Note (`|GetArrayItem` (`/Game/Blueprints/SongbirdSystem/BP_SongbirdComposition.Composition` (`/Game/Blueprints/SongbirdSystem/BP_SongbirdListener.Composition` (`self.BP_SongbirdListener`))) (`self.latestValidNote`))) (not (`self.IgnoreNotes`)))
    (`MaterialInstanceDynamic.SetVectorParameterValue` (`|GetArrayItem` (`self.NotesDynMats`) (`self.latestValidNote`)) "Color" (`self.CorrectColor`))
    (bind _result (`/Engine/EditorBlueprintResources/StandardMacros.IncrementInt` (`self.latestValidNote`))
      (:`  `
        (bind _output_get (set `self.latestValidNote` (`KismetMathLibrary.Clamp` _result 0 _returnvalue)))
        (if (== _output_get _returnvalue)
          (`KismetSystemLibrary.Delay` 2.0)
          (for _array_element (`self.NotesDynMats`)
            (`MaterialInstanceDynamic.SetVectorParameterValue` _array_element "Color" (`self.AllGoodColor`)))
          (`KismetSystemLibrary.Delay` 1.0)
          (`self.SongbirdSangCorrectly`))))
    (else
      (set `self.IgnoreNotes` true)
      (set `self.latestValidNote` 0)
      (for _array_element_2 (`self.NotesDynMats`)
        (`MaterialInstanceDynamic.SetVectorParameterValue` _array_element_2 "Color" (`self.BadColor`)))
      (`KismetSystemLibrary.Delay` 2.0)
      (for (_array_element_3 _array_index) (`self.NotesDynMats`) :!label _label_2
        (`MaterialInstanceDynamic.SetVectorParameterValue` _array_element_3 "Color" (`KismetMathLibrary.Conv_ColorToLinearColor` (`/Game/Blueprints/SongbirdSystem/BP_SongbirdNote.Color` (`|GetArrayItem` (`/Game/Blueprints/SongbirdSystem/BP_SongbirdComposition.Composition` (`/Game/Blueprints/SongbirdSystem/BP_SongbirdListener.Composition` (`self.BP_SongbirdListener`))) _array_index)))))
      (set `self.IgnoreNotes` false))))

(event `SetColors`
  (goto _label_2))

(fn `AttachNoteToDecalPlane`
  (params (StaticMeshComp :type "StaticMeshComponent Object Reference"))
  (returns (Distance :type "Float (single-precision)") (Location :type "Vector Structure"))
  (bind _returnvalue (`SceneComponent.K2_GetComponentLocation` StaticMeshComp))
  (bind _outhit (`KismetSystemLibrary.LineTraceSingle` :`Start` _returnvalue :`End` (+ _returnvalue (* (`SceneComponent.GetRightVector` StaticMeshComp) -100.0)) :`TraceChannel` "TraceTypeQuery1" :`DrawDebugType` "Persistent"))
  (bind (_bblockinghit _binitialoverlap _time _distance _location) (`GameplayStatics.BreakHitResult` _outhit))
  (return _distance _location))

(fn `UserConstructionScript`
  (bind (_size_x _size_y) (`KismetMathLibrary.BreakVector2D` (`self.Size`)))
  (bind _returnvalue (/ _size_x 100.0))
  (bind _returnvalue_2 (/ _size_y 100.0))
  (`SceneComponent.SetRelativeScale3D` (`self.Decal`) (`KismetMathLibrary.MakeVector` 1.0 _returnvalue _returnvalue_2))
  (`SceneComponent.SetRelativeScale3D` (`self.BP_SongbirdListener`) (`KismetMathLibrary.MakeVector` (* _returnvalue_2 2.0) 1.0 (* _returnvalue 2.0)))
  (`self.ConstructSheet`))
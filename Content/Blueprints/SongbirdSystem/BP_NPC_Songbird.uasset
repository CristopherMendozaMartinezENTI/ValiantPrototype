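; BP_NPC_Songbird is a songbird NPC in the songbird system that signals when it has been collected.
; On receiving a Flow notify, it prints a debug message and calls the OnCollectSongbird event dispatcher.
; It has no other active logic, as BeginPlay, overlap and Tick are disabled stubs and the construction script only calls its parent.
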(event `self.Flow.ReceiveNotify`
  (params (FlowComponent :type "FlowComponent Object Reference") (NotifyTag :type "GameplayTag Structure (by ref)"))
  (`KismetSystemLibrary.PrintString` "COLLECTED SONGBIRD" true true (struct :`G` 1.0 :`B` 0.230062 :`A` 1.0) 5.0)
  (`self.OnCollectSongbird` self))

(fn `UserConstructionScript`
  (`parent.UserConstructionScript`))
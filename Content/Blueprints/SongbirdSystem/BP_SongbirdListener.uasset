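; BP_SongbirdListener reacts to notes it hears in the songbird system and broadcasts OnValidate with whether they pass.
; In composition mode it collects notes and, after a retriggerable one-second pause, sends them to Composition for validation.
; The Composition's validation result, bound at BeginPlay, is relayed through the same dispatcher.
; Otherwise it validates each note immediately, either against NoteToHear when ExactNote is set or accepting any note.
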(event `self.ReceiveBeginPlay`
  (`/Engine/EditorBlueprintResources/StandardMacros.IsValid` (`self.Composition`)
    (:`Is Valid`
      (add `/Game/Blueprints/SongbirdSystem/BP_SongbirdComposition.OnValidateComposition` (`self.Composition`) (delegate `CustomEvent`)))))

(event `CustomEvent`
  (params (IsValid :type Boolean))
  (`self.OnValidate` IsValid))

(event `HearSound`
  (params (Note :type "/Game/Blueprints/SongbirdSystem/BP_SongbirdNote Object Reference (by ref)"))
  (bind _heardnotes (`self.HeardNotes`))
  (bind _heardnotes_2 (`self.HeardNotes`))
  (if (`self.ListenToComposition`)
    (`KismetArrayLibrary.Array_Add` _heardnotes_2 Note)
    (`KismetSystemLibrary.RetriggerableDelay` 1.0)
    (`/Game/Blueprints/SongbirdSystem/BP_SongbirdComposition.ValidateComposition` (`self.Composition`) _heardnotes_2)
    (`KismetArrayLibrary.Array_Remove` _heardnotes (`KismetArrayLibrary.Array_Length` _heardnotes))
    (elif (`self.ExactNote`)
      (`self.OnValidate` (== Note (`self.NoteToHear`)))
      (else
        (`self.OnValidate` true)))))
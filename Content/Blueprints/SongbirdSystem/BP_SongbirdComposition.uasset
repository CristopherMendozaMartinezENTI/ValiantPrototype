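; BP_SongbirdComposition holds a Composition sequence for the songbird system and checks submitted sequences against it.
; ValidateComposition compares the last four entries of the incoming array with the last four of Composition, position by position.
; It broadcasts the boolean result through the OnValidateComposition dispatcher, reporting false when the input has fewer than four entries.
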(event `ValidateComposition`
  (params (NewParam :type "Array of /Game/Blueprints/SongbirdSystem/BP_SongbirdNote Object Reference"))
  (bind _returnvalue (`KismetArrayLibrary.Array_LastIndex` NewParam))
  (bind _composition (`self.Composition`))
  (bind _returnvalue_2 (`KismetArrayLibrary.Array_LastIndex` _composition))
  (if (>= (`KismetArrayLibrary.Array_Length` NewParam) 4)
    (`self.OnValidateComposition` (and (== (`|GetArrayItem` NewParam _returnvalue) (`|GetArrayItem` _composition _returnvalue_2)) (== (`|GetArrayItem` NewParam (- _returnvalue 1)) (`|GetArrayItem` _composition (- _returnvalue_2 1))) (== (`|GetArrayItem` NewParam (- _returnvalue 2)) (`|GetArrayItem` _composition (- _returnvalue_2 2))) (== (`|GetArrayItem` NewParam (- _returnvalue 3)) (`|GetArrayItem` _composition (- _returnvalue_2 3)))))
    (else
      (`self.OnValidateComposition` false))))
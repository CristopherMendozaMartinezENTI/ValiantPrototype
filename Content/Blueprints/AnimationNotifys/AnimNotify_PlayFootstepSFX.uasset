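; Animation notify that plays footstep audio matched to the ground surface under the animated character.
; It line traces vertically through the owner's location on the Visibility channel, with debug drawing left on, and reads the hit's physical surface.
; The surface sets a global GroundType audio parameter, defaulting to the Stone value, then the Footsteps event plays attached to the mesh.
; Without a hit, no sound plays.
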(fn `Received_Notify`
  (params (MeshComp :type "SkeletalMeshComponent Object Reference") (Animation :type "AnimSequenceBase Object Reference") (EventReference :type "AnimNotifyEventReference Structure (by ref)"))
  (returns (ReturnValue :type Boolean))
  (bind _returnvalue (`ActorComponent.GetOwner` MeshComp))
  (bind _returnvalue_2 (`Actor.K2_GetActorLocation` _returnvalue))
  (bind (_outhit _returnvalue_3) (`KismetSystemLibrary.LineTraceSingle` (`KismetMathLibrary.MakeVector` (.x _returnvalue_2) (.y _returnvalue_2) (+ (.z _returnvalue_2) 100.0)) (`KismetMathLibrary.MakeVector` (.x _returnvalue_2) (.y _returnvalue_2) (- (.z _returnvalue_2) 200.0)) "TraceTypeQuery1" false (`|MakeArray` _returnvalue) "ForDuration" true (struct :`R` 1.0 :`A` 1.0) (struct :`G` 1.0 :`A` 1.0) 3.0))
  (if _returnvalue_3
    (switch `EPhysicalSurface` (`GameplayStatics.GetSurfaceType` _outhit)
      (:`SurfaceType_Default`
        (`FMODBlueprintStatics.SetGlobalParameterByName` "GroundType" :!label _label))
      (:`SurfaceType1`
        (goto _label))
      (:`SurfaceType2`
        (`FMODBlueprintStatics.SetGlobalParameterByName` "GroundType" 1.0))
      (:`SurfaceType3`
        (`FMODBlueprintStatics.SetGlobalParameterByName` "GroundType" 2.0))
      (:`SurfaceType4`
        (`FMODBlueprintStatics.SetGlobalParameterByName` "GroundType" 3.0)))
    (`FMODBlueprintStatics.PlayEventAttached` "/Game/FMOD/Events/SFX/Player/Footsteps.Footsteps" (`local.MeshComp`) "None" (0.0 0.0 0.0) "KeepRelativeOffset")
    (return true)
    (else
      (return false))))
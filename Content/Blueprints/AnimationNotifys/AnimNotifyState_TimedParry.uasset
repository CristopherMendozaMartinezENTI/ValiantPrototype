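; Anim notify state that marks the timed parry window within an animation.
; On begin and end it sends start and stop parry window messages to the mesh's anim instance.
; An optional debug flag tints material slot 2 red during the window and white afterward through dynamic material instances.
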(fn `Received_NotifyBegin`
  (params (MeshComp :type "SkeletalMeshComponent Object Reference") (Animation :type "AnimSequenceBase Object Reference") (TotalDuration :type "Float (single-precision)") (EventReference :type "AnimNotifyEventReference Structure (by ref)"))
  (returns (ReturnValue :type Boolean))
  (message `/Game/Blueprints/AnimationNotifys/BPI_Notifies.OnStartParryWindow` (`SkeletalMeshComponent.GetAnimInstance` MeshComp))
  (if (`self.Debug Show Marker`)
    (bind _returnvalue (`PrimitiveComponent.CreateDynamicMaterialInstance` MeshComp 2 null "None"))
    (`MaterialInstanceDynamic.SetVectorParameterValue` _returnvalue "Color" (struct :`R` 1.0 :`A` 1.0)))
  (return false))

(fn `Received_NotifyEnd`
  (params (MeshComp :type "SkeletalMeshComponent Object Reference") (Animation :type "AnimSequenceBase Object Reference") (EventReference :type "AnimNotifyEventReference Structure (by ref)"))
  (returns (ReturnValue :type Boolean))
  (message `/Game/Blueprints/AnimationNotifys/BPI_Notifies.OnStopParryWindow` (`SkeletalMeshComponent.GetAnimInstance` MeshComp))
  (if (`self.Debug Show Marker`)
    (bind _returnvalue (`PrimitiveComponent.CreateDynamicMaterialInstance` MeshComp 2 null "None"))
    (`MaterialInstanceDynamic.SetVectorParameterValue` _returnvalue "Color" (struct :`R` 1.0 :`G` 1.0 :`B` 1.0 :`A` 1.0)))
  (return false))
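; Player pawn for winged flight: it starts in Flying mode and constantly moves along the camera's forward vector, steered by mouse look.
; UpdateMomentum, not called within this file, builds momentum when diving and bleeds it otherwise, driving fly speed with a pitch curve.
; It also triggers speed-based FOV and dive camera shake; dash input adds timeline-driven momentum.
; Procedural wing animation is disconnected, and sphere-trace surface assist is never called here.
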(event `self.ReceiveBeginPlay`
  (`self.InitInputActions`)
  (`self.SetupProceduralAnimation`)
  (`CharacterMovementComponent.SetMovementMode` (`self.CharacterMovement`) "MOVE_Flying" 0))

(event `Mouse Tick`
  (bind (_returnvalue_x _returnvalue_y) (`KismetMathLibrary.BreakVector2D` (`|GetInputActionValue`)))
  (bind _baselookuprate (`self.BaseLookUpRate`))
  (bind _returnvalue (+ _returnvalue_y 0.0))
  (`self.AddControllerYawInput` (* _returnvalue_x (`self.BaseTurnRate`)))
  (if (`self.InvertMouse`)
    (`self.AddControllerPitchInput` (* _returnvalue _baselookuprate))
    (else
      (`self.AddControllerPitchInput` (* (* _returnvalue -1.0) _baselookuprate)))))

(event `self.ReceiveTick`
  (params (DeltaSeconds :type "Float (single-precision)"))
  (`self.Mouse Tick`)
  (`self.OrientationTick`)
  (`self.Movement Tick`))

(event `OrientationTick`)

(event `Movement Tick`
  (`self.AddMovementInput` (`SceneComponent.GetForwardVector` (`self.PlayerCamera`))))

(event `UpdateMomentum`
  (params (DeltaTime :type "Float (double-precision)"))
  (set `CharacterMovementComponent.MaxFlySpeed` (`KismetMathLibrary.FClamp` (+ (`CurveFloat.GetFloatValue` (`self.DiveFloatCurve`) (`self.Pitch`)) (* (+ (`self.AccumulatedMomentum`) (`self.MomentumExtraSpeed`)) 10.0) (`self.ExtraSpeed`)) 0.0 3000.0) (`self.CharacterMovement`))
  (`|ExecutionSequence`
    (:`then_0`
      (`self.AdjustFOVBasedOnSpeed` DeltaTime))
    (:`then_1`
      (if (> (`self.Pitch`) 10.0)
        ;[1 1 1] Diving
        (`self.AddMomentum` DeltaTime 10.0)
        (`/Game/MarketplaceAssets/Low_Poly_Legend_Thunderbird/Character/UI/UI_Thunderbird.SetPitch` (`self.Damage Indicator Reference`) "Diving")
        (`CameraShakeSourceComponent.Start` (`self.Diving Camera Shake`))
        (else
          (if (< (`self.Pitch`) -10.0)
            ;[1 1 1] Ascending
            (`self.RemoveMomentum` DeltaTime 5.0)
            (`/Game/MarketplaceAssets/Low_Poly_Legend_Thunderbird/Character/UI/UI_Thunderbird.SetPitch` (`self.Damage Indicator Reference`) "Ascending")
            (else
              ;[1 1 1] Gliding
              (`self.RemoveMomentum` DeltaTime 2.0)
              (`/Game/MarketplaceAssets/Low_Poly_Legend_Thunderbird/Character/UI/UI_Thunderbird.SetPitch` (`self.Damage Indicator Reference`) "Gliding")))
          (`CameraShakeSourceComponent.StopAllCameraShakes` (`self.Diving Camera Shake`) true))))
    (:`then_2`
      (`KismetSystemLibrary.PrintString` (`KismetStringLibrary.Conv_DoubleToString` (+ (`self.AccumulatedMomentum`) (`self.MomentumExtraSpeed`))) true true (struct :`G` 0.66 :`B` 1.0 :`A` 1.0) DeltaTime "Momentum"))))

(event `EnhancedInput|/Game/ThirdPerson/Input/Actions/IA_Dash`
  (params (ActionValue :type Boolean) (ElapsedSeconds :type "Float (double-precision)") (TriggeredSeconds :type "Float (double-precision)") (InputAction :type "InputAction Object Reference" :default "/Game/ThirdPerson/Input/Actions/IA_Dash.IA_Dash"))
  (:`Triggered`
    (bind (_direction _newtrack_0) (`Timeline|Timeline` :!via `PlayFromStart`)
      (:`Update`
        (set `self.MomentumExtraSpeed` _newtrack_0)))))

(event `RemoveMomentum`
  (params (DT :type "Float (double-precision)") (DeaccelerationRate :type "Float (double-precision)"))
  (set `self.AccumulatedMomentum` (`KismetMathLibrary.FClamp` (- (`self.AccumulatedMomentum`) (* DT DeaccelerationRate)) 0.0 (`self.MaxAccomulatedMomentum`)))
  (set `self.MomentumExtraSpeed` (`KismetMathLibrary.FClamp` (- (`self.MomentumExtraSpeed`) (* DT DeaccelerationRate)) 0.0 30.0)))

(event `AddMomentum`
  (params (DT :type "Float (double-precision)") (`Acceleration Rate` :type "Float (double-precision)"))
  (set `self.AccumulatedMomentum` (`KismetMathLibrary.FClamp` (+ (`self.AccumulatedMomentum`) (* DT `Acceleration Rate`) 0.0) 0.0 (`self.MaxAccomulatedMomentum`))))

(fn `AdjustFOVBasedOnSpeed`
  (params (DeltaTime :type "Float (double-precision)"))
  (`CameraComponent.SetFieldOfView` (`self.PlayerCamera`) (`KismetMathLibrary.FInterpTo` (`CameraComponent.FieldOfView` (`self.PlayerCamera`)) (`KismetMathLibrary.MapRangeClamped` (`KismetMathLibrary.VSize` (`self.GetVelocity`)) 600.0 1000.0 90.0 120.0) DeltaTime)))

(fn `BellowHelperLinetraces`
  (bind (_returnvalue_roll _returnvalue_pitch _returnvalue_yaw) (`KismetMathLibrary.BreakRotator` (`KismetMathLibrary.Conv_VectorToRotator` (`SceneComponent.GetForwardVector` (`self.PlayerCamera`)))))
  (bind (_returnvalue_roll_2 _returnvalue_pitch_2 _returnvalue_yaw_2) (`KismetMathLibrary.BreakRotator` (`KismetMathLibrary.Conv_VectorToRotator` (`SceneComponent.GetForwardVector` (`self.PlayerCamera`)))))
  (bind _returnvalue (+ (`SceneComponent.K2_GetComponentLocation` (`self.Mesh`)) (0.0 0.0 0.0)))
  (bind (_outhit _returnvalue_2) (`KismetSystemLibrary.SphereTraceSingle` :`Start` _returnvalue :`End` _returnvalue :`Radius` 70.0 :`TraceChannel` "TraceTypeQuery1" :`DrawDebugType` "ForOneFrame"))
  (if _returnvalue_2
    (bind _returnvalue_3 (`KismetMathLibrary.Cross_VectorVector` (`SceneComponent.GetRightVector` (`self.CapsuleComponent`)) (`.Normal` (`GameplayStatics.BreakHitResult` _outhit))))
    (`CharacterMovementComponent.AddForce` (`self.CharacterMovement`) (* _returnvalue_3 1000.0))
    (bind (_returnvalue_roll_3 _returnvalue_pitch_3) (`KismetMathLibrary.BreakRotator` (`KismetMathLibrary.Conv_VectorToRotator` _returnvalue_3)))
    (`SceneComponent.K2_SetWorldRotation` (`self.AutoAimDirection`) (`KismetMathLibrary.MakeRotator` _returnvalue_roll (`KismetMathLibrary.SelectFloat` _returnvalue_pitch _returnvalue_pitch_3 (> _returnvalue_pitch 10.0)) _returnvalue_yaw) false false)
    (else
      (`SceneComponent.K2_SetWorldRotation` (`self.AutoAimDirection`) (`KismetMathLibrary.MakeRotator` _returnvalue_roll_2 _returnvalue_pitch_2 _returnvalue_yaw_2) false false))))

(fn `Dash`
  (if (`self.IsDashing`)
    (`CharacterMovementComponent.AddForce` (`self.CharacterMovement`) (* (`SceneComponent.GetForwardVector` (`self.PlayerCamera`)) (`self.ForwardDashForce`)))
    (set `CharacterMovementComponent.MaxFlySpeed` 2500.0 (`self.CharacterMovement`))))

(fn `HelperLinetraces`
  (`self.BellowHelperLinetraces`))

(fn `InitInputActions`
  (bind _asplayer_controller (cast `PlayerController` (`self.GetController`)))
  (bind _returnvalue (pcsubsystem `EnhancedInputLocalPlayerSubsystem` _asplayer_controller))
  (`/Engine/EditorBlueprintResources/StandardMacros.IsValid` _returnvalue
    (:`Is Valid`
      (`EnhancedInputSubsystemInterface.AddMappingContext` _returnvalue "/Game/ThirdPerson/Input/IMC_Default.IMC_Default" 0 (struct)))))

(fn `SetupProceduralAnimation`)

(fn `UserConstructionScript`)
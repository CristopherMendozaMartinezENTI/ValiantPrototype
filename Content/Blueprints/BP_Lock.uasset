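; BP_Lock is a lock actor that visually dissolves when opened and reverses the effect when closed.
; BeginPlay creates a dynamic material instance on the static mesh.
; OpenLock and CloseLock drive a scalar parameter through separate Dissolve timelines, forward and reversed, though the parameter name is set to None.
; Opening also spawns an attached NS_LockDissolve Niagara system on every timeline update, rather than once.
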(event `self.ReceiveBeginPlay`
  (bind _returnvalue (`KismetMaterialLibrary.CreateDynamicMaterialInstance` (`PrimitiveComponent.GetMaterial` (`self.StaticMesh`) 0)))
  (bind _output_get (set `self.mat` _returnvalue))
  (`PrimitiveComponent.SetMaterial` (`self.StaticMesh`) 0 _output_get))

(event `OpenLock`
  (bind (_direction _dissolve) (`Timeline|Timeline` :!via `PlayFromStart`)
    (:`Update`
      (`MaterialInstanceDynamic.SetScalarParameterValue` (`self.mat`) "None" _dissolve)
      (`NiagaraFunctionLibrary.SpawnSystemAttached` "/Game/VFX/VFX/NS_LockDissolve.NS_LockDissolve" (`self.StaticMesh`) "None" (0.0 0.0 0.0) (struct) "KeepRelativeOffset"))))

(event `CloseLock`
  (bind (_direction _dissolve) (`Timeline|Timeline_0` :!via `ReverseFromEnd`)
    (:`Update`
      (`MaterialInstanceDynamic.SetScalarParameterValue` (`self.mat`) "None" _dissolve))))

(fn `UserConstructionScript`)
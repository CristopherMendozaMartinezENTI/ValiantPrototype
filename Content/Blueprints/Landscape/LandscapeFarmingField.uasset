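; Landscape farm field actor that builds a flat Geometry Script mesh from a spline outline.
; Rebuild samples around spline points using a Smooth offset, extrudes a zero-height polygon, then applies an editor visualization material and UV scale.
; Helpers zero spline tangents and create or update a baked static mesh asset with an RVT farmfield material.
; The construction script tints the baked mesh through a dynamic material's Color parameter.
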(event `self.OnRebuildGeneratedMesh`
  (params (TargetMesh :type "DynamicMesh Object Reference"))
  (bind _spline (`self.Spline`))
  (bind _spline_2 (`self.Spline`))
  (bind _spline_3 (`self.Spline`))
  (bind _polygon_vertices (`self.Polygon Vertices`))
  (bind _innersplinepos (`self.InnerSplinePos`))
  (bind _returnvalue (`SplineComponent.GetLocationAtSplineInputKey` _spline_2 0.0 "Local"))
  (set `self.OutputMesh` TargetMesh)
  (`|ExecutionSequence`
    (:`then_0`
      ;[1 1 1 1 70] Base Mesh
      (for _index (range (`SplineComponent.GetNumberOfSplinePoints` (`self.Spline`)))
        (bind _returnvalue_2 (- _index (`self.Smooth`)))
        (bind _returnvalue_3 (`SplineComponent.GetLocationAtSplineInputKey` _spline_3 _returnvalue_2 "Local"))
        ;;[1 0 0 0.2 60] InputKey前
        (`KismetArrayLibrary.Array_Add` (`self.InnerSplinePos`) (+ _returnvalue_3 (* (`self.Offset`) (`SplineComponent.GetRightVectorAtSplineInputKey` _spline_3 _returnvalue_2 "Local"))))
        (`KismetArrayLibrary.Array_Add` (`self.Polygon Vertices`) (`KismetMathLibrary.MakeVector2D` (.x _returnvalue_3) (.y _returnvalue_3)))
        ;;[1 0 0 0.2 60] InputKey
        (`KismetArrayLibrary.Array_Add` (`self.InnerSplinePos`) (+ _returnvalue (* (`self.Offset`) (`SplineComponent.GetRightVectorAtSplineInputKey` _spline_2 0.0 "Local"))))
        (`KismetArrayLibrary.Array_Add` (`self.Polygon Vertices`) (`KismetMathLibrary.MakeVector2D` (.x _returnvalue) (.y _returnvalue)))
        (bind _returnvalue_4 (+ _index (`self.Smooth`)))
        (bind _returnvalue_5 (`SplineComponent.GetLocationAtSplineInputKey` _spline _returnvalue_4 "Local"))
        ;;[1 0 0 0.2 60] InputKey後
        (`KismetArrayLibrary.Array_Add` (`self.InnerSplinePos`) (+ _returnvalue_5 (* (`self.Offset`) (`SplineComponent.GetRightVectorAtSplineInputKey` _spline _returnvalue_4 "Local"))))
        (`KismetArrayLibrary.Array_Add` (`self.Polygon Vertices`) (`KismetMathLibrary.MakeVector2D` (.x _returnvalue_5) (.y _returnvalue_5))))
      ;;[1 1 1] Comment
      (`KismetArrayLibrary.Array_Remove` _innersplinepos (`KismetArrayLibrary.Array_LastIndex` _innersplinepos))
      (`KismetArrayLibrary.Array_Remove` _polygon_vertices (`KismetArrayLibrary.Array_LastIndex` _polygon_vertices))
      (bind _returnvalue_6 (`GeometryScriptLibrary_MeshPrimitiveFunctions.AppendSimpleExtrudePolygon` (`self.OutputMesh`) (struct) (`KismetMathLibrary.MakeTransform` (0.0 0.0 0.0)) (`self.Polygon Vertices`) 0.0 1 true "Base" null))
      (bind _returnvalue_7 (`GeometryScriptLibrary_MeshNormalsFunctions.RecomputeNormals` _returnvalue_6 (struct) false null))
      (bind _returnvalue_8 (`GeometryScriptLibrary_MeshMaterialFunctions.RemapMaterialIDs` _returnvalue_7 0 0 null))
      (set `self.OutputMesh` _returnvalue_8))
    (:`then_1`)
    (:`then_3`
      ;[1 1 1] マテリアル
      (`GeometryScriptLibrary_SceneUtilityFunctions.SetComponentMaterialList` (`self.DynamicMeshComponent`) (`|MakeArray` "/Game/Blueprints/Landscape/M_FarmfieldEditorVisualization.M_FarmfieldEditorVisualization" :!type "MaterialInterface Object Reference") null)
      (`GeometryScriptLibrary_MeshUVFunctions.ScaleMeshUVs` (`self.OutputMesh`) 0 (`self.UVScale`) (0.0 0.0) (struct) null))))

(fn `Bake To Landscape`
  (bind _returnvalue (`BaseDynamicMeshComponent.GetDynamicMesh` (`self.DynamicMeshComponent`)))
  (bind _bakedmesh (`self.BakedMesh`)
    (:`then`
      (`GeometryScriptLibrary_StaticMeshFunctions.CopyMeshToStaticMesh` _returnvalue _bakedmesh (make `GeometryScriptCopyMeshToAssetOptions` false false false true (`|MakeArray` "/Game/Blueprints/Landscape/M_RVTFarmfield.M_RVTFarmfield" :!type "MaterialInterface Object Reference")) (struct) null
        (:`Success`
          (`StaticMeshComponent.SetStaticMesh` (`self.StaticMesh`) (`self.BakedMesh`)))))
    (:`else`)))

(fn `Create Static Mesh `
  (bind _returnvalue (`BaseDynamicMeshComponent.GetDynamicMesh` (`self.DynamicMeshComponent`)))
  (bind _returnvalue_2 (`GeometryScriptLibrary_CreateNewAssetFunctions.CreateNewStaticMeshAssetFromMesh` _returnvalue (`KismetStringLibrary.Concat_StrStr` "/Game/Fields/" "SM" ".Field." (`self.GetActorLabel` true) "." (`KismetStringLibrary.Conv_IntToString` (`KismetMathLibrary.RandomIntegerInRange` 0 10000))) (struct) null)
    (:`Success`
      (set `self.BakedMesh` _returnvalue_2)
      (`self.Bake To Landscape`))))

(fn `Remove Smooth Tangents`
  (bind _returnvalue (`KismetMathLibrary.MakeVector` 0.0))
  (for _index (range (`SplineComponent.GetNumberOfSplinePoints` (`self.Spline`)))
    (`SplineComponent.SetTangentsAtSplinePoint` (`self.Spline`) _index _returnvalue _returnvalue "Local" true)))

(fn `UserConstructionScript`
  (`self.BakedMesh`
    (:`then`
      (bind _returnvalue (`PrimitiveComponent.CreateDynamicMaterialInstance` (`self.StaticMesh`) 0 "/Game/Blueprints/Landscape/M_RVTFarmfield.M_RVTFarmfield" "None"))
      (`MaterialInstanceDynamic.SetVectorParameterValue` _returnvalue "Color" (`self.Color`)))
    (:`else`)))
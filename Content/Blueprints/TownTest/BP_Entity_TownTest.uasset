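; Town test entity whose window glow follows the hour of the day.
; The construction script creates a dynamic material instance from the static mesh's first material slot and stores it.
; Each tick, after calling the parent, it samples a lights curve at the current hour and writes the result to the material's WindowEmissive parameter.
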(event `self.ReceiveTick`
  (params (DeltaSeconds :type "Float (single-precision)"))
  (`parent.ReceiveTick` DeltaSeconds)
  (bind _hour (`self.GetHour`))
  (`MaterialInstanceDynamic.SetScalarParameterValue` (`self.Mat`) "WindowEmissive" (`CurveFloat.GetFloatValue` (`self.LightsCurve`) _hour)))

(fn `UserConstructionScript`
  (bind _staticmesh (`self.StaticMesh`))
  (`parent.UserConstructionScript`)
  (bind _returnvalue (`PrimitiveComponent.CreateDynamicMaterialInstance` _staticmesh 0 (`PrimitiveComponent.GetMaterial` _staticmesh 0) "None"))
  (bind _output_get (set `self.Mat` _returnvalue))
  (`PrimitiveComponent.SetMaterial` (`self.StaticMesh`) 0 _output_get))
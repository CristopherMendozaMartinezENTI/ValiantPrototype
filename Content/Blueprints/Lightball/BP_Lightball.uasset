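; BP_Lightball is a light ball actor that loops along a spline, moving its Scene component each Tick by constant-velocity time sampling.
; TransitionToOtherSpline pauses this motion, tweens the actor to another spline actor's location with its forward axis pointing away from it, then restarts on that spline.
; An older player-fleeing, trace-based steering graph is disconnected, and AvoidObstacles is a stub that traces without acting.
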(event `self.ReceiveBeginPlay`)

(event `self.ReceiveTick`
  (params (DeltaSeconds :type "Float (single-precision)"))
  (bind _spline (`/Game/Blueprints/BP_SimpleSpline.Spline` (`self.CurrentSpline`)))
  (if (`self.CanMove`)
    (bind _output_get (set `self.CurrDIstance` (mod (+ (* DeltaSeconds (`self.Speed`)) (`self.CurrDIstance`)) (`SplineComponent.Duration` _spline))))
    (`SceneComponent.K2_SetWorldTransform` (`self.Scene`) (`SplineComponent.GetTransformAtTime` _spline _output_get "World" true false) false false)))

(event `TransitionToOtherSpline`
  (params (NextSpline :type "/Game/Blueprints/BP_SimpleSpline Object Reference"))
  (bind _returnvalue (`self.K2_GetActorLocation` NextSpline))
  (set `self.CanMove` false)
  (bind _output_get (set `self.NewVar` (`self.K2_GetActorLocation`)))
  (bind (_asynctaskproxy _value) (`FCTweenBPActionVector.TweenVector` _output_get _returnvalue 5.0)
    (:`ApplyEasing`
      (`self.K2_SetActorLocation` _value)
      (`self.K2_SetActorRotation` (`KismetMathLibrary.Conv_VectorToRotator` (`KismetMathLibrary.Normal` (- _output_get _returnvalue)))))
    (:`OnComplete`
      (set `self.CurrentSpline` NextSpline)
      (set `self.CurrDIstance` 0.0)
      (set `self.CanMove` true))))

(fn `AvoidObstacles`
  (bind _returnvalue (`self.K2_GetActorLocation`))
  (bind (_outhit _returnvalue_2) (`KismetSystemLibrary.LineTraceSingle` _returnvalue (+ _returnvalue (* (`self.GetActorForwardVector`) 250.0)) "TraceTypeQuery1"))
  (if _returnvalue_2
    _))

(fn `UserConstructionScript`)
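; Actor component that projects a decal drop shadow beneath its owner, either a blob or a render-target shadow.
; On BeginPlay it disables decals on owner meshes, creates the decal and, optionally, an orthographic depth capture showing only the owner.
; Each tick, a ring of downward traces finds nearest and furthest ground to fit the decal.
; Smoothed distance drives opacity and blur or density, recapturing manually only on change or AlwaysUpdate.
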(event `self.ReceiveBeginPlay`
  (`self.Set`))

(event `self.ReceiveTick`
  (params (DeltaSeconds :type "Float (single-precision)"))
  (`self.Update`))

(fn `DrawTraces`
  (returns (Return :type Boolean))
  (locals (bReturn_Local :type Boolean) (ImpactPoint_Local :type "Array of Float (double-precision)"))
  (bind _tracecount (`self.TraceCount`))
  (bind _impactpoint_local (`local.ImpactPoint_Local`))
  (bind (_returnvalue_x _returnvalue_y) (`KismetMathLibrary.BreakVector` (`Actor.K2_GetActorLocation` (`self.GetOwner`))))
  (bind (_returnvalue_x_2 _returnvalue_y_2 _returnvalue_z) (`KismetMathLibrary.BreakVector` (`Actor.K2_GetActorLocation` (`self.GetOwner`))))
  (bind (_returnvalue_x_3 _returnvalue_y_3) (`KismetMathLibrary.BreakVector` (`Actor.K2_GetActorLocation` (`self.GetOwner`))))
  ;[1 1 1] Loop through vector rotations to draw a circle of line traces around the character
  (for _index (range 1 (+ _tracecount 1))
    (bind _returnvalue (+ (`Actor.K2_GetActorLocation` (`self.GetOwner`)) (* (`KismetMathLibrary.RotateAngleAxis` (1.0 0.0 0.0) (* (/ (`KismetMathLibrary.Conv_IntToDouble` _index) (`KismetMathLibrary.Conv_IntToDouble` _tracecount)) 360.0) (0.0 0.0 1.0)) (`self.DecalSize`))))
    (bind (_outhit _returnvalue_2) (`KismetSystemLibrary.LineTraceSingle` :`Start` _returnvalue :`End` (- _returnvalue (`KismetMathLibrary.MakeVector` 0.0 0.0 (`self.TraceLength`))) :`TraceChannel` "TraceTypeQuery1" :`DrawDebugType` (select `bool` (`self.bDebugMode`) :`true` "ForOneFrame" :!type "EDrawDebugTrace Enum") :`DrawTime` 0.01))
    ;[1 1 1] Update Closest/Furthest Point if applicable
    (if (`.bInitialOverlap` (`GameplayStatics.BreakHitResult` _outhit))
      _
      (elif _returnvalue_2
        (set `local.bReturn_Local` true)
        (`KismetArrayLibrary.Array_Add` (`local.ImpactPoint_Local`) (.z (`.Location` (`GameplayStatics.BreakHitResult` _outhit)))))))
  (`|ExecutionSequence`
    (:`then_0`
      ;[1 1 1] Draw shortest and longest point (Debug only)
      (if (`self.bDebugMode`)
        (`KismetSystemLibrary.DrawDebugPoint` (`KismetMathLibrary.MakeVector` _returnvalue_x _returnvalue_y (`.MaxValue` (`KismetMathLibrary.MaxOfFloatArray` (`local.ImpactPoint_Local`)))) 16.0 (struct :`G` 1.0 :`A` 1.0))
        (`KismetSystemLibrary.DrawDebugPoint` (`KismetMathLibrary.MakeVector` _returnvalue_x_3 _returnvalue_y_3 (`.MinValue` (`KismetMathLibrary.MinOfFloatArray` (`local.ImpactPoint_Local`)))) 16.0 (struct :`B` 1.0 :`A` 1.0))))
    (:`then_1`
      ;[1 1 1] Set Closest/Furthest Distance
      (set `self.ClosestDistance` (- _returnvalue_z (`.MaxValue` (`KismetMathLibrary.MaxOfFloatArray` _impactpoint_local))))
      (set `self.FurthestDistance` (- _returnvalue_z (`.MinValue` (`KismetMathLibrary.MinOfFloatArray` _impactpoint_local))))
      (return (`local.bReturn_Local`)))))

(fn `Set`
  (bind _rendertextureresolution (`self.RenderTextureResolution`))
  (bind _decalcomponent (`self.DecalComponent`))
  ;[1 1 1] Set Owner's Mesh Components to not recieve Decals
  (for _array_element (`Actor.K2_GetComponentsByClass` (`self.GetOwner`) "/Script/Engine.MeshComponent")
    (`PrimitiveComponent.SetReceivesDecals` _array_element false))
  ;[1 1 1] Add Decal Component
  (bind _returnvalue (`|AddComponentByClass` (`self.GetOwner`) "/Script/Engine.DecalComponent" true (`KismetMathLibrary.MakeTransform` (0.0 0.0 0.0) (struct :`Pitch` -90.0 :`Roll` 90.0))))
  (set `self.DecalComponent` _returnvalue)
  ;[1 1 1] Select Material and create an Instance
  (`DecalComponent.SetDecalMaterial` _decalcomponent (select `bool` (`self.bUseRenderTexture`) :`false` "/Game/Graphics/DropShadow/Decals/M_BlobShadow.M_BlobShadow" :`true` "/Game/Graphics/DropShadow/Decals/M_DropShadow.M_DropShadow" :!type "MaterialInterface Object Reference"))
  (bind _returnvalue_2 (`DecalComponent.CreateDynamicMaterialInstance` _decalcomponent))
  (set `self.Material` _returnvalue_2)
  ;[1 1 1] Add Scene Capture Component
  (if (`self.bUseRenderTexture`)
    (bind _returnvalue_3 (`|AddComponentByClass` (`self.GetOwner`) "/Script/Engine.SceneCaptureComponent2D" true (`KismetMathLibrary.MakeTransform` (0.0 0.0 0.0) (struct :`Pitch` -90.0))))
    (bind _output_get (set `self.SceneCaptureComponent` _returnvalue_3))
    (set `SceneCaptureComponent2D.ProjectionType` "Orthographic" _output_get)
    (set `SceneCaptureComponent2D.OrthoWidth` (`self.SceneCaptureOrthoWidth`) _output_get)
    (set `SceneCaptureComponent.PrimitiveRenderMode` "PRM_UseShowOnlyList" _output_get)
    (set `SceneCaptureComponent.CaptureSource` "SCS_SceneDepth" _output_get)
    (set `SceneCaptureComponent.bCaptureEveryFrame` false _output_get)
    (set `SceneCaptureComponent.bCaptureOnMovement` false _output_get)
    ;[1 1 1] Create a new Render Target and apply it to our Material
    (bind _returnvalue_4 (`KismetRenderingLibrary.CreateRenderTarget2D` _rendertextureresolution _rendertextureresolution "RTF_R16f"))
    (bind _output_get_2 (set `SceneCaptureComponent2D.TextureTarget` _returnvalue_4 (`self.SceneCaptureComponent`)))
    (set `SceneCaptureComponent.ShowOnlyActors` (`|MakeArray` (`self.GetOwner`)) (`self.SceneCaptureComponent`))
    (`MaterialInstanceDynamic.SetTextureParameterValue` (`self.Material`) "Render target" _output_get_2)))

(fn `Update`
  (bind _returnvalue (`self.GetOwner`))
  (bind _material (`self.Material`))
  (bind (_returnvalue_x _returnvalue_y _returnvalue_z) (`KismetMathLibrary.BreakVector` (`Actor.K2_GetActorLocation` (`self.GetOwner`))))
  (bind _returnvalue_2 (`KismetMathLibrary.MapRangeClamped` (`self.CurrentDistance`) (`self.BlurAndDensityMinDistance`) (`self.BlurAndDensityMaxDistance`) 0.0 1.0))
  (bind (_returnvalue_x_2 _returnvalue_y_2 _returnvalue_z_2) (`KismetMathLibrary.BreakVector` (`Actor.K2_GetActorLocation` _returnvalue)))
  (bind (_returnvalue_x_3 _returnvalue_y_3 _returnvalue_z_3) (`KismetMathLibrary.BreakVector` (`Actor.K2_GetActorLocation` (`self.GetOwner`))))
  (bind _returnvalue_3 (/ (`self.DecalSize`) 256.0))
  ;[1 1 1] Draw Drop Shadow Traces
  (bind _return (`self.DrawTraces`))
  (if _return
    ;[1 1 1] Check Update
    (if (or (!= (`self.CurrentDistance`) (`self.ClosestDistance`)) (`self.bAlwaysUpdate`))
      ;[1 1 1] Interp to Closest Distance
      (set `self.CurrentDistance` (`KismetMathLibrary.FInterpTo` (`self.CurrentDistance`) (`self.ClosestDistance`) (`GameplayStatics.GetWorldDeltaSeconds`) (`self.FadeSpeed`)))
      ;[1 1 1] Set Decal Component's scale and location
      (`SceneComponent.SetWorldScale3D` (`self.DecalComponent`) (`KismetMathLibrary.MakeVector` (/ (`self.FurthestDistance`) 128.0) _returnvalue_3 _returnvalue_3))
      (`SceneComponent.K2_SetWorldLocation` (`self.DecalComponent`) (`KismetMathLibrary.MakeVector` _returnvalue_x _returnvalue_y (- _returnvalue_z (* (`self.ClosestDistance`) 0.5))) false false)
      ;[1 1 1] Update the material parameters
      (`MaterialInstanceDynamic.SetScalarParameterValue` (`self.Material`) "Cutoff mask distance" (- (+ _returnvalue_z_2 32.0) (.z (`.BoxExtent` (`Actor.GetActorBounds` _returnvalue true false)))))
      (`MaterialInstanceDynamic.SetScalarParameterValue` (`self.Material`) "Opacity" (`KismetMathLibrary.Lerp` 0.0 (`self.Opacity`) (`KismetMathLibrary.MapRangeClamped` (`self.CurrentDistance`) (`self.OpacityMinDistance`) (`self.OpacityMaxDistance`) 0.0 1.0)))
      (if (`self.bUseRenderTexture`)
        (`MaterialInstanceDynamic.SetScalarParameterValue` _material "Blur" (`CurveFloat.GetFloatValue` (`self.BlurCurve`) _returnvalue_2))
        ;[1 1 1] Set Scene Capture Component position
        (`SceneComponent.K2_SetWorldLocation` (`self.SceneCaptureComponent`) (`KismetMathLibrary.MakeVector` _returnvalue_x_3 _returnvalue_y_3 (+ _returnvalue_z_3 (`self.SceneCaptureHeight`))) false false)
        ;[1 1 1] Capture target
        (`SceneCaptureComponent2D.CaptureScene` (`self.SceneCaptureComponent`))
        (else
          (`MaterialInstanceDynamic.SetScalarParameterValue` _material "Density" (`CurveFloat.GetFloatValue` (`self.DensityCurve`) _returnvalue_2)))))))
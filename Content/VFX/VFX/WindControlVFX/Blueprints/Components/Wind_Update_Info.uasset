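; Wind_Update_Info is a Blueprint that pushes the Wind Manager's wind settings to particle effects in the level.
; WindUpdateInfo reads rotation, speed and gravity from BP_Wind_Manager, then finds every actor implementing Interface_Wind_Particle_True.
; It converts rotation and speed into a scaled horizontal vector, with gravity as Z.
; That vector sets the "Wind" parameter on each of those actors' ParticleSystemComponents.
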(fn `Wind_Update_Info`
  ;[1 0 0] Actualizamos la dirección del viento en las partículas según los parámetros del Wind Manager
  (bind _returnvalue (`GameplayStatics.GetActorOfClass` null "/Game/VFX/VFX/WindControlVFX/Blueprints/BP_Wind_Manager.BP_Wind_Manager_C"))
  ;;[0 1 1] Cogemos todas las BP con la Interface de Wind particle y accedemos a sus componentes de tipo Particle
  ;;;[1 1 0] Miramos Interface
  (bind _outactors (`GameplayStatics.GetAllActorsWithInterface` null "/Game/VFX/VFX/WindControlVFX/Blueprints/Components/Interface_Wind_Particle_True.Interface_Wind_Particle_True_C"))
  (for _array_element _outactors
    ;;;[0 1 0] Miramos Particulas
    (for _array_element_2 (`Actor.K2_GetComponentsByClass` _array_element "/Script/Engine.ParticleSystemComponent")
      (bind _returnvalue_2 (+ (`/Game/VFX/VFX/WindControlVFX/Blueprints/BP_Wind_Manager.Wind Rotation` _returnvalue) 90.0))
      (bind _wind_speed (`/Game/VFX/VFX/WindControlVFX/Blueprints/BP_Wind_Manager.Wind Speed` _returnvalue))
      (`ParticleSystemComponent.SetVectorParameter` _array_element_2 "Wind" (`KismetMathLibrary.MakeVector` (* (* (`KismetMathLibrary.DegSin` _returnvalue_2) _wind_speed) 250.0) (* (* _wind_speed (`KismetMathLibrary.DegCos` _returnvalue_2)) -250.0) (`/Game/VFX/VFX/WindControlVFX/Blueprints/BP_Wind_Manager.Gravity` _returnvalue))))))
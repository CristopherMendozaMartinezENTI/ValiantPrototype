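; Wind manager that randomly varies wind speed, and optionally direction, to drive particle effects.
; Two independent BeginPlay loops wait random intervals, then either snap to new random values or blend to them through duration-scaled timelines.
; Each change, blend tick and construction run adds the yaw to an arrow and pushes a "Wind" vector, with gravity as Z, into particle components on all actors implementing the wind particle interface.
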(event `self.ReceiveBeginPlay`
  (`|ExecutionSequence`
    (:`then_0`
      (if (`self.Random Wind Rotation`)
        (if (`self.Use Smooth wind changes`)
          (`KismetSystemLibrary.Delay` (`KismetMathLibrary.RandomFloatInRange` (`self.Min time before the wind rotation changes (sec)`) (`self.Max time before the wind rotation changes (sec)`)) :!label _label)
          (set `self.Old Wind Rotation` (`self.Wind Rotation`))
          (set `self.New Wind Rotation` (`KismetMathLibrary.RandomFloatInRange` (`self.Min Wind Rotation Value`) (`self.Max Wind Rotation Value`)))
          (`TimelineComponent.SetPlayRate` (`self.Timeline_0`) (/ 1.0 (`self.Duration of the smooth change of values (sec)`)))
          (bind (_direction _lerp) (`Timeline|Timeline_0` :!via `PlayFromStart`)
            (:`Update`
              (set `self.Wind Rotation` (`KismetMathLibrary.Lerp` (`self.Old Wind Rotation`) (`self.New Wind Rotation`) _lerp))
              (`self.Update Wind Values`))
            (:`Finished`
              (goto _label)))
          (else
            (`KismetSystemLibrary.Delay` (`KismetMathLibrary.RandomFloatInRange` (`self.Min time before the wind rotation changes (sec)`) (`self.Max time before the wind rotation changes (sec)`)) :!label _label_2)
            (set `self.New Wind Rotation` (`KismetMathLibrary.RandomFloatInRange` (`self.Min Wind Rotation Value`) (`self.Max Wind Rotation Value`)))
            (set `self.Wind Rotation` (`self.New Wind Rotation`))
            (`self.Update Wind Values`)
            (goto _label_2)))))
    (:`then_1`
      (if (`self.Use Smooth wind changes`)
        (`KismetSystemLibrary.Delay` (`KismetMathLibrary.RandomFloatInRange` (`self.Min time before the wind speed changes (sec)`) (`self.Max time before the wind speed changes (sec)`)) :!label _label_3)
        (set `self.Old Wind Speed` (`self.Wind Speed`))
        (set `self.New Wind Speed` (`KismetMathLibrary.RandomFloatInRange` (`self.Min Wind Speed Value`) (`self.Max Wind Speed Value`)))
        (`TimelineComponent.SetPlayRate` (`self.Timeline_1`) (/ 1.0 (`self.Duration of the smooth change of values (sec)`)))
        (bind (_direction_2 _lerp_2) (`Timeline|Timeline_1` :!via `PlayFromStart`)
          (:`Update`
            (set `self.Wind Speed` (`KismetMathLibrary.Lerp` (`self.Old Wind Speed`) (`self.New Wind Speed`) _lerp_2))
            (`self.Update Wind Values`))
          (:`Finished`
            (goto _label_3)))
        (else
          (`KismetSystemLibrary.Delay` (`KismetMathLibrary.RandomFloatInRange` (`self.Min time before the wind speed changes (sec)`) (`self.Max time before the wind speed changes (sec)`)) :!label _label_4)
          (set `self.New Wind Speed` (`KismetMathLibrary.RandomFloatInRange` (`self.Min Wind Speed Value`) (`self.Max Wind Speed Value`)))
          (set `self.Wind Speed` (`self.New Wind Speed`))
          (`self.Update Wind Values`)
          (goto _label_4))))))

(fn `Update Wind Values`
  (bind _wind_speed (`self.Wind Speed`))
  (bind _returnvalue (+ (`self.Wind Rotation`) 90.0))
  (`SceneComponent.K2_AddRelativeRotation` (`self.Arrow`) (`KismetMathLibrary.MakeRotator` 0.0 0.0 (`self.Wind Rotation`)) false false)
  (bind _outactors (`GameplayStatics.GetAllActorsWithInterface` "/Game/VFX/VFX/WindControlVFX/Blueprints/Components/Interface_Wind_Particle_True.Interface_Wind_Particle_True_C"))
  (for _array_element _outactors
    (for _array_element_2 (`self.K2_GetComponentsByClass` _array_element "/Script/Engine.ParticleSystemComponent")
      (`ParticleSystemComponent.SetVectorParameter` _array_element_2 "Wind" (`KismetMathLibrary.MakeVector` (* (* (`KismetMathLibrary.DegSin` _returnvalue) _wind_speed) 250.0) (* (* _wind_speed (`KismetMathLibrary.DegCos` _returnvalue)) -250.0) (`self.Gravity`))))))

(fn `UserConstructionScript`
  (`self.Update Wind Values`))
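; River generator actor that builds a flowing river or waterfall surface along an editable spline in the construction script.
; It adds a spline mesh per segment, taking position, tangents, roll and scale from the spline points times a global Scale.
; Each segment gets a dynamic material for speed, yaw-based rotation, border intensity and opacity mask, with fades only on end segments.
; A box trace that snaps the last point to the ground exists but is disabled.
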(event `self.ReceiveBeginPlay`)

(fn `SetupParameters`
  (params (Material :type "MaterialInstanceDynamic Object Reference") (`Current Index` :type Integer) (Spline :type "SplineComponent Object Reference"))
  (bind (_returnvalue_roll _returnvalue_pitch _returnvalue_yaw) (`KismetMathLibrary.BreakRotator` (`SceneComponent.K2_GetComponentRotation` Spline)))
  (`/Engine/EditorBlueprintResources/StandardMacros.IsValid` Spline
    (:`Is Valid`
      (`/Engine/EditorBlueprintResources/StandardMacros.IsValid` Material
        (:`Is Valid`
          (`|ExecutionSequence`
            (:`then_0`
              (if (== (- (`SplineComponent.GetNumberOfSplinePoints` Spline) 2) `Current Index`)
                (`MaterialInstanceDynamic.SetScalarParameterValue` Material "Back Fade" (`self.BackFade`))))
            (:`then_1`
              (if (== `Current Index` 0)
                (`MaterialInstanceDynamic.SetScalarParameterValue` Material "Front Fade" (`self.FrontFade`))))
            (:`then_2`
              (`MaterialInstanceDynamic.SetScalarParameterValue` Material "Rotation" (/ _returnvalue_yaw 360.0)))
            (:`then_3`
              (`MaterialInstanceDynamic.SetScalarParameterValue` Material "Speed" (`self.Speed`)))
            (:`then_4`
              (`MaterialInstanceDynamic.SetScalarParameterValue` Material "Boarder Intensity" (`self.BoarderColor`)))
            (:`then_5`
              (`MaterialInstanceDynamic.SetScalarParameterValue` Material "Opacity Mask" (`self.OpacityMask`)))))))))

(fn `SetupRiverTrace`
  (params (`Spline Input` :type "SplineComponent Object Reference") (Scale :type "Float (double-precision)"))
  (bind _returnvalue (`SplineComponent.GetNumberOfSplinePoints` `Spline Input`))
  (bind _returnvalue_2 (- _returnvalue 1))
  (bind _returnvalue_3 (`SplineComponent.GetLocationAtSplinePoint` `Spline Input` _returnvalue_2 "World"))
  (bind _outhit (`KismetSystemLibrary.BoxTraceSingle` :`Start` (`SplineComponent.GetLocationAtSplinePoint` `Spline Input` (- _returnvalue 1) "World") :`End` (+ (* (0.0 0.0 -1.0) 1000.0) _returnvalue_3) :`HalfSize` (`KismetMathLibrary.MakeVector` 1.0 (* Scale 30.0) 1.0) :`Orientation` (`SceneComponent.K2_GetComponentRotation` `Spline Input`) :`TraceChannel` "TraceTypeQuery1" :`bTraceComplex` true :`DrawTime` 1.0))
  (`SplineComponent.SetLocationAtSplinePoint` `Spline Input` _returnvalue_2 (`KismetMathLibrary.MakeVector` (.x _returnvalue_3) (.y _returnvalue_3) (.z (`.ImpactPoint` (`GameplayStatics.BreakHitResult` _outhit)))) "World" true))

(fn `SetupSplineMesh`
  (params (`Spline Comp` :type "SplineComponent Object Reference") (Scale :type "Float (double-precision)"))
  (for _index (range (+ (- (`SplineComponent.GetNumberOfSplinePoints` `Spline Comp`) 2) 1))
    (bind _returnvalue (`AddComponent|NODE_AddSplineMeshComponent-3`))
    (bind _returnvalue_2 (`PrimitiveComponent.CreateDynamicMaterialInstance` _returnvalue 0 (`self.Material`) "None"))
    (`self.SetupParameters` _returnvalue_2 _index `Spline Comp`)
    (bind (_returnvalue_x _returnvalue_y) (`KismetMathLibrary.BreakVector` (`SplineComponent.GetScaleAtSplinePoint` `Spline Comp` _index)))
    (`SplineMeshComponent.SetStartScale` _returnvalue (`KismetMathLibrary.MakeVector2D` (* _returnvalue_x Scale) (* Scale _returnvalue_y)) true)
    (bind (_returnvalue_x_2 _returnvalue_y_2) (`KismetMathLibrary.BreakVector` (`SplineComponent.GetScaleAtSplinePoint` `Spline Comp` (+ _index 1))))
    (`SplineMeshComponent.SetEndScale` _returnvalue (`KismetMathLibrary.MakeVector2D` (* _returnvalue_x_2 Scale) (* Scale _returnvalue_y_2)) true)
    (`SceneComponent.K2_AttachToComponent` _returnvalue `Spline Comp` "None" "KeepRelative" "KeepRelative" "KeepRelative" true)
    (`SplineMeshComponent.SetStartRoll` _returnvalue (* (`SplineComponent.GetRollAtSplinePoint` `Spline Comp` _index "Local") 0.01) true)
    (`SplineMeshComponent.SetEndRoll` _returnvalue (* (`SplineComponent.GetRollAtSplinePoint` `Spline Comp` (+ _index 1) "Local") 0.01) true)
    (bind (_location _tangent) (`SplineComponent.GetLocationAndTangentAtSplinePoint` `Spline Comp` _index "Local"))
    (bind (_location_2 _tangent_2) (`SplineComponent.GetLocationAndTangentAtSplinePoint` `Spline Comp` (+ _index 1) "Local"))
    (`SplineMeshComponent.SetStartAndEnd` _returnvalue _location _tangent _location_2 _tangent_2 true)))

(fn `UserConstructionScript`
  (if false
    (`self.SetupRiverTrace` (`self.Spline`) (`self.Scale`)))
  (`self.SetupSplineMesh` (`self.Spline`) (`self.Scale`)))
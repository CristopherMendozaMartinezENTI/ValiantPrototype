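; Day-night sky actor that rotates sun and moon lights by hour and drives the sky sphere's dynamic material.
; Tick reads the hour from the time component's DayTimeManager; the construction script repeats the update for editor preview.
; UpdateSky derives sun direction, color and height, then applies the normal or rainy preset through hour-based color curves.
; Normal tints height fog; rain disables sunlight and stars and drives volumetric fog material parameters.
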(event `self.ReceiveBeginPlay`)

(event `self.ReceiveTick`
  (params (DeltaSeconds :type "Float (single-precision)"))
  (bind (_returnvalue_roll _returnvalue_pitch _returnvalue_yaw) (`KismetMathLibrary.BreakRotator` (`self.K2_GetActorRotation`)))
  (bind _sun_actor (`self.Sun Actor`))
  (bind _moon_actor (`self.Moon Actor`))
  ;[1 1 1] Check Hour of the day and update SunActor
  (if (`KismetSystemLibrary.IsValid` (`/Game/Blueprints/TimeManager/BPC_TimeComponent.Day Time Manager` (`self.BPC_TimeComponent`)))
    (set `self.Hour` (`/Game/Blueprints/TimeManager/BP_DayTimeManager.Get Hour` (`/Game/Blueprints/TimeManager/BPC_TimeComponent.Day Time Manager` (`self.BPC_TimeComponent`))))
    (bind _output_get (set `self.Sun Angle` (+ (* (/ (`self.Hour`) 6.0) 90.0) 90.0)))
    (`/Engine/EditorBlueprintResources/StandardMacros.IsValid` _sun_actor
      (:`Is Valid`
        (`self.K2_SetActorRotation` _sun_actor (`KismetMathLibrary.MakeRotator` 0.0 _output_get _returnvalue_yaw) false)
        (`/Engine/EditorBlueprintResources/StandardMacros.IsValid` _moon_actor
          (:`Is Valid`
            (`self.K2_SetActorRotation` _moon_actor (`KismetMathLibrary.MakeRotator` -360.0 (+ (* (/ (`self.Hour`) 6.0) 90.0) -90.0) _returnvalue_yaw) false)
            (`self.UpdateSky`)))))))

(fn `SetPostProcessMats`)

(fn `UpdateNormalDay`
  (locals (NewLocalVar :type "Light Object Reference"))
  (bind _sun_height (`self.Sun height`))
  (bind _sky_material (`self.Sky material`))
  (bind _sky_material_2 (`self.Sky material`))
  (`MaterialInstanceDynamic.SetVectorParameterValue` _sky_material "Horizon color" (`CurveLinearColor.GetClampedLinearColorValue` (`self.Horizon Color `) (`self.Hour`)))
  (`MaterialInstanceDynamic.SetVectorParameterValue` _sky_material "Zenith color" (`CurveLinearColor.GetClampedLinearColorValue` (`self.Zenith Color `) (`self.Hour`)))
  (`MaterialInstanceDynamic.SetScalarParameterValue` _sky_material "Horizon falloff" (`KismetMathLibrary.Lerp` 3.0 7.0 (`KismetMathLibrary.Abs` (`self.Sun height`))))
  (`MaterialInstanceDynamic.SetVectorParameterValue` _sky_material "Overall color" (`self.Overall Color`))
  (`MaterialInstanceDynamic.SetScalarParameterValue` _sky_material_2 "Cloud speed" (`self.Cloud speed`))
  (`MaterialInstanceDynamic.SetScalarParameterValue` _sky_material_2 "Sun brightness" (`self.Sun brightness`))
  (`MaterialInstanceDynamic.SetScalarParameterValue` _sky_material_2 "Sun height" (`KismetMathLibrary.SelectFloat` (`KismetMathLibrary.Abs` _sun_height) 0.0 (< _sun_height 0.0)))
  (`MaterialInstanceDynamic.SetScalarParameterValue` _sky_material_2 "Cloud opacity" (`self.Cloud opacity`))
  (`MaterialInstanceDynamic.SetScalarParameterValue` _sky_material_2 "Stars brightness" (`self.Stars brightness`))
  (`ExponentialHeightFogComponent.SetFogInscatteringColor` (`self.ExponentialHeightFog`) (`CurveLinearColor.GetClampedLinearColorValue` (`self.Horizon Color `) (`self.Hour`))))

(fn `UpdateRainyDay`
  (bind _celshader (`self.Celshader`))
  (bind _sun_height (`self.Sun height`))
  (bind _sun_height_2 (`self.Sun height`))
  (bind _volumetricfoginstance (`self.VolumetricFogInstance`))
  (bind _sky_material (`self.Sky material`))
  (bind _sky_material_2 (`self.Sky material`))
  (`LightComponent.SetIntensity` (`Light.LightComponent` (`self.Sun Actor`)) 0.0)
  (`MaterialInstanceDynamic.SetVectorParameterValue` _sky_material "Horizon color" (`CurveLinearColor.GetClampedLinearColorValue` (`self.Horizon Color - Rain`) (`self.Hour`)))
  (`MaterialInstanceDynamic.SetVectorParameterValue` _sky_material "Zenith color" (`CurveLinearColor.GetClampedLinearColorValue` (`self.Zenith Color - Rain`) (`self.Hour`)))
  (`MaterialInstanceDynamic.SetVectorParameterValue` _sky_material "Cloud color" (`CurveLinearColor.GetClampedLinearColorValue` (`self.Cloud Color - Rain`) _sun_height_2))
  (`MaterialInstanceDynamic.SetScalarParameterValue` _sky_material "Horizon falloff" (`KismetMathLibrary.Lerp` 3.0 7.0 (`KismetMathLibrary.Abs` _sun_height_2)))
  (`MaterialInstanceDynamic.SetVectorParameterValue` _sky_material "Overall color" (`self.Overall Color`))
  (`MaterialInstanceDynamic.SetScalarParameterValue` _sky_material_2 "Cloud speed" (`self.Cloud speed`))
  (`MaterialInstanceDynamic.SetScalarParameterValue` _sky_material_2 "Sun brightness" 0.0)
  (`MaterialInstanceDynamic.SetScalarParameterValue` _sky_material_2 "Sun height" (`KismetMathLibrary.SelectFloat` (`KismetMathLibrary.Abs` _sun_height) 0.0 (< _sun_height 0.0)))
  (`MaterialInstanceDynamic.SetScalarParameterValue` _sky_material_2 "Cloud opacity" (`self.Cloud opacity`))
  (`MaterialInstanceDynamic.SetScalarParameterValue` _sky_material_2 "Stars brightness" 0.0)
  (`/Engine/EditorBlueprintResources/StandardMacros.IsValid` _volumetricfoginstance
    (:`Is Valid`
      (bind _asmaterial_instance_dynamic (cast `MaterialInstanceDynamic` _volumetricfoginstance))
      (`MaterialInstanceDynamic.SetVectorParameterValue` _asmaterial_instance_dynamic "FogColor" (`CurveLinearColor.GetClampedLinearColorValue` (`self.Horizon Color - Rain`) (`self.Hour`)))
      (`MaterialInstanceDynamic.SetScalarParameterValue` _asmaterial_instance_dynamic "FogOpacity" (`CurveFloat.GetFloatValue` (`self.Fog Density - Rain`) (`self.Hour`)))
      (`MaterialInstanceDynamic.SetScalarParameterValue` _asmaterial_instance_dynamic "FogDistance" (`CurveFloat.GetFloatValue` (`self.Fog Distance`) (`self.Hour`)))
      (`/Engine/EditorBlueprintResources/StandardMacros.IsValid` _celshader
        (:`Is Valid`
          (bind _asmaterial_instance_dynamic_2 (cast `MaterialInstanceDynamic` _celshader))
          (`MaterialInstanceDynamic.SetVectorParameterValue` _asmaterial_instance_dynamic_2 "Shadow Tint" (`CurveLinearColor.GetClampedLinearColorValue` (`self.Celshader Exposure - Rain`) (`self.Hour`))))))))

(fn `UpdateSky`
  (bind _sky_material (`self.Sky material`))
  (bind _sky_material_2 (`self.Sky material`))
  (`/Engine/EditorBlueprintResources/StandardMacros.IsValid` (`self.Sun Actor`)
    (:`Is Valid`
      (`MaterialInstanceDynamic.SetVectorParameterValue` _sky_material_2 "Light direction" (`KismetMathLibrary.Conv_VectorToLinearColor` (`KismetMathLibrary.Conv_RotatorToVector` (`self.K2_GetActorRotation` (`self.Sun Actor`)))))
      (`MaterialInstanceDynamic.SetVectorParameterValue` _sky_material_2 "Sun color" (`KismetMathLibrary.Conv_ColorToLinearColor` (`LightComponentBase.LightColor` (`Light.LightComponent` (`self.Sun Actor`)))))
      (set `self.Sun height` (`KismetMathLibrary.MapRangeUnclamped` (.pitch (`self.K2_GetActorRotation` (`self.Sun Actor`))) 0.0 -90.0 0.0 1.0)))
    (:`Is Not Valid`
      (`MaterialInstanceDynamic.SetVectorParameterValue` _sky_material "Light direction" (`KismetMathLibrary.Conv_VectorToLinearColor` (`KismetMathLibrary.Conv_RotatorToVector` (`KismetMathLibrary.MakeRotator` 0.0 (`KismetMathLibrary.MapRangeUnclamped` (`self.Sun height`) -1.0 1.0 90.0 -90.0) (.yaw (`self.K2_GetActorRotation`))))))
      (`MaterialInstanceDynamic.SetVectorParameterValue` _sky_material "Sun color" (`KismetMathLibrary.LinearColorLerp` (struct :`R` 1.0 :`G` 0.221 :`B` 0.04 :`A` 1.0) (struct :`R` 0.954 :`G` 0.901 :`B` 0.74412 :`A` 1.0) (`KismetMathLibrary.FClamp` (+ (`self.Sun height`) 0.2))))))
  (switch `int` (`KismetMathLibrary.Conv_ByteToInt` (`self.SkyPreset`))
    (:`0`
      (`self.UpdateNormalDay`))
    (:`1`
      (`self.UpdateRainyDay`))))

(fn `UserConstructionScript`
  (bind (_returnvalue_roll _returnvalue_pitch _returnvalue_yaw) (`KismetMathLibrary.BreakRotator` (`self.K2_GetActorRotation`)))
  (bind _sun_actor (`self.Sun Actor`))
  (bind _moon_actor (`self.Moon Actor`))
  (`self.SetPostProcessMats`)
  (bind _returnvalue (`PrimitiveComponent.CreateDynamicMaterialInstance` (`self.SkySphereMesh`) 0 "/Game/VFX/DayCicle/Materials/M_Sky.M_Sky" "None"))
  (set `self.Sky material` _returnvalue)
  (if (`self.Refresh material`)
    _
    (else
      _))
  (set `self.Refresh material` true)
  (bind _output_get (set `self.Sun Angle` (+ (* (/ (`self.Hour`) 6.0) 90.0) 90.0)))
  (`/Engine/EditorBlueprintResources/StandardMacros.IsValid` _sun_actor
    (:`Is Valid`
      (`self.K2_SetActorRotation` _sun_actor (`KismetMathLibrary.MakeRotator` 0.0 _output_get _returnvalue_yaw) false)
      (`/Engine/EditorBlueprintResources/StandardMacros.IsValid` _moon_actor
        (:`Is Valid`
          (`self.K2_SetActorRotation` _moon_actor (`KismetMathLibrary.MakeRotator` -360.0 (+ (* (/ (`self.Hour`) 6.0) 90.0) -90.0) _returnvalue_yaw) false)
          (`self.UpdateSky`))))))
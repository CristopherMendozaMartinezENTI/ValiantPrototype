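; Sky sphere Blueprint that drives a sky material with sun, gradient, cloud and star settings taken from its variables.
; The construction script creates a dynamic material instance and runs RefreshMaterial, with a self-resetting bool as an editor refresh toggle.
; Sun direction, color and height follow an assigned directional light, otherwise direction and color derive from SunHeight; negative height blends in stars.
; UpdateSunDirection re-pushes only light-driven values and some colors.
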(fn `RefreshMaterial`
  (bind _sky_material (`self.Sky material`))
  (bind _sky_material_2 (`self.Sky material`))
  (bind _sky_material_3 (`self.Sky material`))
  (bind _sun_height (`self.Sun height`))
  (bind _sky_material_4 (`self.Sky material`))
  (`/Engine/EditorBlueprintResources/StandardMacros.IsValid` (`self.Directional light actor`) ; Has a directional light been assigned?
    (:`Is Valid`
      (`MaterialInstanceDynamic.SetVectorParameterValue` _sky_material_3 "Light direction" (`KismetMathLibrary.Conv_VectorToLinearColor` (`KismetMathLibrary.Conv_RotatorToVector` (`self.K2_GetActorRotation` (`self.Directional light actor`)))))
      (`MaterialInstanceDynamic.SetVectorParameterValue` _sky_material_3 "Sun color" (`KismetMathLibrary.Conv_ColorToLinearColor` (`LightComponentBase.LightColor` (`Light.LightComponent` (`self.Directional light actor`)))))
      (set `self.Sun height` (`KismetMathLibrary.MapRangeUnclamped` (.pitch (`self.K2_GetActorRotation` (`self.Directional light actor`))) 0.0 -90.0 0.0 1.0)))
    (:`Is Not Valid`
      (`MaterialInstanceDynamic.SetVectorParameterValue` _sky_material_2 "Light direction" (`KismetMathLibrary.Conv_VectorToLinearColor` (`KismetMathLibrary.Conv_RotatorToVector` (`KismetMathLibrary.MakeRotator` 0.0 (`KismetMathLibrary.MapRangeUnclamped` (`self.Sun height`) -1.0 1.0 90.0 -90.0) (.yaw (`self.K2_GetActorRotation`))))))
      (`MaterialInstanceDynamic.SetVectorParameterValue` _sky_material_2 "Sun color" (`KismetMathLibrary.LinearColorLerp` (struct :`R` 1.0 :`G` 0.221 :`B` 0.04 :`A` 1.0) (struct :`R` 0.954 :`G` 0.901 :`B` 0.74412 :`A` 1.0) (`KismetMathLibrary.FClamp` (+ (`self.Sun height`) 0.2))))))
  (`MaterialInstanceDynamic.SetVectorParameterValue` _sky_material "Horizon color" (`self.Horizon color`))
  (`MaterialInstanceDynamic.SetVectorParameterValue` _sky_material "Zenith color" (`self.Zenith Color`))
  (`MaterialInstanceDynamic.SetVectorParameterValue` _sky_material "Overall color" (`self.Overall Color`))
  (`MaterialInstanceDynamic.SetVectorParameterValue` _sky_material "Cloud color" (`self.Cloud color`))
  (`MaterialInstanceDynamic.SetScalarParameterValue` _sky_material "Horizon falloff" (`self.Horizon Falloff`))
  (`MaterialInstanceDynamic.SetScalarParameterValue` _sky_material_4 "Cloud speed" (`self.Cloud speed`))
  (`MaterialInstanceDynamic.SetScalarParameterValue` _sky_material_4 "Sun brightness" (`self.Sun brightness`))
  (`MaterialInstanceDynamic.SetScalarParameterValue` _sky_material_4 "Sun height" (`KismetMathLibrary.SelectFloat` (`KismetMathLibrary.Abs` _sun_height) 0.0 (< _sun_height 0.0)))
  (`MaterialInstanceDynamic.SetScalarParameterValue` _sky_material_4 "Cloud opacity" (`self.Cloud opacity`))
  (`MaterialInstanceDynamic.SetScalarParameterValue` _sky_material_4 "Stars brightness" (`self.Stars brightness`))
  (`MaterialInstanceDynamic.SetScalarParameterValue` _sky_material_4 "OverallBrightness" (`self.OverallBrightness`)))

(fn `UpdateSunDirection`
  (bind _sky_material (`self.Sky material`))
  (bind _sun_height (`self.Sun height`))
  (bind _sky_material_2 (`self.Sky material`))
  (`MaterialInstanceDynamic.SetVectorParameterValue` _sky_material "Light direction" (`KismetMathLibrary.Conv_VectorToLinearColor` (`KismetMathLibrary.Conv_RotatorToVector` (`self.K2_GetActorRotation` (`self.Directional light actor`)))))
  (`MaterialInstanceDynamic.SetVectorParameterValue` _sky_material "Sun color" (`KismetMathLibrary.Conv_ColorToLinearColor` (`LightComponentBase.LightColor` (`Light.LightComponent` (`self.Directional light actor`)))))
  (set `self.Sun height` (`KismetMathLibrary.MapRangeUnclamped` (.pitch (`self.K2_GetActorRotation` (`self.Directional light actor`))) 0.0 -90.0 0.0 1.0))
  (`MaterialInstanceDynamic.SetVectorParameterValue` _sky_material_2 "Horizon color" (`self.Horizon color`))
  (`MaterialInstanceDynamic.SetVectorParameterValue` _sky_material_2 "Zenith color" (`self.Zenith Color`))
  (`MaterialInstanceDynamic.SetVectorParameterValue` _sky_material_2 "Cloud color" (`self.Cloud color`))
  (`MaterialInstanceDynamic.SetScalarParameterValue` _sky_material_2 "Horizon falloff" (`self.Horizon Falloff`))
  (`MaterialInstanceDynamic.SetScalarParameterValue` _sky_material_2 "Sun height" (`KismetMathLibrary.SelectFloat` (`KismetMathLibrary.Abs` _sun_height) 0.0 (< _sun_height 0.0))))

(fn `UserConstructionScript`
  (bind _skyspheremesh (`self.SkySphereMesh`))
  (bind _returnvalue (`PrimitiveComponent.CreateDynamicMaterialInstance` _skyspheremesh 0 (`PrimitiveComponent.GetMaterial` _skyspheremesh 0) "None"))
  (set `self.Sky material` _returnvalue)
  (if (`self.Refresh material`)
    _
    (else
      _))
  (set `self.Refresh material` false)
  (`self.RefreshMaterial`))
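; BP_InteractiveFoliageChunk is a chunk of interactive foliage that links its foliage component to a Manager.
; Its construction script assigns the Manager to FoliageComponent.Manager in every configuration.
; Two flags choose whether the default component stays untouched, the component reference is swapped to SourceFoliageComp, or the existing component receives parameters from that source via SetFoliageParameters.
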(fn `UserConstructionScript`
  (if (`self.leaveDefaultComponent`)
    (set `/Game/VFX/DynamicFoliage/Blueprints/Classes/BP_Interactive_FoliageComp.Manager` (`self.manager`) (`self.FoliageComponent`))
    (elif (`self.replaceWithSourceComponent`)
      (set `self.FoliageComponent` (`self.sourceFoliageComp`))
      (set `/Game/VFX/DynamicFoliage/Blueprints/Classes/BP_Interactive_FoliageComp.Manager` (`self.manager`) (`self.FoliageComponent`))
      (else
        (set `/Game/VFX/DynamicFoliage/Blueprints/Classes/BP_Interactive_FoliageComp.Manager` (`self.manager`) (`self.FoliageComponent`))
        (`/Game/VFX/DynamicFoliage/Blueprints/Classes/BP_Interactive_FoliageComp.SetFoliageParameters` (`self.FoliageComponent`) (`self.sourceFoliageComp`))))))
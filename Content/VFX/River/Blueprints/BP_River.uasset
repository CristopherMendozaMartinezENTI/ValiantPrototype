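; Spline-based river actor that builds its water surface and waterfall mist and splash particles, and optionally makes physics objects float and drift downstream.
; Construction lays spline meshes per segment and spawns particles where the tangent drops steeply.
; At BeginPlay, spline-mesh triggers are created along the river for buoyancy.
; Tick disables gravity on overlapping bodies, applying height-based lift and spline-direction flow, steered from obstacles by averaging three trace normals while moving.
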(event `self.ReceiveBeginPlay`
  (if (`self.EnableBuoyancy`)
    (`self.CreateTriggerMeshes`)))

(event `self.ReceiveActorBeginOverlap`
  (params (OtherActor :type "Actor Object Reference"))
  (if (`self.EnableBuoyancy`)
    (`KismetArrayLibrary.Array_AddUnique` (`self.ActorInWaterList`) (`self.GetComponentByClass` OtherActor "/Script/Engine.StaticMeshComponent"))))

(event `self.ReceiveActorEndOverlap`
  (params (OtherActor :type "Actor Object Reference"))
  (bind _returnvalue (`self.GetComponentByClass` OtherActor "/Script/Engine.StaticMeshComponent"))
  ;[1 1 1] Activamos la gravedad de los objetos despues del overlap
  (if (`self.EnableBuoyancy`)
    (`PrimitiveComponent.SetEnableGravity` _returnvalue true)
    (`KismetArrayLibrary.Array_RemoveItem` (`self.ActorInWaterList`) _returnvalue)))

(event `self.ReceiveTick`
  (params (DeltaSeconds :type "Float (single-precision)"))
  (bind _spline (`self.Spline`))
  (bind _impact_normals (`self.Impact Normals`))
  (bind _returnvalue (* (/ (`self.EasyScale`) 2.0) 100.0))
  (`|ExecutionSequence`
    (:`then_0`
      ;[1 1 1] Debug - Object Flow
      (if (`self.Physics Flow Debug`)
        (set `self.Physics Flow Debug Type` "ForDuration")
        (else
          (set `self.Physics Flow Debug Type` "None")))
      ;[1 1 1] Cogemos los overlapping actors de la trigger list y los seteamos a 'actor in water list'
      (if (`self.EnableBuoyancy`)
        (for (_array_element _array_index) (`self.TriggerList`)
          (for _array_element_2 (`self.ActorInWaterList`)
            ;[1 1 1] Recorremos "actor in water list", cogemos los mesh componenes y los seteamos a "mesh components in water"
            (`/Engine/EditorBlueprintResources/StandardMacros.IsValid` _array_element_2
              (:`Is Valid`
                (if (`PrimitiveComponent.IsOverlappingActor` _array_element (`ActorComponent.GetOwner` _array_element_2))
                  ;[1 1 1] Comprobamos si las meshes tiene "simulating physics"
                  (if (`SceneComponent.IsAnySimulatingPhysics` _array_element_2)
                    ;[1 1 1] Seteamos gravedad dependiendo si esta la mesh eencima o debajo del agua
                    (`PrimitiveComponent.SetEnableGravity` _array_element_2 false)
                    ;[1 1 1] Miramos la velocidad si el objeto se detiene
                    (if (== (`SceneComponent.GetComponentVelocity` _array_element_2) (0.0 0.0 0.0) :`ErrorTolerance` 7.0)
                      (bind _returnvalue_2 (`SplineComponent.GetDirectionAtSplinePoint` _spline _array_index "World"))
                      (bind _returnvalue_3 (`PrimitiveComponent.GetMass` _array_element_2))
                      (bind _returnvalue_4 (* (`self.Physics Flow Speed`) _returnvalue_3))
                      (bind (_returnvalue_x _returnvalue_y) (`KismetMathLibrary.BreakVector` (* _returnvalue_2 _returnvalue_4)))
                      (bind (_returnvalue_x_2 _returnvalue_y_2 _returnvalue_z) (`KismetMathLibrary.BreakVector` (`SplineComponent.GetLocationAtSplinePoint` _spline _array_index "World")))
                      (bind (_returnvalue_x_3 _returnvalue_y_3 _returnvalue_z_2) (`KismetMathLibrary.BreakVector` (`SceneComponent.K2_GetComponentLocation` _array_element_2)))
                      (bind (_returnvalue_x_4 _returnvalue_y_4 _returnvalue_z_3) (`KismetMathLibrary.BreakVector` (* (* (`KismetMathLibrary.MakeVector` 0.0 0.0 600.0) _returnvalue_3) (`KismetMathLibrary.FClamp` (/ (- _returnvalue_z _returnvalue_z_2) 50.0) -1.0))))
                      (set `self.RiverForce` (`KismetMathLibrary.MakeVector` _returnvalue_x _returnvalue_y _returnvalue_z_3))
                      ;[1 1 1] Sumamos las fuerzas del rio y el bouyancy ricamente para tener un rio guapo guapisimo
                      (`PrimitiveComponent.AddForce` _array_element_2 (`self.RiverForce`) "None" false :!label _label)
                      (else
                        ;[1 1 1] Proyectamos tres lineas y miramos la normal del sitio donde colisiona y con eso calculamos la direccion del rio
                        (`|ExecutionSequence`
                          (:`then_0`
                            (bind (_returnvalue_x_5 _returnvalue_y_5) (`KismetMathLibrary.BreakVector` (`SceneComponent.K2_GetComponentLocation` _array_element_2)))
                            (bind _returnvalue_5 (`KismetMathLibrary.MakeVector` _returnvalue_x_5 _returnvalue_y_5 _returnvalue_z))
                            (bind (_returnvalue_x_6 _returnvalue_y_6) (`KismetMathLibrary.BreakVector` (`SceneComponent.GetComponentVelocity` _array_element_2)))
                            (bind _returnvalue_6 (`KismetMathLibrary.Normal` (`KismetMathLibrary.MakeVector` _returnvalue_x_6 _returnvalue_y_6)))
                            (bind _returnvalue_7 (`KismetMathLibrary.Cross_VectorVector` _returnvalue_6 (0.0 0.0 1.0)))
                            (bind _impactnormal (`self.TraceNormal` _returnvalue_5 (+ _returnvalue_5 (* (+ _returnvalue_6 (`KismetMathLibrary.NegateVector` (* _returnvalue_7 (`self.Physics Flow Direction Width`)))) (`self.Physics Flow Direction Length`)))))
                            (`KismetArrayLibrary.Array_Set` _impact_normals 0 _impactnormal true))
                          (:`then_1`
                            (bind _impactnormal_2 (`self.TraceNormal` _returnvalue_5 (+ _returnvalue_5 (* (`SplineComponent.GetDirectionAtSplinePoint` (`self.Spline`) _array_index "World") (`self.Physics Flow Direction Length`)))))
                            (`KismetArrayLibrary.Array_Set` _impact_normals 1 _impactnormal_2 true))
                          (:`then_2`
                            (bind _impactnormal_3 (`self.TraceNormal` _returnvalue_5 (+ _returnvalue_5 (* (+ _returnvalue_6 (* _returnvalue_7 (`self.Physics Flow Direction Width`))) (`self.Physics Flow Direction Length`)))))
                            (`KismetArrayLibrary.Array_Set` _impact_normals 2 _impactnormal_3 true))
                          (:`then_3`
                            ;[1 1 1] Debug - Flow Direction
                            (if (not (not (`self.Physics Flow Debug`)))
                              (bind _returnvalue_8 (`SceneComponent.K2_GetComponentLocation` _array_element_2))
                              (bind (_returnvalue_x_7 _returnvalue_y_7) (`KismetMathLibrary.BreakVector` (`SceneComponent.GetComponentVelocity` _array_element_2)))
                              (bind _returnvalue_9 (+ (* (* (`KismetMathLibrary.MakeVector` (.x (`KismetMathLibrary.GetVectorArrayAverage` (`self.Impact Normals`))) (.y (`KismetMathLibrary.GetVectorArrayAverage` (`self.Impact Normals`)))) (`self.Physics Flow Avoidance Strength`)) (/ (`KismetMathLibrary.VSize` (`KismetMathLibrary.MakeVector` _returnvalue_x_7 _returnvalue_y_7)) 200.0)) _returnvalue_2))
                              (`KismetSystemLibrary.DrawDebugArrow` _returnvalue_8 (+ _returnvalue_8 (* _returnvalue_9 500.0)) 1000.0 (struct :`G` 0.665348 :`B` 1.0 :`A` 1.0) 0.1 5.0))
                            (bind (_returnvalue_x_8 _returnvalue_y_8) (`KismetMathLibrary.BreakVector` (* _returnvalue_9 _returnvalue_4)))
                            (set `self.RiverForce` (`KismetMathLibrary.MakeVector` _returnvalue_x_8 _returnvalue_y_8 _returnvalue_z_3))
                            (goto _label)))))
                    (else
                      (`PrimitiveComponent.SetEnableGravity` _array_element_2 true))))))))))
    (:`then_1`
      ;[1 1 1] Seteamos las particulas de la cascada respecto la escala del rio
      (for _array_element_3 (`self.ListOfWaterfallParticles`)
        (`/Engine/EditorBlueprintResources/StandardMacros.IsValid` _array_element_3
          (:`Is Valid`
            (`ParticleSystemComponent.SetVectorParameter` _array_element_3 "Location" (`KismetMathLibrary.MakeVector` 0.0 (`KismetMathLibrary.RandomFloatInRange` (* _returnvalue -1.0) _returnvalue)))
            (`PrimitiveComponent.CreateDynamicMaterialInstance` _array_element_3 0 "/Game/VFX/River/Materials/Particles/Mist_Inst.Mist_Inst" "None")
            (`PrimitiveComponent.CreateDynamicMaterialInstance` _array_element_3 1 "/Game/VFX/River/Materials/Particles/Splash_Inst.Splash_Inst" "None")))))))

(fn `CreateTriggerMeshes`
  (bind _spline (`self.Spline`))
  (bind _watertriggerthickness (`self.WaterTriggerThickness`))
  ;[1 1 1] Loop spline points
  (`KismetArrayLibrary.Array_Clear` (`self.TriggerList`))
  (for _index (range (+ (- (`SplineComponent.GetNumberOfSplinePoints` (`self.Spline`)) 2) 1))
    ;[1 1 1] Añadimos triggers
    (bind _returnvalue (`AddComponent|NODE_AddSplineMeshComponent-2`))
    (bind _returnvalue_x (`KismetMathLibrary.BreakVector` (`SplineComponent.GetScaleAtSplinePoint` (`self.Spline`) _index)))
    ;[1 1 1] Seteamos escalas
    (`SplineMeshComponent.SetStartScale` _returnvalue (`KismetMathLibrary.MakeVector2D` (* (* _returnvalue_x 0.4) (`self.EasyScale`)) _watertriggerthickness) true)
    (bind _returnvalue_x_2 (`KismetMathLibrary.BreakVector` (`SplineComponent.GetScaleAtSplinePoint` (`self.Spline`) (+ _index 1))))
    (`SplineMeshComponent.SetEndScale` _returnvalue (`KismetMathLibrary.MakeVector2D` (* (* _returnvalue_x_2 0.4) (`self.EasyScale`)) _watertriggerthickness) true)
    (bind (_location _tangent) (`SplineComponent.GetLocationAndTangentAtSplinePoint` _spline _index "Local"))
    (bind _returnvalue_2 (+ (- (* (.z (`.BoxExtent` (`KismetSystemLibrary.GetComponentBounds` _returnvalue))) (`self.WaterTriggerThickness`)) 128.0) (`self.WaterTriggerHeightOffset`)))
    (bind (_location_2 _tangent_2) (`SplineComponent.GetLocationAndTangentAtSplinePoint` _spline (+ _index 1) "Local"))
    ;[1 1 1] Lo colocamos en el Root
    (`SplineMeshComponent.SetStartAndEnd` _returnvalue (`KismetMathLibrary.MakeVector` (.x _location) (.y _location) (- (.z _location) _returnvalue_2)) _tangent (`KismetMathLibrary.MakeVector` (.x _location_2) (.y _location_2) (- (.z _location_2) _returnvalue_2)) _tangent_2 true)
    (`KismetArrayLibrary.Array_AddUnique` (`self.TriggerList`) _returnvalue)))

(fn `TraceNormal`
  (params (Start :type "Vector Structure") (End :type "Vector Structure"))
  (returns (ImpactNormal :type "Vector Structure"))
  (bind _outactorlist (`KismetSystemLibrary.GetActorListFromComponentList` (`self.ActorInWaterList`) "/Script/Engine.Actor"))
  (bind _outhit (`KismetSystemLibrary.LineTraceSingle` Start End "TraceTypeQuery1" false _outactorlist (`self.Physics Flow Debug Type`) true (struct :`R` 1.0 :`A` 1.0) (struct :`G` 1.0 :`A` 1.0) 0.1))
  (return (`.ImpactNormal` (`GameplayStatics.BreakHitResult` _outhit))))

(fn `UserConstructionScript`
  (bind _spline (`self.Spline`))
  (bind _easyscale (`self.EasyScale`))
  (bind _easyscale_2 (`self.EasyScale`))
  (bind _spline_2 (`self.Spline`))
  ;[1 1 1] Loop spline points
  (for _index (range (+ (- (`SplineComponent.GetNumberOfSplinePoints` (`self.Spline`)) 2) 1))
    (`|ExecutionSequence`
      (:`then_0`
        ;[1 1 1] Añadimos la mesh y el material
        (bind _returnvalue (`AddComponent|NODE_AddSplineMeshComponent-0`))
        (set `ActorComponent.ComponentTags` (`|MakeArray` (`self.Fluid Interaction Tag`)) _returnvalue)
        (`PrimitiveComponent.SetMaterial` _returnvalue 0 (`self.River Material`))
        (bind (_returnvalue_roll _returnvalue_pitch _returnvalue_yaw) (`KismetMathLibrary.BreakRotator` (`SceneComponent.K2_GetComponentRotation` _returnvalue)))
        (`MeshComponent.SetScalarParameterValueOnMaterials` _returnvalue "ObjectZRotation" (/ (`KismetMathLibrary.Abs` _returnvalue_yaw) 360.0))
        (bind (_returnvalue_x _returnvalue_y) (`KismetMathLibrary.BreakVector` (`SplineComponent.GetScaleAtSplinePoint` (`self.Spline`) _index)))
        ;[1 1 1] Setamos escala
        (`SplineMeshComponent.SetStartScale` _returnvalue (`KismetMathLibrary.MakeVector2D` (* _returnvalue_x _easyscale) (* _easyscale _returnvalue_y)) true)
        (bind (_returnvalue_x_2 _returnvalue_y_2) (`KismetMathLibrary.BreakVector` (`SplineComponent.GetScaleAtSplinePoint` (`self.Spline`) (+ _index 1))))
        (`SplineMeshComponent.SetEndScale` _returnvalue (`KismetMathLibrary.MakeVector2D` (* _returnvalue_x_2 _easyscale_2) (* _easyscale_2 _returnvalue_y_2)) true)
        ;[1 1 1] Lo colocamos en el Root
        (`SceneComponent.K2_AttachToComponent` _returnvalue null "None" "KeepRelative" "KeepRelative" "KeepRelative" true)
        (bind (_location _tangent) (`SplineComponent.GetLocationAndTangentAtSplinePoint` _spline _index "Local"))
        (bind (_location_2 _tangent_2) (`SplineComponent.GetLocationAndTangentAtSplinePoint` _spline (+ _index 1) "Local"))
        (`SplineMeshComponent.SetStartAndEnd` _returnvalue _location _tangent _location_2 _tangent_2 true))
      (:`then_2`
        (bind (_returnvalue_x_3 _returnvalue_y_3 _returnvalue_z) (`KismetMathLibrary.BreakVector` (`SplineComponent.GetTangentAtSplinePoint` _spline_2 _index "Local")))
        ;[1 1 1] Setamos waterfalls
        (if (and (< _returnvalue_z (`self.Waterfall Tangent Start`)) (`self.Waterfalls`))
          (bind _returnvalue_2 (`AddComponent|NODE_AddParticleSystemComponent-0` :`RelativeTransform` (`KismetMathLibrary.MakeTransform` (`SplineComponent.GetLocationAtSplinePoint` _spline_2 _index "Local") (`SplineComponent.GetRotationAtSplinePoint` _spline_2 _index "Local"))))
          (`ParticleSystemComponent.SetFloatParameter` _returnvalue_2 "SplashDensity" (`self.Splash Density`))
          (`ParticleSystemComponent.SetFloatParameter` _returnvalue_2 "MistDensity" (`self.Mist Density`))
          (`ParticleSystemComponent.SetEmitterEnable` _returnvalue_2 "Particle Emitter" true)
          (bind _returnvalue_3 (`PrimitiveComponent.CreateDynamicMaterialInstance` _returnvalue_2 0 "/Game/VFX/River/Materials/Particles/Mist_Inst.Mist_Inst" "None"))
          (`MaterialInstanceDynamic.SetScalarParameterValue` _returnvalue_3 "Emissive Toggle" (`KismetMathLibrary.Conv_BoolToDouble` false))
          (bind _returnvalue_4 (`PrimitiveComponent.CreateDynamicMaterialInstance` _returnvalue_2 1 "/Game/VFX/River/Materials/Particles/Splash_Inst.Splash_Inst" "None"))
          (`MaterialInstanceDynamic.SetScalarParameterValue` _returnvalue_4 "Emissive Toggle" (`KismetMathLibrary.Conv_BoolToDouble` false))
          (`KismetArrayLibrary.Array_AddUnique` (`self.ListOfWaterfallParticles`) _returnvalue_2))))))
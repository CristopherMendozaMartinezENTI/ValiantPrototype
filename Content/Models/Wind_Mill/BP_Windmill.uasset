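; Windmill actor that spins its blade mesh.
; On BeginPlay the blade gets a random starting roll offset, so placed windmills do not turn in sync.
; Each Tick, while the blade is visible, it adds frame-time-scaled roll with a small random speed variation re-rolled every frame.
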(event `self.ReceiveBeginPlay`
  (`SceneComponent.K2_AddRelativeRotation` (`self.SM_Blade`) (`KismetMathLibrary.MakeRotator` (`KismetMathLibrary.RandomFloatInRange` 0.0 40.0)) false false))

(event `self.ReceiveTick`
  (params (DeltaSeconds :type "Float (single-precision)"))
  (if (`SceneComponent.IsVisible` (`self.SM_Blade`))
    (`SceneComponent.K2_AddRelativeRotation` (`self.SM_Blade`) (`KismetMathLibrary.MakeRotator` (* DeltaSeconds 30.0 (`KismetMathLibrary.RandomFloatInRange` 0.9 1.2))) false false)))

(fn `UserConstructionScript`)
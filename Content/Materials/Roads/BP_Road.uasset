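; BP_Road is a spline road actor that builds its meshes and material in the construction script.
; When UpdateInRealtime is set, ReconstructMeshes adds one spline mesh per segment, following point tangents and scales.
; Custom primitive data flags the first and last segments, and a per-road dynamic material receives falloff, dirt, tiling and colour settings.
; GetClosestPoint returns an interpolated spline location near a world position.
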(fn `GetClosestPoint`
  (params (WorldLocation :type "Vector Structure (by ref)"))
  (returns (ClosestPoint :type "Vector Structure"))
  (bind _splineref (`self.SplineRef`))
  (bind _returnvalue (`SplineComponent.FindInputKeyClosestToWorldLocation` (`self.SplineRef`) WorldLocation))
  (bind _returnvalue_2 (`KismetMathLibrary.FFloor` _returnvalue))
  (bind _returnvalue_3 (+ _returnvalue_2 1))
  (bind _returnvalue_4 (`SplineComponent.GetDistanceAlongSplineAtSplinePoint` _splineref _returnvalue_3))
  (return (`SplineComponent.GetLocationAtDistanceAlongSpline` (`self.SplineRef`) (- _returnvalue_4 (* (- (`SplineComponent.GetDistanceAlongSplineAtSplinePoint` _splineref _returnvalue_2) _returnvalue_4) (- _returnvalue (`KismetMathLibrary.Conv_IntToDouble` _returnvalue_3)))) "World")))

(fn `ReconstructMeshes`
  (params (SplineRef :type "SplineComponent Object Reference"))
  (bind _road_material_instance (`self.Road Material Instance`))
  (bind _splineref (`self.SplineRef`))
  (set `self.SplineRef` SplineRef)
  (`KismetArrayLibrary.Array_Clear` (`self.SplineMeshes`))
  (bind _returnvalue (`KismetMaterialLibrary.CreateDynamicMaterialInstance` (`self.Road Material`)))
  (set `self.Road Material Instance` _returnvalue)
  (if (`self.UpdateInRealtime`)
    (for _index (range (+ (- (`SplineComponent.GetNumberOfSplinePoints` (`self.SplineRef`)) 2) 1))
      (bind _returnvalue_2 (`AddComponent|NODE_AddSplineMeshComponent-2`))
      (`KismetArrayLibrary.Array_Add` (`self.SplineMeshes`) _returnvalue_2)
      (`SplineMeshComponent.SetForwardAxis` _returnvalue_2 "X" true)
      (bind _returnvalue_3 (+ _index 1))
      (`SplineMeshComponent.SetStartAndEnd` _returnvalue_2 (`SplineComponent.GetLocationAtSplinePoint` _splineref _index "Local") (`SplineComponent.GetTangentAtSplinePoint` _splineref _index "Local") (`SplineComponent.GetLocationAtSplinePoint` _splineref _returnvalue_3 "Local") (`SplineComponent.GetTangentAtSplinePoint` _splineref _returnvalue_3 "Local") true)
      (bind (_returnvalue_x _returnvalue_y _returnvalue_z) (`KismetMathLibrary.BreakVector` (`SplineComponent.GetScaleAtSplinePoint` _splineref _index)))
      (`SplineMeshComponent.SetStartScale` _returnvalue_2 (`KismetMathLibrary.MakeVector2D` _returnvalue_y _returnvalue_z) true)
      (bind (_returnvalue_x_2 _returnvalue_y_2 _returnvalue_z_2) (`KismetMathLibrary.BreakVector` (`SplineComponent.GetScaleAtSplinePoint` _splineref _returnvalue_3)))
      (`SplineMeshComponent.SetEndScale` _returnvalue_2 (`KismetMathLibrary.MakeVector2D` _returnvalue_y_2 _returnvalue_z_2) true)
      (`PrimitiveComponent.SetMaterial` _returnvalue_2 0 (`self.Road Material Instance`))
      (if (== _index 0)
        (`PrimitiveComponent.SetCustomPrimitiveDataFloat` _returnvalue_2 0 1.0)
        (elif (== _index (- (`SplineComponent.GetNumberOfSplinePoints` (`self.SplineRef`)) 2))
          (`PrimitiveComponent.SetCustomPrimitiveDataFloat` _returnvalue_2 1 1.0)))))
  ;[1 1 1] Make all these variables Public so you can edit them in the editor PER road
  (`MaterialInstanceDynamic.SetScalarParameterValue` _road_material_instance "RoadFalloffOffset" 0.0)
  (`MaterialInstanceDynamic.SetScalarParameterValue` _road_material_instance "RoadFalloffHardness" (`self.RoadFalloffHardness`))
  (`MaterialInstanceDynamic.SetScalarParameterValue` _road_material_instance "RoadOpacityContrast" (`self.RoadOpacityContrast`))
  (`MaterialInstanceDynamic.SetScalarParameterValue` _road_material_instance "NormalFlatness" (`self.RoadNormalFlatness`))
  (`MaterialInstanceDynamic.SetScalarParameterValue` _road_material_instance "DirtOffset" (`self.DirtOffset`))
  (`MaterialInstanceDynamic.SetScalarParameterValue` _road_material_instance "DirtContrast" (`self.DirtContrast`))
  (`MaterialInstanceDynamic.SetScalarParameterValue` _road_material_instance "Tiling X" (`self.Tiling X`))
  (`MaterialInstanceDynamic.SetScalarParameterValue` _road_material_instance "Tiling Y" (`self.Tiling Y`))
  (`MaterialInstanceDynamic.SetScalarParameterValue` _road_material_instance "NoiseInfluence" (`self.NoiseInfluence`))
  (`MaterialInstanceDynamic.SetVectorParameterValue` _road_material_instance "DirtColour" (`self.DirtColour`))
  (`MaterialInstanceDynamic.SetVectorParameterValue` _road_material_instance "RoadColour" (`self.RoadColour`))
  (`MaterialInstanceDynamic.SetScalarParameterValue` _road_material_instance "RoadEndFalloffHardness" (`self.RoadEndFalloffHardness`)))

(fn `UserConstructionScript`
  (`self.ReconstructMeshes` (`self.SplineRef`)))